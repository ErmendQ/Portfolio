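; BP_CheckPoint is a checkpoint actor for the side-scroller that records a respawn location and gives access to the skills menu.
; The first overlap of its Sphere by BP_SideScrollingCharacter writes the checkpoint's location to the character's CheckPointLocation, guarded by a DoOnce.
; Overlap begin and end open and close a Gate, so IA_Interact creates a new W_Skills widget only while the character is inside.
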(event `self.ReceiveBeginPlay`
  (`self.EnableInput` (`GameplayStatics.GetPlayerController` 0)))

(event `self.Sphere.OnComponentBeginOverlap`
  (params (OverlappedComponent :type "PrimitiveComponent Object Reference") (OtherActor :type "Actor Object Reference") (OtherComp :type "PrimitiveComponent Object Reference") (OtherBodyIndex :type Integer) (bFromSweep :type Boolean) (SweepResult :type "HitResult Structure (by ref)"))
  (if (== (`GameplayStatics.GetObjectClass` OtherActor) "/Game/MyContent/Blueprints/BP_SideScrollingCharacter.BP_SideScrollingCharacter_C")
    (`|ExecutionSequence`
      (:`then_0`
        (`/Engine/EditorBlueprintResources/StandardMacros.DoOnce` false
          (:`Completed`
            (bind _asbp_side_scrolling_character (cast `/Game/MyContent/Blueprints/BP_SideScrollingCharacter` OtherActor))
            (set `/Game/MyContent/Blueprints/BP_SideScrollingCharacter.CheckPointLocation` (`self.K2_GetActorLocation`) _asbp_side_scrolling_character))))
      (:`then_1`
        (goto _label :!via `Open`)))))

(event `EnhancedInput|/Game/MyContent/Input/IA_Interact`
  (params (ActionValue :type Boolean) (ElapsedSeconds :type "Float (double-precision)") (TriggeredSeconds :type "Float (double-precision)") (InputAction :type "InputAction Object Reference" :default "/Game/MyContent/Input/IA_Interact.IA_Interact"))
  (:`Triggered`
    (`/Engine/EditorBlueprintResources/StandardMacros.Gate` true :!label _label
      (:`Exit`
        (bind _returnvalue (`|CreateWidget` "/Game/MyContent/Widgets/W_Skills.W_Skills_C" (`GameplayStatics.GetPlayerController` 0)))
        (`UserWidget.AddToViewport` _returnvalue -1)))))

(event `self.Sphere.OnComponentEndOverlap`
  (params (OverlappedComponent :type "PrimitiveComponent Object Reference") (OtherActor :type "Actor Object Reference") (OtherComp :type "PrimitiveComponent Object Reference") (OtherBodyIndex :type Integer))
  (if (== (`GameplayStatics.GetObjectClass` OtherActor) "/Game/MyContent/Blueprints/BP_SideScrollingCharacter.BP_SideScrollingCharacter_C")
    (goto _label :!via `Close`)))

(fn `UserConstructionScript`)