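; BPC_Pouring is an actor component that pours drink liquid from its owner, such as a bottle.
; It takes the pour origin from the owner's scene component tagged "Pour", which must exist.
; StartPour runs a fast looping timer that fires the ConsumeVolume dispatcher and spawns a BP_LiquidProjectile carrying drink type and pressure, until StopPour clears it.
; The pressure multiplier scales flow, with the default matching a speed-pourer spirit bottle.
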(event `self.ReceiveBeginPlay`
  ;[0 1 0 1 30] IMPORTANT: In order for the pouring to work, the owning actor must have a scene component with the tag "Pour" which serves as the origin of the pouring liquid
  (set `self.PourOrigin` (`|GetArrayItem` (`Actor.GetComponentsByTag` (`self.GetOwner`) "/Script/Engine.SceneComponent" "Pour"))))

(event `StartPour`
  (params (PressureMultiplier :type "Float (single-precision)") (`Drink Type` :type "/Game/Blueprints/Enums/E_DrinkTypes Enum" :default "NewEnumerator0"))
  ;[0 0.2812 0.2812 1 30] Pouring loop: Default pressure is 1 which means 10ml or 10vol of liquid per second, this is the pouring speed of a basic spirit bottle equipped with a speed pourer
  (bind _returnvalue (`KismetSystemLibrary.K2_SetTimerDelegate` (delegate `Pouring`) 0.01 true))
  (set `self.PourTimerHandle` _returnvalue))

(event `Pouring`
  ;[0 0.2812 0.2812 1 30] Pouring loop: Default pressure is 1 which means 10ml or 10vol of liquid per second, this is the pouring speed of a basic spirit bottle equipped with a speed pourer
  (`self.ConsumeVolume` (/ (stale `StartPour` PressureMultiplier) 10.0))
  (`|SpawnActorFromClass` "/Game/Blueprints/BP_LiquidProjectile.BP_LiquidProjectile_C" (`SceneComponent.K2_GetComponentToWorld` (`self.PourOrigin`)) "Undefined" "MultiplyWithRoot" null (stale `StartPour` `Drink Type`) (stale `StartPour` PressureMultiplier) null))

(event `StopPour`
  ;[0 0.2812 0.2812 1 30] Pouring loop: Default pressure is 1 which means 10ml or 10vol of liquid per second, this is the pouring speed of a basic spirit bottle equipped with a speed pourer
  ;;[0 0 0] Stop pouring loop
  (`KismetSystemLibrary.K2_ClearAndInvalidateTimerHandle` (`self.PourTimerHandle`)))