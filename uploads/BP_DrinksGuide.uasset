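; BP_DrinksGuide is a drinks guide actor that can be focused on for a zoomed-in view.
; Focus ignores the hit location and returns the Cube component's world location with zoom enabled and a fixed FOV amount.
; The item functions return a fixed type, with ammo and property functions left as zero or empty stubs.
; The event graph and construction script contain no logic.
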(fn `Focus`
  (params (HitLocation :type "Vector Structure"))
  (returns (Location :type "Vector Structure") (Zoom :type Boolean) (ZoomAmountInFOV :type "Float (double-precision)"))
  (return (`SceneComponent.K2_GetComponentLocation` (`self.Cube`)) true 50.0))

(fn `GetAmmo`
  (returns (Return :type Integer))
  (return 0))

(fn `GetAmmoText`
  (returns (Return :type "TextRenderComponent Object Reference"))
  (return null))

(fn `GetItemProperties`
  (returns (Return :type "/Game/Blueprints/DataTables/Structs/S_Item2 Structure"))
  (return))

(fn `GetItemType`
  (returns (ReturnValue :type "/Game/Blueprints/Enums/E_Items Enum"))
  (return "NewEnumerator1"))

(fn `GetMaxAmmo`
  (returns (Return :type Integer))
  (return 0))

(fn `SetAmmo`
  (params (Amount :type Integer))
  (returns (Return :type Integer))
  (return 0))

(fn `UserConstructionScript`)