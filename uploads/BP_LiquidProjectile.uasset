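; BP_LiquidProjectile is a projectile of liquid that fills glasses with a set drink type.
; On BeginPlay it looks up its DrinkType in DT_DrinkTypes and tints its mesh materials with that row's Color.
; On hit, it calls Fill on the other actor's BPC_Glass component, if present, passing the drink type and pressure multiplier, then destroys itself whatever it hit.
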(event `self.ReceiveBeginPlay`
  ;[0 1 0] Set projectile liquid material color
  (bind _returnvalue (`|GetDataTableRow` "/Game/Blueprints/DataTables/DT_DrinkTypes.DT_DrinkTypes" (`KismetStringLibrary.Conv_StringToName` (`|GetEnumeratorNameAsString` (`self.Drink Type`))))
    (:`then`
      (`MeshComponent.SetVectorParameterValueOnMaterials` (`self.StaticMesh`) "Color" (`KismetMathLibrary.Conv_LinearColorToVector` (`KismetMathLibrary.Conv_ColorToLinearColor` (`.Color_22_A7F580704C3BA7C8009C3AB9F719A5F7` (break `/Game/Blueprints/DataTables/Structs/S_DrinkType` _returnvalue))))))))

(event `self.ReceiveHit`
  (params (MyComp :type "PrimitiveComponent Object Reference") (Other :type "Actor Object Reference") (OtherComp :type "PrimitiveComponent Object Reference") (bSelfMoved :type Boolean) (HitLocation :type "Vector Structure") (HitNormal :type "Vector Structure") (NormalImpulse :type "Vector Structure") (Hit :type "HitResult Structure (by ref)"))
  (bind _returnvalue (`self.GetComponentByClass` Other "/Game/Blueprints/Components/BPC_Glass.BPC_Glass_C"))
  ;[0 1 0] When hitting actor with the BPC_Glass component, fill with set drink type, destroy after regardless of hit actor
  (`|ExecutionSequence`
    (:`then_0`
      (`/Engine/EditorBlueprintResources/StandardMacros.IsValid` _returnvalue
        (:`Is Valid`
          (`/Game/Blueprints/Components/BPC_Glass.Fill` _returnvalue (`self.Drink Type`) (`self.Pressure Multiplier`)))))
    (:`then_1`
      (`self.K2_DestroyActor`))))

(fn `UserConstructionScript`)