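; BP_ForceFieldPanel is a panel actor that switches off a linked force field.
; Taking damage calls Toggle, and the Toggleon event calls Disable on ControlledForcefield if that reference is valid.
; Toggle is not defined in this graph, and no event here re-enables the field.
; The construction script colors Cube2 glowing green or red from the Unlocked flag, so that color is not updated by these events.
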(event `self.ToggleOn`
  (params (BP_PC :type "/Game/MyContent/Blueprints/Core/BP_PC_Default Object Reference"))
  (bind _controlledforcefield (`self.ControlledForcefield`))
  ;[1 1 1] Disable
  (`/Engine/EditorBlueprintResources/StandardMacros.IsValid` _controlledforcefield
    (:`Is Valid`
      (`/Game/MyContent/Blueprints/EnvironmentInteractables/BP_ForceField.Disable` _controlledforcefield))))

(event `/Game/MyContent/Blueprints/Interfaces/BI_Interaction.Damage`
  (params (Amount :type "Float (double-precision)") (Damager :type "/Game/FirstPerson/Blueprints/BP_FirstPersonCharacter Object Reference") (Type :type "/Game/MyContent/Blueprints/Enums/E_DamageTypes Enum" :default "NewEnumerator0"))
  ;[1 1 1] Disable
  (`self.Toggle` null))

(fn `UserConstructionScript`
  (bind _cube2 (`self.Cube2`))
  (`parent.UserConstructionScript`)
  (if (`self.Unlocked`)
    (`PrimitiveComponent.SetMaterial` _cube2 0 "/Game/Erik/Mats/M_GreyboxGlowGreen.M_GreyboxGlowGreen")
    (else
      (`PrimitiveComponent.SetMaterial` _cube2 0 "/Game/Erik/Mats/M_GreyboxGlowRed.M_GreyboxGlowRed"))))