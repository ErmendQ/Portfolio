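; BP_Inmate is an interactable prison NPC with a random mesh, chosen idle animation and look-at widget.
; It builds an interaction list for talking, plus optional item trading and gambling.
; Talking shows preset or random DataTable subtitles and gives a one-time clue, optionally gated by Charisma.
; Interactions route through server-to-multicast events; card games consume an item and award a prize through the linked Table's win event.
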(event `self.ReceiveBeginPlay`
  (bind _table (`self.Table`))
  ;[0 0.08041 1] Begin play
  (`|ExecutionSequence`
    (:`then_0`
      ;;[1 1 1] Set widget ref
      (bind _asw_world_space_interaction (cast `/Game/MyContent/UI/W_WorldSpaceInteraction` (`WidgetComponent.GetWidget` (`self.Widget`))))
      (set `self.Ref_TextWidget` _asw_world_space_interaction)
      (`self.SetInteractions`)
      ;;[1 1 1] SetAnimation
      (switch `/Game/MyContent/Blueprints/Enums/Inmates/E_InmateIdles` (`self.Animation`)
        (:`NewEnumerator0`
          (`SkeletalMeshComponent.PlayAnimation` (`self.Mesh`) "/Game/MyContent/Animations/InmateIdles/Anim_SittingIdle.Anim_SittingIdle" true))
        (:`NewEnumerator3`
          (`SkeletalMeshComponent.PlayAnimation` (`self.Mesh`) "/Game/MyContent/Animations/InmateIdles/AnimSittingIdle2.AnimSittingIdle2" true))
        (:`NewEnumerator6`
          (`SkeletalMeshComponent.PlayAnimation` (`self.Mesh`) "/Game/MyContent/Animations/InmateIdles/Anim_SittingWritingIdle.Anim_SittingWritingIdle" true))
        (:`NewEnumerator7`
          (`SkeletalMeshComponent.PlayAnimation` (`self.Mesh`) "/Game/MyContent/Animations/InmateIdles/Anim_SittingTalkingIdle.Anim_SittingTalkingIdle" true))
        (:`NewEnumerator1`
          (`SkeletalMeshComponent.PlayAnimation` (`self.Mesh`) "/Game/MyContent/Animations/InmateIdles/Anim_SadIdle.Anim_SadIdle" true))
        (:`NewEnumerator2`
          (`SkeletalMeshComponent.PlayAnimation` (`self.Mesh`) "/Game/MyContent/Animations/InmateIdles/Anim_StandardIdle.Anim_StandardIdle" true))
        (:`NewEnumerator5`
          (`SkeletalMeshComponent.PlayAnimation` (`self.Mesh`) "/Game/MyContent/Animations/InmateIdles/Anim_LeaningIdle.Anim_LeaningIdle" true))
        (:`NewEnumerator4`
          (`SkeletalMeshComponent.PlayAnimation` (`self.Mesh`) "/Game/MyContent/Animations/InmateIdles/Anim_LayingIdle.Anim_LayingIdle" true))))
    (:`then_1`
      ;;[1 1 1] Card game reward
      (`/Engine/EditorBlueprintResources/StandardMacros.IsValid` _table
        (:`Is Valid`
          (add `/Game/Erik/BP_CardTable.PlayerWon` _table (delegate `PlayerWon_Event`)))))
    (:`then_2`
      ;;[1 1 1] Set array of random voicelines
      (bind _outrownames (`DataTableFunctionLibrary.GetDataTableRowNames` "/Game/MyContent/Databases/Voicelines/DT_Voicelines.DT_Voicelines"))
      (for _array_element _outrownames
        (if (`KismetStringLibrary.Contains` (`KismetStringLibrary.Conv_NameToString` _array_element) "NewRow")
          (`KismetArrayLibrary.Array_Add` (`self.RandomVoiceLineRows`) _array_element))))))

(event `PlayerWon_Event`
  (bind _playercontroller (`/Game/Erik/BP_CardTable.PlayerController` (`self.Table`)))
  ;[0 0.08041 1] Begin play
  ;;[1 1 1] Card game reward
  (`/Engine/EditorBlueprintResources/StandardMacros.IsValid` _playercontroller
    (:`Is Valid`
      (`/Game/MyContent/Blueprints/Core/BP_PC_Default.AddItem` _playercontroller (`self.WinItem`)))))

(event `LookedAt`
  ;[1 1 1] Looked at widget appear/disappear
  (`|ExecutionSequence`
    (:`then_0`
      (bind _widget (`self.Widget`)
        (:`then`
          (`SceneComponent.SetVisibility` _widget true false))
        (:`else`)))
    (:`then_1`
      (`KismetSystemLibrary.RetriggerableDelay` 0.1)
      (`SceneComponent.SetVisibility` _widget false false))))

(event `SetInteractions`
  ;[1 1 1] Set interactions
  (`self.SRV_SetInteractions`))

(event `SRV_SetInteractions`
  ;[1 1 1] Set interactions
  (`self.MC_SetInteractions`))

(event `MC_SetInteractions`
  (bind _interactions (`self.Interactions`))
  ;[1 1 1] Set interactions
  (`KismetArrayLibrary.Array_Clear` _interactions)
  (`KismetArrayLibrary.Array_Add` _interactions "NewEnumerator11")
  (`|ExecutionSequence`
    (:`then_0`
      (if (`self.TradeOffer`)
        (`KismetArrayLibrary.Array_Add` (`self.Interactions`) "NewEnumerator12")))
    (:`then_1`
      (if (`self.Gambler`)
        (`KismetArrayLibrary.Array_Add` (`self.Interactions`) "NewEnumerator22")))))

(event `UpdateWidgetText`
  (bind _ref_textwidget (`self.Ref_TextWidget`))
  ;[1 1 1] Widget text setup
  (`/Engine/EditorBlueprintResources/StandardMacros.IsValid` (`self.Ref_TextWidget`)
    (:`Is Valid`
      (set `/Game/MyContent/UI/W_WorldSpaceInteraction.Name` (`KismetTextLibrary.Conv_NameToText` (`self.Name`)) (`self.Ref_TextWidget`))
      (set `/Game/MyContent/UI/W_WorldSpaceInteraction.Interactions` (`self.Interactions`) _ref_textwidget)
      (`/Game/MyContent/UI/W_WorldSpaceInteraction.Update` _ref_textwidget))))

(event `/Game/MyContent/Blueprints/Interfaces/BI_Interaction.Interaction`
  (params (Interactor :type "/Game/MyContent/Blueprints/Core/BP_PC_Default Object Reference") (Inventory :type "Array of /Game/MyContent/Blueprints/Enums/E_Items Enum (by ref)" :default _) (Proceed :type Boolean) (InteractionOptionIndex :type Integer))
  (bind _ref_playerhud (`/Game/MyContent/Blueprints/Core/BP_PC_Default.Ref_PlayerHUD` Interactor))
  (bind _output (`|GetArrayItem` (`self.Interactions`) InteractionOptionIndex))
  ;[1 1 1] Interaction
  (`self.SRV_Interaction` Interactor _output (`self.MissionClue`) (`self.InfoType`))
  (if (`|EnumEquality` _output "NewEnumerator11")
    ;;[0 0 0] Subtitles
    (if (`self.NeedsCharisma`)
      (if (`/Game/MyContent/Blueprints/Core/BP_PC_Default.Skill_CharismaExpert` Interactor)
        (`/Engine/EditorBlueprintResources/StandardMacros.IsValid` _ref_playerhud :!label _label
          (:`Is Valid`
            (if (`KismetTextLibrary.EqualEqual_TextText` (`self.DisplayedText`) "")
              (bind _returnvalue (`|GetDataTableRow` "/Game/MyContent/Databases/Voicelines/DT_Voicelines.DT_Voicelines" (`KismetArrayLibrary.Array_Random` (`self.RandomVoiceLineRows`)))
                (:`then`
                  (`/Game/MyContent/UI/Player/W_PlayerHUD.DisplaySubs` _ref_playerhud (`.Text_6_4B1CA5464D99210387319DBAA15A7E78` (break `/Game/MyContent/Databases/Voicelines/F_Voicelines` _returnvalue))) ; Random
                ))
              (else
                (`/Game/MyContent/UI/Player/W_PlayerHUD.DisplaySubs` _ref_playerhud (`self.DisplayedText`)) ; Preset
              ))))
        (else
          (`/Engine/EditorBlueprintResources/StandardMacros.IsValid` _ref_playerhud
            (:`Is Valid`
              (`/Game/MyContent/UI/Player/W_PlayerHUD.DisplaySubs` _ref_playerhud (`self.NoCharismaDisplayedText`)) ; Needs charisma and player has none
            ))))
      (else
        (goto _label)))))

(event `SRV_Interaction`
  (params (InteractorPC :type "/Game/MyContent/Blueprints/Core/BP_PC_Default Object Reference") (InteractionType :type "/Game/MyContent/Blueprints/Enums/E_InteractionTypes Enum" :default "NewEnumerator0") (Info :type Text) (InfoType :type "/Game/MyContent/Blueprints/Enums/E_MissionClueTypes Enum" :default "NewEnumerator0"))
  ;[1 1 1] Interaction
  (`self.MC_Interaction` InteractorPC InteractionType Info InfoType))

(event `MC_Interaction`
  (params (InteractorPC :type "/Game/MyContent/Blueprints/Core/BP_PC_Default Object Reference") (InteractionType :type "/Game/MyContent/Blueprints/Enums/E_InteractionTypes Enum" :default "NewEnumerator0") (Info :type Text) (InfoType :type "/Game/MyContent/Blueprints/Enums/E_MissionClueTypes Enum" :default "NewEnumerator0"))
  (bind _ref_playercharacter (`/Game/MyContent/Blueprints/Core/BP_PC_Default.Ref_PlayerCharacter` InteractorPC))
  (bind _table (`self.Table`))
  (bind _ref_playerhud (`/Game/MyContent/Blueprints/Core/BP_PC_Default.Ref_PlayerHUD` InteractorPC))
  (bind _ref_playercharacter_2 (`/Game/MyContent/Blueprints/Core/BP_PC_Default.Ref_PlayerCharacter` InteractorPC))
  ;[1 1 1] Interaction
  (`/Engine/EditorBlueprintResources/StandardMacros.IsValid` InteractorPC
    (:`Is Valid`
      (if (`|EnumEquality` InteractionType "NewEnumerator12")
        ;;[0 0 0] TradeItem
        (if (`KismetArrayLibrary.Array_Contains` (`/Game/MyContent/Blueprints/Core/BP_PC_Default.Items` InteractorPC) (`self.NeededItem`))
          (bind _success (`/Game/MyContent/Blueprints/Core/BP_PC_Default.UseItem` InteractorPC (`self.NeededItem`) false))
          (if _success
            (`/Game/MyContent/Blueprints/Core/BP_PC_Default.AddItem` InteractorPC (`self.GivenItem`))
            (`/Game/MyContent/UI/Player/W_PlayerHUD.DisplaySubs` _ref_playerhud (`self.TradeSuccessText`))
            (`GameplayStatics.PlaySound2D` "/Game/MyContent/Audio/CUEs/SC_TradeComplete.SC_TradeComplete" 1.0 1.0 0.0 null null)
            (set `self.TradeOffer` false))
          (else
            (`/Game/FirstPerson/Blueprints/BP_FirstPersonCharacter.FeedbackMessage` (`/Game/MyContent/Blueprints/Core/BP_PC_Default.Ref_PlayerCharacter` InteractorPC) "" "NewEnumerator0" "NewEnumerator2" "NewEnumerator0" (`self.NeededItem`))
            (`/Game/MyContent/UI/Player/W_PlayerHUD.DisplaySubs` _ref_playerhud (`self.TradeFailText`))))
        (elif (`|EnumEquality` InteractionType "NewEnumerator11")
          ;;[0 0 0] Get info
          (if (or (and (`/Game/MyContent/Blueprints/Core/BP_PC_Default.Skill_CharismaExpert` InteractorPC) (`self.NeedsCharisma`)) (not (`self.NeedsCharisma`)))
            (if (not (`self.InfoGiven`))
              (set `self.InfoGiven` true)
              (if (not (`KismetTextLibrary.EqualEqual_TextText` Info ""))
                (`/Engine/EditorBlueprintResources/StandardMacros.IsValid` _ref_playercharacter_2
                  (:`Is Valid`
                    (`/Game/FirstPerson/Blueprints/BP_FirstPersonCharacter.FeedbackMessage` _ref_playercharacter_2 Info InfoType "NewEnumerator1" "NewEnumerator0" "NewEnumerator0"))))))
          (elif (`|EnumEquality` InteractionType "NewEnumerator22")
            ;;[0 0 0] Play cards
            (bind _returnvalue (`/Game/MyContent/Blueprints/Core/BP_PC_Default.HasItem?` InteractorPC "NewEnumerator28"))
            (if _returnvalue
              (`/Engine/EditorBlueprintResources/StandardMacros.IsValid` _ref_playercharacter
                (:`Is Valid`
                  (`/Game/FirstPerson/Blueprints/BP_FirstPersonCharacter.SRV_PlayCards` _ref_playercharacter _table InteractorPC)
                  (`self.EnableInput` _table InteractorPC)
                  (set `/Game/Erik/BP_CardTable.PlayerController` InteractorPC _table)
                  (`/Game/Erik/BP_CardTable.Reset` _table)
                  (`/Game/MyContent/Blueprints/Core/BP_PC_Default.UseItem` InteractorPC "NewEnumerator28" false)))
              (else
                (`/Game/FirstPerson/Blueprints/BP_FirstPersonCharacter.FeedbackMessage` _ref_playercharacter "" "NewEnumerator0" "NewEnumerator2" "NewEnumerator0" "NewEnumerator28")))))))))

(fn `GetInteractionsAmount`
  (returns (Amount :type Integer))
  (return (`KismetArrayLibrary.Array_Length` (`self.Interactions`))))

(fn `LookAt`
  (params (Examiner :type "/Game/MyContent/Blueprints/Core/BP_PC_Default Object Reference") (HitLocation :type "Vector Structure"))
  (returns (InteractionType :type "/Game/MyContent/Blueprints/Enums/E_InteractionTypes Enum") (Name :type String) (CanAccess :type Boolean))
  (bind _output_get (set `self.Ref_PC` Examiner))
  (set `/Game/MyContent/UI/W_WorldSpaceInteraction.Ref_PC` _output_get (`self.Ref_TextWidget`))
  (`self.UpdateWidgetText`)
  (`self.LookedAt`)
  (return "NewEnumerator0" "" false))

(fn `UserConstructionScript`
  (`SkeletalMeshComponent.SetSkeletalMeshAsset` (`self.Mesh`) (`KismetArrayLibrary.Array_Random` (`self.SKMs`))))