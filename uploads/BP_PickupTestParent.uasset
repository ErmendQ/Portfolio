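; Base interactable item pickup that can be added to the interactor's inventory or, if it is food, used to restore health.
; The ItemType enum selects a DT_ItemPickups row, which supplies the mesh during construction and the name and heal amount at BeginPlay.
; Pickup goes through a server-to-multicast event chain and requires a free slot.
; LookAt keeps the world-space prompt visible via a retriggerable delay, while highlighting uses custom depth stencil.
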(event `self.ReceiveBeginPlay`
  ;[1 1 1] Sets the name of the item displayed on HUD
  (bind _returnvalue (`|GetDataTableRow` "/Game/MyContent/Databases/Items/DT_ItemPickups.DT_ItemPickups" (`self.RowID`))
    (:`then`
      (bind (_typeid _name _description _icon _staticmesh _pickupsound _equipactor _dropspawnactor _isgun _damage _shotdelay _recoil _meleeattackspeed _throwforce _throwactor _noise _infiniteuse _shootsound _swingsound _healamount) (break `/Game/MyContent/Databases/Items/F_ItemPickup` _returnvalue))
      (set `self.Heal Amount` _healamount)
      (set `self.Name` (`KismetStringLibrary.Conv_NameToString` _name))
      ;[1 1 1] Set name in world space widget
      (bind _asw_world_space_interaction (cast `/Game/MyContent/UI/W_WorldSpaceInteraction` (`WidgetComponent.GetWidget` (`self.Widget`))))
      (bind _output_get (set `self.As Test World Space` _asw_world_space_interaction))
      (set `/Game/MyContent/UI/W_WorldSpaceInteraction.Interactions` (select `bool` (`self.IsFood`) :`false` (`|MakeArray` "NewEnumerator3" :!type "/Game/MyContent/Blueprints/Enums/E_InteractionTypes Enum") :`true` (`|MakeArray` "NewEnumerator3" "NewEnumerator21" :!type "/Game/MyContent/Blueprints/Enums/E_InteractionTypes Enum")) _output_get)
      (set `/Game/MyContent/UI/W_WorldSpaceInteraction.Name` (`KismetTextLibrary.Conv_StringToText` (`self.Name`)) _output_get))))

(event `LookedAt`
  ;[1 1 1] World space widget appear/disappear
  (`|ExecutionSequence`
    (:`then_0`
      (`SceneComponent.SetVisibility` (`self.Widget`) true false))
    (:`then_1`
      (`KismetSystemLibrary.RetriggerableDelay` 0.01)
      (`SceneComponent.SetVisibility` (`self.Widget`) false false))))

(event `/Game/MyContent/Blueprints/Interfaces/BI_Interaction.Interaction`
  (params (Interactor :type "/Game/MyContent/Blueprints/Core/BP_PC_Default Object Reference") (Inventory :type "Array of /Game/MyContent/Blueprints/Enums/E_Items Enum (by ref)" :default _) (Proceed :type Boolean) (InteractionOptionIndex :type Integer))
  ;[1 1 1] Interacted
  (if (`|EnumInequality` (`|GetArrayItem` (`/Game/MyContent/UI/W_WorldSpaceInteraction.Interactions` (`self.As Test World Space`)) InteractionOptionIndex) "NewEnumerator21")
    (`self.Sever_Interaction` Interactor)
    (else
      (`/Game/FirstPerson/Blueprints/BP_FirstPersonCharacter.Server_AddHealth` (`/Game/MyContent/Blueprints/Core/BP_PC_Default.Ref_PlayerCharacter` Interactor) (`self.Heal Amount`))
      (`self.K2_DestroyActor`))))

(event `Sever_Interaction`
  (params (Interactor :type "/Game/MyContent/Blueprints/Core/BP_PC_Default Object Reference"))
  ;[1 1 1] Interacted
  (`self.Multicast_Interaction` Interactor))

(event `Multicast_Interaction`
  (params (Interactor :type "/Game/MyContent/Blueprints/Core/BP_PC_Default Object Reference"))
  ;[1 1 1] Interacted
  (`self.PickUpItem` Interactor)
  (`self.PickedUp`))

(event `/Game/MyContent/Blueprints/Interfaces/BI_Interaction.Highlight`
  (bind _cube (`self.Cube`))
  ;[1 1 1] Highlight
  (`PrimitiveComponent.SetRenderCustomDepth` _cube true)
  (`PrimitiveComponent.SetCustomDepthStencilValue` _cube 2))

(event `/Game/MyContent/Blueprints/Interfaces/BI_Interaction.DeHighlight`
  (bind _cube (`self.Cube`))
  ;[1 1 1] Highlight
  (`PrimitiveComponent.SetRenderCustomDepth` _cube false)
  (`PrimitiveComponent.SetCustomDepthStencilValue` _cube 0))

(fn `GetInteractionsAmount`
  (returns (Amount :type Integer))
  (if (`self.IsFood`)
    (return 2)
    (else
      (return 1))))

(fn `LookAt`
  (params (Examiner :type "/Game/MyContent/Blueprints/Core/BP_PC_Default Object Reference") (HitLocation :type "Vector Structure"))
  (returns (InteractionType :type "/Game/MyContent/Blueprints/Enums/E_InteractionTypes Enum") (Name :type String) (CanAccess :type Boolean))
  (`/Engine/EditorBlueprintResources/StandardMacros.IsValid` Examiner
    (:`Is Valid`
      (set `/Game/MyContent/UI/W_WorldSpaceInteraction.Ref_PC` Examiner (`self.As Test World Space`))
      (`self.LookedAt`)
      (return "NewEnumerator3" (`self.Name`) false))))

(fn `PickUpItem`
  (params (Interactor :type "/Game/MyContent/Blueprints/Core/BP_PC_Default Object Reference"))
  (`/Engine/EditorBlueprintResources/StandardMacros.IsValid` Interactor
    (:`Is Valid`
      ;[1 1 1] Has free item slot
      (if (< (`KismetArrayLibrary.Array_Length` (`/Game/MyContent/Blueprints/Core/BP_PC_Default.Items` Interactor)) (`/Game/MyContent/Blueprints/Core/BP_PC_Default.ItemSlots` Interactor))
        (bind _returnvalue (`|GetDataTableRow` "/Game/MyContent/Databases/Items/DT_ItemPickups.DT_ItemPickups" (`self.RowID`))
          (:`then`
            (`/Game/MyContent/Blueprints/Core/BP_PC_Default.AddItem` Interactor (`.TypeID_26_6085895F47BFB36E5CE9399F3397E6E7` (break `/Game/MyContent/Databases/Items/F_ItemPickup` _returnvalue)))
            (`GameplayStatics.PlaySound2D` "/Game/MyContent/Audio/CUEs/SC_TradeComplete.SC_TradeComplete" 1.0 (`KismetMathLibrary.RandomFloatInRange` 0.8 1.2) 0.0 null null)
            (`self.K2_DestroyActor`)))))))

(fn `UserConstructionScript`
  ;[1 1 1] Set static mesh
  (bind _outrownames (`DataTableFunctionLibrary.GetDataTableRowNames` "/Game/MyContent/Databases/Items/DT_ItemPickups.DT_ItemPickups"))
  (for _array_element _outrownames
    (if (== _array_element (`|GetEnumeratorNameAsString` (`self.ItemType`)))
      (set `self.RowID` _array_element)
      (bind _returnvalue (`|GetDataTableRow` "/Game/MyContent/Databases/Items/DT_ItemPickups.DT_ItemPickups" _array_element)
        (:`then`
          (bind (_typeid _name _description _icon _staticmesh) (break `/Game/MyContent/Databases/Items/F_ItemPickup` _returnvalue))
          (if (!= _staticmesh null)
            (`StaticMeshComponent.SetStaticMesh` (`self.Cube`) _staticmesh)))))))