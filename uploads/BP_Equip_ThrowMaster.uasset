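; Base equippable for throwable items that lets the first-person player aim and throw the selected item.
; On the shoot input it looks up the throw actor for its item type in DT_ItemPickups and has the character spawn it server-side from the mesh location.
; Throw direction comes from a camera line trace, turned toward the hit point or trace end to correct for mesh offset.
; Throwing also consumes the inventory item, updates holster state and exits aiming.
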(event `self.ReceiveBeginPlay`
  ;[1 1 1] Casting refs+input
  (bind _asbp_first_person_character (cast `/Game/FirstPerson/Blueprints/BP_FirstPersonCharacter` (`GameplayStatics.GetPlayerCharacter` 0)))
  (set `self.Ref_Character` _asbp_first_person_character)
  (bind _asbp_pc_default (cast `/Game/MyContent/Blueprints/Core/BP_PC_Default` (`GameplayStatics.GetPlayerController` 0)))
  (set `self.Ref_PC` _asbp_pc_default)
  (`self.EnableInput` (`GameplayStatics.GetPlayerController` 0)))

(event `EnhancedInput|/Game/FirstPerson/Input/Actions_Default/IA_Shoot`
  (params (ActionValue :type Boolean) (ElapsedSeconds :type "Float (double-precision)") (TriggeredSeconds :type "Float (double-precision)") (InputAction :type "InputAction Object Reference" :default "/Game/FirstPerson/Input/Actions_Default/IA_Shoot.IA_Shoot"))
  (bind _ref_character (`self.Ref_Character`))
  (bind _ref_pc (`self.Ref_PC`))
  ;[1 1 1] Character throw item
  (:`Triggered`
    (bind _lookatrotation (`self.CalculateAimTarget`))
    (bind _returnvalue (`|GetDataTableRow` "/Game/MyContent/Databases/Items/DT_ItemPickups.DT_ItemPickups" (`KismetStringLibrary.Conv_StringToName` (`|GetEnumeratorNameAsString` (`self.ItemType`))))
      (:`then`
        (`/Game/FirstPerson/Blueprints/BP_FirstPersonCharacter.SRV_ThrowProjectile` (`self.Ref_Character`) (`.ThrowActor_51_4A049C2B448CFF970A395287205FA6D8` (break `/Game/MyContent/Databases/Items/F_ItemPickup` _returnvalue)) (`SceneComponent.K2_GetComponentLocation` (`self.StaticMesh`)) _lookatrotation)
        ;[1 1 1] Remove item from inventory
        (`/Game/MyContent/Blueprints/Core/BP_PC_Default.SRV_UseItem` _ref_pc (`|GetArrayItem` (`/Game/MyContent/Blueprints/Core/BP_PC_Default.Items` _ref_pc) (`/Game/MyContent/Blueprints/Core/BP_PC_Default.SelectedItemIndex` _ref_pc)))
        (`self.ThrowUnholster`)
        (if (`/Game/FirstPerson/Blueprints/BP_FirstPersonCharacter.IsAiming` _ref_character)
          (`/Game/FirstPerson/Blueprints/BP_FirstPersonCharacter.AimOut` _ref_character))))))

(event `EnhancedInput|/Game/FirstPerson/Input/Actions_Default/IA_Aim`
  (params (ActionValue :type Boolean) (ElapsedSeconds :type "Float (double-precision)") (TriggeredSeconds :type "Float (double-precision)") (InputAction :type "InputAction Object Reference" :default "/Game/FirstPerson/Input/Actions_Default/IA_Aim.IA_Aim"))
  (bind _ref_character (`self.Ref_Character`))
  ;[1 1 1] Aiming
  (:`Started`
    (`/Game/FirstPerson/Blueprints/BP_FirstPersonCharacter.AimIn` _ref_character))
  (:`Completed`
    (`/Game/FirstPerson/Blueprints/BP_FirstPersonCharacter.AimOut` _ref_character)))

(fn `CalculateAimTarget`
  (returns (LookAtRotation :type "Rotator Structure"))
  (bind _ref_character (`self.Ref_Character`))
  (bind _firstpersoncamera (`/Game/FirstPerson/Blueprints/BP_FirstPersonCharacter.FirstPersonCamera` _ref_character))
  (bind _returnvalue (`SceneComponent.K2_GetComponentLocation` _firstpersoncamera))
  (bind (_outhit _returnvalue_2) (`KismetSystemLibrary.LineTraceSingle` _returnvalue (+ _returnvalue (* (`SceneComponent.GetForwardVector` _firstpersoncamera) 10000.0)) "TraceTypeQuery1" false (`|MakeArray` _ref_character :!type "Actor Object Reference")))
  (if _returnvalue_2
    (bind (_bblockinghit _binitialoverlap _time _distance _location _impactpoint _normal _impactnormal _physmat _hitactor _hitcomponent _hitbonename _bonename _hititem _elementindex _faceindex _tracestart _traceend) (`GameplayStatics.BreakHitResult` _outhit))
    ;[0 0 0] Hit
    (return (`KismetMathLibrary.FindLookAtRotation` (`SceneComponent.K2_GetComponentLocation` (`self.StaticMesh`)) _location))
    (else
      ;[0 0 0] No hit
      (return (`KismetMathLibrary.FindLookAtRotation` (`SceneComponent.K2_GetComponentLocation` (`self.StaticMesh`)) _traceend)))))

(fn `ThrowUnholster`
  (if (`/Game/FirstPerson/Blueprints/BP_FirstPersonCharacter.ItemHolstered` (`self.Ref_Character`))
    (`/Game/MyContent/Blueprints/Core/BP_PC_Default.ItemHolster` (`self.Ref_PC`))))

(fn `UserConstructionScript`)