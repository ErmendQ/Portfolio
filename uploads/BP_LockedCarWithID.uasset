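; Interactable car that, on its first interaction, plays a door-open sound and yields Zsuzsanna Virág Horváth's ID card.
; Shortly after BeginPlay, it moves the interactable component's indication sphere and widget to InteractionOrigin.
; InteractionA runs once, messaging a referenced actor, removing the prompt widget and disabling sphere collision.
; It spawns BP_ViragID at the Cube's transform and manually triggers that card's indication overlap with the player.
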(event `self.ReceiveBeginPlay`
  (`parent.ReceiveBeginPlay`)
  (`KismetSystemLibrary.Delay` 0.5)
  (`SceneComponent.K2_SetWorldLocation` (`/Game/MyContent/Blueprints/Components/BPC_Interactable.IndicationSphere` (`self.BPC_Interactable`)) (`SceneComponent.K2_GetComponentLocation` (`self.InteractionOrigin`)) false false)
  (`SceneComponent.K2_SetWorldLocation` (`/Game/MyContent/Blueprints/Components/BPC_Interactable.InteractionWidgetComp` (`self.BPC_Interactable`)) (`SceneComponent.K2_GetComponentLocation` (`self.InteractionOrigin`)) false false))

(event `self.InteractionA`
  (bind (_returnvalue_location _returnvalue_rotation) (`KismetMathLibrary.BreakTransform` (`SceneComponent.K2_GetComponentToWorld` (`self.Cube`))))
  (`/Engine/EditorBlueprintResources/StandardMacros.DoOnce` false
    (:`Completed`
      (message `/Game/MyContent/SurviivalHorrorInventory/BPI_Interaction.Interact` (`self.Actor`) null)
      (`ActorComponent.K2_DestroyComponent` (`/Game/MyContent/Blueprints/Components/BPC_Interactable.InteractionWidgetComp` (`self.BPC_Interactable`)))
      (`PrimitiveComponent.SetCollisionProfileName` (`self.Sphere`) "NoCollision" true)
      (bind _returnvalue (`|SpawnActorFromClass` "/Game/MyContent/Blueprints/Docs/BP_ViragID.BP_ViragID_C" (`KismetMathLibrary.MakeTransform` _returnvalue_location _returnvalue_rotation) "Undefined" "MultiplyWithRoot" null "ID Card" "Name: Zsuzsanna Virág Horváth \n \nSex: F \n \nDate of birth: 11.09.2000 \n \nID Number: 098061" false null))
      (`/Game/MyContent/Blueprints/Components/BPC_Interactable.IndicationSphereOverlap` :`self` (`/Game/MyContent/Blueprints/Docs/BP_DocumentMaster.BPC_Interactable` _returnvalue) :`OtherActor` (`GameplayStatics.GetPlayerCharacter` 0))
      (`GameplayStatics.PlaySoundAtLocation` "/Game/MyContent/Audio/SC_CarDoorOpen.SC_CarDoorOpen" (`self.K2_GetActorLocation`) (struct) 1.0 1.0 0.0 null null null null))))

(fn `UserConstructionScript`
  (`parent.UserConstructionScript`))