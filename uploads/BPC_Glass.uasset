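; Actor component for drinking glasses that handles pouring, consuming, emptying, dirt buildup, cleaning and drink spoilage.
; Fill volume, capped by DT_Items, drives the tagged liquid mesh's material, with drink colors HSV-blended by volume and contained types recorded.
; Pouring starts a looping timer that eventually swaps beer foam for flies.
; RepNotifies on foam, flies and dirtiness update the owner's tagged Niagara effects and glass tint.
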(event `self.ReceiveBeginPlay`
  (bind _returnvalue (`self.GetOwner`))
  ;[0 0 0 1 98] Begin play - setup
  (`|ExecutionSequence`
    (:`then_0`
      ;;[1 1 1] Set glass volume based on data table value
      (bind _returnvalue_2 (message `/Game/Blueprints/Interfaces/BPI_Interactable.GetItemType` _returnvalue))
      (bind _returnvalue_3 (`|GetDataTableRow` "/Game/Blueprints/DataTables/DT_Items.DT_Items" (`KismetStringLibrary.Conv_StringToName` (`|GetEnumeratorNameAsString` _returnvalue_2)))
        (:`then`
          (set `self.MaxVolume` (`.Liquid_Volume_80_D54AA3054BD484B0A47D5EA08B507F56` (break `/Game/Blueprints/DataTables/Structs/S_Item2` _returnvalue_3))))))
    (:`then_1`
      ;;[1 1 1] Create reference to liquid mesh and set fill to 0
      (set `self.LiquidMesh` (`|GetArrayItem` (`Actor.GetComponentsByTag` _returnvalue "/Script/Engine.StaticMeshComponent" "Liquid")))
      (set `self.CurrentVolume` 0.0)
      (`self.RefreshFillMaterial&Mesh` "NewEnumerator0"))
    (:`then_2`
      (`self.RefreshGlassMaterial`))))

(event `Fill`
  (params (DrinkType :type "/Game/Blueprints/Enums/E_DrinkTypes Enum" :default "NewEnumerator0") (PressureMultiplier :type "Float (double-precision)"))
  (bind _returnvalue (/ PressureMultiplier 10.0))
  ;[0.1094 0.1094 0.1094] Fill 10ml || 10 volume || 1 second of pouring || 1cl || 1/4 shot glass || 1/500 beer || 1/100 wine || 1 unit ingredient
  (set `self.CurrentVolume` (`KismetMathLibrary.FClamp` (+ (`self.CurrentVolume`) _returnvalue) 0.0 (`self.MaxVolume`)))
  (`self.RefreshFillMaterial&Mesh` DrinkType _returnvalue)
  (`|ExecutionSequence`
    (:`then_0`
      ;[0 1 1] Spawn beer foam at top of the liquid (turn off on repeated pours)
      (set `self.FoamOn?` false)
      (`KismetSystemLibrary.RetriggerableDelay` 0.5)
      (set `self.FoamOn?` true))
    (:`then_1`
      ;[0 0 0 1 30] Start degradation timer after drink poured
      (`/Engine/EditorBlueprintResources/StandardMacros.DoOnce` false :!label _label
        (:`Completed`
          (if (`KismetSystemLibrary.K2_IsValidTimerHandle` (`self.DrinkDegradationTimer`))
            (`KismetSystemLibrary.K2_ClearAndInvalidateTimerHandle` (`self.DrinkDegradationTimer`)))
          (bind _returnvalue_2 (`KismetSystemLibrary.K2_SetTimerDelegate` (delegate `DrinkDegradation`) 1.0 true))
          (set `self.DrinkDegradationTimer` _returnvalue_2)
          (set `self.SecondsSincePoured` 0))))))

(event `DrinkDegradation`
  ;[0 0 0 1 30] Start degradation timer after drink poured
  ;; Start Drink Degradation
  (bind _result (`/Engine/EditorBlueprintResources/StandardMacros.IncrementInt` (`self.SecondsSincePoured`))
    (:`  `
      (if (> _result (`self.SecondsForDrinkToGoBad`))
        (`|ExecutionSequence`
          (:`then_0`
            (set `self.FliesOn?` true))
          (:`then_1`
            (set `self.FoamOn?` false)))))))

(event `Consume`
  (params (Amount :type "Float (double-precision)"))
  ;[0 0 0 1 30] Consume (as customer or player)
  (set `self.CurrentVolume` (`KismetMathLibrary.FClamp` (- (`self.CurrentVolume`) Amount) 0.0 (`self.MaxVolume`)))
  (`self.MC_ConsumeShowAll`))

(event `MC_ConsumeShowAll`
  ;[0 0 0 1 30] Consume (as customer or player)
  (`|ExecutionSequence`
    (:`then_0`
      (if (> (`self.CurrentVolume`) 1.0)
        (`self.RefreshFillMaterial&Mesh` "NewEnumerator0")
        (else
          (`self.Empty`))))
    (:`then_1`
      (`/Engine/EditorBlueprintResources/StandardMacros.DoOnce` false :!label _label_2
        (:`Completed`
          (set `self.FoamOn?` false)
          (set `self.FliesOn?` false)
          (`KismetSystemLibrary.K2_ClearAndInvalidateTimerHandle` (`self.DrinkDegradationTimer`)))))))

(event `StopDrinkDegradation`
  ;[0 0 0 1 30] Start degradation timer after drink poured
  ;; Stop the Degration Timer
  (`KismetSystemLibrary.K2_ClearAndInvalidateTimerHandle` (`self.DrinkDegradationTimer`)))

(event `Empty`
  ;[0 0 0 1 30] EmptyGlass
  (set `self.CurrentVolume` 0.0)
  (`self.RefreshFillMaterial&Mesh` "NewEnumerator0")
  (`KismetArrayLibrary.Array_Clear` (`self.DrinkTypesContained`))
  (`|ExecutionSequence`
    (:`then_0`
      (goto _label_2 :!via `Reset`))
    (:`then_1`
      (goto _label :!via `Reset`))))

(event `Clean`
  (params (Amount :type "Float (double-precision)"))
  ;[0 0 0 1 30] Clean the Glass
  (set `self.GlassDirtyness` (`KismetMathLibrary.FClamp` (- (`self.GlassDirtyness`) Amount)))
  (`self.Empty`)
  (`self.RefreshGlassMaterial`)
  (`|ExecutionSequence`
    (:`then_0`
      (set `self.FliesOn?` false))
    (:`then_1`
      (set `self.FoamOn?` false))))

(event `DirtyBuildup`
  (params (Amount :type "Float (double-precision)"))
  ;[0 0 0 1 30] Call to apply dirt buildup
  (set `self.GlassDirtyness` (`KismetMathLibrary.FClamp` (+ (`self.GlassDirtyness`) Amount)))
  (`self.RefreshGlassMaterial`))

(fn `OnRep_FliesOn?`
  (`self.ToggleFlies` (`self.FliesOn?`)))

(fn `OnRep_FoamOn?`
  (`self.ToggleFoam` (`self.FoamOn?`)))

(fn `OnRep_GlassDirtyness`
  (`self.RefreshGlassMaterial`))

(fn `RefreshFillMaterial&Mesh`
  (params (DrinkType :type "/Game/Blueprints/Enums/E_DrinkTypes Enum" :default "NewEnumerator0") (VolumeAdded :type "Float (double-precision)"))
  (bind _liquidmesh (`self.LiquidMesh`))
  (bind _returnvalue (`KismetMathLibrary.MapRangeUnclamped` (`self.CurrentVolume`) 0.0 (`self.MaxVolume`) 0.0 1.0))
  (`|ExecutionSequence`
    (:`then_0`
      ;[1 1 1] Calculate fill progress and apply to material
      (`MeshComponent.SetScalarParameterValueOnMaterials` (`self.LiquidMesh`) "Fill" _returnvalue)
      ;[1 1 1] If empty, hide mesh. If refilled, show mesh
      (if (< _returnvalue 0.01)
        (`/Engine/EditorBlueprintResources/StandardMacros.DoOnce` false :!label _label
          (:`Completed`
            (`SceneComponent.SetVisibility` _liquidmesh false false)
            (goto _label_2 :!via `Reset`)))
        (else
          (`/Engine/EditorBlueprintResources/StandardMacros.DoOnce` false :!label _label_2
            (:`Completed`
              (`SceneComponent.SetVisibility` _liquidmesh true false)
              (goto _label :!via `Reset`))))))
    (:`then_1`
      ;[1 1 1] Skip color and array if drink type is none
      (if (`|EnumInequality` DrinkType "NewEnumerator0")
        ;[1 1 1] If add to drinks array if not already contained
        (if (not (`KismetArrayLibrary.Array_Contains` (`self.DrinkTypesContained`) DrinkType))
          (`KismetArrayLibrary.Array_Add` (`self.DrinkTypesContained`) DrinkType))
        ;[1 1 1] Set color of drinks based on mix
        (bind _returnvalue_2 (`|GetDataTableRow` "/Game/Blueprints/DataTables/DT_DrinkTypes.DT_DrinkTypes" (`KismetStringLibrary.Conv_StringToName` (`|GetEnumeratorNameAsString` DrinkType)))
          (:`then`
            (bind _returnvalue_3 (`KismetMathLibrary.LinearColorLerpUsingHSV` (`self.DrinkColor`) (`KismetMathLibrary.Conv_ColorToLinearColor` (`.Color_22_A7F580704C3BA7C8009C3AB9F719A5F7` (break `/Game/Blueprints/DataTables/Structs/S_DrinkType` _returnvalue_2))) (/ VolumeAdded (`self.CurrentVolume`))))
            (set `self.DrinkColor` _returnvalue_3)
            (`MeshComponent.SetVectorParameterValueOnMaterials` (`self.LiquidMesh`) "Color" (`KismetMathLibrary.Conv_LinearColorToVector` _returnvalue_3))))))))

(fn `RefreshGlassMaterial`
  (bind _output (`|GetArrayItem` (`Actor.GetComponentsByTag` (`self.GetOwner`) "/Script/Engine.StaticMeshComponent" "Glass")))
  (`/Engine/EditorBlueprintResources/StandardMacros.IsValid` _output
    (:`Is Valid`
      (`MeshComponent.SetColorParameterValueOnMaterials` _output "BaseColorFactor" (`KismetMathLibrary.LinearColorLerp` (struct :`R` 0.630757 :`G` 0.597202 :`B` 0.597202 :`A` 0.270588) (struct :`R` 0.046875 :`G` 0.022602 :`A` 1.0) (`self.GlassDirtyness`))))))

(fn `ToggleFlies`
  (params (`Active?` :type Boolean))
  (bind _output (`|GetArrayItem` (`Actor.GetComponentsByTag` (`self.GetOwner`) "/Script/Niagara.NiagaraComponent" "Flies")))
  (`/Engine/EditorBlueprintResources/StandardMacros.IsValid` (`|GetArrayItem` (`Actor.GetComponentsByTag` (`self.GetOwner`) "/Script/Niagara.NiagaraComponent" "Flies"))
    (:`Is Valid`
      (if `Active?`
        ; Activate the flies
        (`self.Activate` _output false)
        (else
          ; Deactivate the flies
          (if (`self.IsActive` _output)
            (`self.Deactivate` _output)))))))

(fn `ToggleFoam`
  (params (`Active?` :type Boolean))
  (bind _output (`|GetArrayItem` (`Actor.GetComponentsByTag` (`self.GetOwner`) "/Script/Niagara.NiagaraComponent" "BeerFoam")))
  (`/Engine/EditorBlueprintResources/StandardMacros.IsValid` (`|GetArrayItem` (`Actor.GetComponentsByTag` (`self.GetOwner`) "/Script/Niagara.NiagaraComponent" "BeerFoam"))
    (:`Is Valid`
      (if `Active?`
        ; Activate and set position of foam
        (`self.Activate` _output false)
        (`SceneComponent.K2_SetRelativeLocation` _output (`KismetMathLibrary.MakeVector` 0.0 0.0 (`KismetMathLibrary.MapRangeClamped` (`self.CurrentVolume`) 0.0 (`self.MaxVolume`) 2.0 20.0)) false false)
        (else
          ; Deactivate the Foam
          (if (`self.IsActive` _output)
            (`self.Deactivate` _output)))))))