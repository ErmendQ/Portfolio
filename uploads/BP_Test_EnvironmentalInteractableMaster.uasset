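; Base actor for environmental interactables that players toggle directly or first unlock by lockpick, item, numpad or hacking.
; LookAt moves a world-space widget to the hit point and shows it via retriggerable delay, listing options built from lock state or an override.
; Interactions route through server to multicast events, branching on the chosen option.
; Unlocking refreshes the widget and calls Toggle, which fires empty ToggleOn/ToggleOff hooks for children.
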(event `LookedAt`
  ;[1 1 1] Looked at widget appear/disappear
  (`|ExecutionSequence`
    (:`then_0`
      (bind _widget (`self.Widget`)
        (:`then`
          (`SceneComponent.SetVisibility` _widget true false))
        (:`else`)))
    (:`then_1`
      (`KismetSystemLibrary.RetriggerableDelay` 0.01)
      (bind _widget_2 (`self.Widget`)
        (:`then`
          (`SceneComponent.SetVisibility` _widget_2 false false))
        (:`else`)))))

(event `self.ReceiveBeginPlay`
  (bind _widget (`self.Widget`))
  ;[0 0.04678 1] Begin play
  (`/Engine/EditorBlueprintResources/StandardMacros.IsValid` _widget
    (:`Is Valid`
      (bind _asw_world_space_interaction (cast `/Game/MyContent/UI/W_WorldSpaceInteraction` (`WidgetComponent.GetWidget` _widget)))
      (set `self.Ref_TextWidget` _asw_world_space_interaction)
      (`self.UpdateWidgetText`))))

(event `UpdateWidgetText`
  (bind _ref_textwidget (`self.Ref_TextWidget`))
  (bind _ref_textwidget_2 (`self.Ref_TextWidget`))
  (bind _ref_textwidget_3 (`self.Ref_TextWidget`))
  (bind _interactiontypes (`self.InteractionTypes`))
  ;[1 1 1] Widget text setup
  (`|ExecutionSequence`
    (:`then_0`
      (`/Engine/EditorBlueprintResources/StandardMacros.IsValid` (`self.Ref_TextWidget`)
        (:`Is Valid`
          (if (not (`self.Override_WidgetText`))
            (if (`self.Unlocked`)
              ;;[0 0 0] Set default text
              (`KismetArrayLibrary.Array_Clear` (`self.InteractionTypes`))
              (`KismetArrayLibrary.Array_Clear` (`/Game/MyContent/UI/W_WorldSpaceInteraction.Interactions` _ref_textwidget_3))
              (`KismetArrayLibrary.Array_Add` (`self.InteractionTypes`) (`self.BaseInteraction`))
              (set `/Game/MyContent/UI/W_WorldSpaceInteraction.Name` (`KismetTextLibrary.Conv_NameToText` (`self.Name`)) _ref_textwidget_3)
              (set `/Game/MyContent/UI/W_WorldSpaceInteraction.IsLocked` false _ref_textwidget_3)
              (set `/Game/MyContent/UI/W_WorldSpaceInteraction.Interactions` (`self.InteractionTypes`) (`self.Ref_TextWidget`))
              (else
                ;;[0 0 0] Set locked interaction types
                (set `/Game/MyContent/UI/W_WorldSpaceInteraction.Name` (`KismetTextLibrary.Conv_NameToText` (`self.Name`)) _ref_textwidget_2)
                (set `/Game/MyContent/UI/W_WorldSpaceInteraction.IsLocked` true _ref_textwidget_2)
                (`KismetArrayLibrary.Array_Clear` _interactiontypes)
                (`KismetArrayLibrary.Array_Add` _interactiontypes (`self.BaseInteraction`))
                (`|ExecutionSequence`
                  (:`then_0`
                    (if (`self.CanLockpick`)
                      (`KismetArrayLibrary.Array_Add` (`self.InteractionTypes`) "NewEnumerator4")))
                  (:`then_1`
                    (if (`self.ItemUnlock`)
                      (`KismetArrayLibrary.Array_Add` (`self.InteractionTypes`) "NewEnumerator9")))
                  (:`then_2`
                    (if (`self.Hackable`)
                      (`KismetArrayLibrary.Array_Add` (`self.InteractionTypes`) "NewEnumerator5")))
                  (:`then_3`
                    (if (`self.Numpad`)
                      (`KismetArrayLibrary.Array_Add` (`self.InteractionTypes`) "NewEnumerator13")))
                  (:`then_4`
                    (set `/Game/MyContent/UI/W_WorldSpaceInteraction.Interactions` (`self.InteractionTypes`) (`self.Ref_TextWidget`))))))
            (else
              ;;[0 0 0] Override
              (set `/Game/MyContent/UI/W_WorldSpaceInteraction.Interactions` (`|MakeArray` (`self.Override_Action`)) _ref_textwidget)
              (set `/Game/MyContent/UI/W_WorldSpaceInteraction.Name` (`self.Override_Name`) _ref_textwidget)
              (set `/Game/MyContent/UI/W_WorldSpaceInteraction.IsLocked` false _ref_textwidget))))))))

(event `/Game/MyContent/Blueprints/Interfaces/BI_Interaction.Interaction`
  (params (Interactor :type "/Game/MyContent/Blueprints/Core/BP_PC_Default Object Reference") (Inventory :type "Array of /Game/MyContent/Blueprints/Enums/E_Items Enum (by ref)" :default _) (Proceed :type Boolean) (InteractionOptionIndex :type Integer))
  ;[1 1 1 1 30] Interaction
  ;;[0 0 0] Interaction interface call
  (if (not (`self.Busy`))
    (`self.Server_Interaction` Interactor Proceed InteractionOptionIndex)))

(event `Server_Interaction`
  (params (BP_PC :type "/Game/MyContent/Blueprints/Core/BP_PC_Default Object Reference") (Proceed :type Boolean) (InteractionOption :type Integer))
  ;[1 1 1 1 30] Interaction
  ;;[0 0 0] Server Interaction
  (`self.Multi_Interaction` BP_PC Proceed InteractionOption))

(event `Multi_Interaction`
  (params (BP_PC :type "/Game/MyContent/Blueprints/Core/BP_PC_Default Object Reference") (Proceed :type Boolean) (InteractionOption :type Integer))
  (bind _unlockitem (`self.UnlockItem`))
  (bind _output (`|GetArrayItem` (`self.InteractionTypes`) InteractionOption))
  ;[1 1 1 1 30] Interaction
  (`/Engine/EditorBlueprintResources/StandardMacros.IsValid` BP_PC
    (:`Is Valid`
      (bind _output_get (set `self.MC_Ref_PC` BP_PC))
      (if (or Proceed (`self.Unlocked`))
        (`self.Toggle` _output_get)
        (else
          ;;[0 0 0] Check for interaction type
          (if (`|EnumEquality` _output "NewEnumerator4")
            ;;[0 0 0] Lockpick
            (bind _returnvalue (`/Game/MyContent/Blueprints/Core/BP_PC_Default.HasItem?` _output_get "NewEnumerator4"))
            (if _returnvalue
              (`/Game/LockPicking/Blueprints/BP_LockPickingComponent.PickLock` (`self.BP_LockPickingComponent`) (select `/Game/MyContent/Blueprints/Enums/E_MinigameDifficulties` (`self.LockpickingDifficulty`) :`NewEnumerator0` 3 :`NewEnumerator1` 3 :`NewEnumerator2` 2 :`NewEnumerator3` 1 :`NewEnumerator4` 1) self _output_get)
              (set `/Game/MyContent/Blueprints/Core/BP_PC_Default.InteractionRange` 0.0 _output_get) ; Disable interaction trace
              (`/Game/MyContent/Blueprints/Core/BP_PC_Default.SRV_SetBusy` _output_get self true)
              (else
                (bind _ref_playercharacter (`/Game/MyContent/Blueprints/Core/BP_PC_Default.Ref_PlayerCharacter` _output_get)
                  (:`then`
                    (`/Game/FirstPerson/Blueprints/BP_FirstPersonCharacter.FeedbackMessage` _ref_playercharacter "" "NewEnumerator0" "NewEnumerator2" "NewEnumerator0" "NewEnumerator4"))
                  (:`else`))))
            (elif (`|EnumEquality` _output "NewEnumerator9")
              ;;[0 0 0] Item unlock / proceed
              (if (`KismetArrayLibrary.Array_Contains` (`/Game/MyContent/Blueprints/Core/BP_PC_Default.Items` _output_get) _unlockitem)
                (set `self.UsedItem` _unlockitem)
                (bind _success (`/Game/MyContent/Blueprints/Core/BP_PC_Default.UseItem` _output_get _unlockitem false))
                (if _success
                  (set `self.Unlocked` true :!label _label)
                  (`self.Toggle` (select `bool` (`KismetSystemLibrary.IsValid` _output_get) :`false` (stale `MC_Unlock` BP_PC) :`true` _output_get))
                  (`self.ED_Unlocked`)
                  (`self.UpdateWidgetText`)
                  (`/Game/MyContent/UI/W_WorldSpaceInteraction.Update` (`self.Ref_TextWidget`)))
                (else
                  (bind _ref_playercharacter_2 (`/Game/MyContent/Blueprints/Core/BP_PC_Default.Ref_PlayerCharacter` _output_get)
                    (:`then`
                      (`/Game/FirstPerson/Blueprints/BP_FirstPersonCharacter.FeedbackMessage` _ref_playercharacter_2 "" "NewEnumerator0" "NewEnumerator2" "NewEnumerator0" (`self.UnlockItem`)))
                    (:`else`))))
              (elif (`|EnumEquality` _output "NewEnumerator13")
                (`/Game/MyContent/Blueprints/Core/BP_PC_Default.OpenNumpad` _output_get self)
                (elif (`|EnumEquality` _output "NewEnumerator5")
                  (bind _returnvalue_2 (`/Game/MyContent/Blueprints/Core/BP_PC_Default.HasItem?` _output_get "NewEnumerator21"))
                  (if _returnvalue_2
                    (`/Game/MyContent/Blueprints/Core/BP_PC_Default.UseItem` _output_get "NewEnumerator21" false)
                    (`self.Unlock` _output_get)
                    (`self.Toggle` _output_get) ; Avoid widget error and stay closed
                    (else
                      (`/Game/MyContent/Blueprints/Core/BP_PC_Default.StartHacking` _output_get self (select `/Game/MyContent/Blueprints/Enums/E_MinigameDifficulties` (`self.Hackdifficulty`) :`NewEnumerator0` 20 :`NewEnumerator1` 25 :`NewEnumerator2` 30 :`NewEnumerator3` 35 :`NewEnumerator4` 40))))
                  (else
                    (bind _ref_playercharacter_3 (`/Game/MyContent/Blueprints/Core/BP_PC_Default.Ref_PlayerCharacter` _output_get) ; Trying to open/use while locked
                      (:`then`
                        (`/Game/FirstPerson/Blueprints/BP_FirstPersonCharacter.FeedbackMessage` _ref_playercharacter_3 "" "NewEnumerator0" "NewEnumerator3" "NewEnumerator0" "NewEnumerator4"))
                      (:`else`))))))))))))

(event `LockpickOpened`
  (params (DestroyedActor :type "Actor Object Reference"))
  (bind _ref_pc (`self.Ref_PC`))
  ;[1 1 1 1 30] Interaction
  ;;[0 0 0] Lockpick opened/quit
  (`/Game/MyContent/Blueprints/Core/BP_PC_Default.SRV_UnlockDoor` (`self.Ref_PC`) self)
  (`/Game/MyContent/Blueprints/Core/BP_PC_Default.SRV_TraceLengthReset` _ref_pc)
  (`/Game/MyContent/Blueprints/Core/BP_PC_Default.SRV_SetBusy` _ref_pc self false))

(event `LockpickQuit`
  (bind _ref_pc (`self.Ref_PC`))
  ;[1 1 1 1 30] Interaction
  ;;[0 0 0] Lockpick opened/quit
  (`/Game/MyContent/Blueprints/Core/BP_PC_Default.SRV_TraceLengthReset` _ref_pc)
  (`/Game/MyContent/Blueprints/Core/BP_PC_Default.SRV_SetBusy` _ref_pc self false))

(event `MC_Unlock`
  (params (BP_PC :type "/Game/MyContent/Blueprints/Core/BP_PC_Default Object Reference"))
  ;[1 1 1 1 30] Interaction
  ;;[0 0 0] Item unlock / proceed
  (goto _label))

(event `Unlock`
  (params (BP_PC :type "/Game/MyContent/Blueprints/Core/BP_PC_Default Object Reference"))
  ;[1 1 1 1 30] Interaction
  ;;[0 0 0] Item unlock / proceed
  (`self.SRV_Unlock` BP_PC))

(event `SRV_Unlock`
  (params (BP_PC :type "/Game/MyContent/Blueprints/Core/BP_PC_Default Object Reference"))
  ;[1 1 1 1 30] Interaction
  ;;[0 0 0] Item unlock / proceed
  (`self.MC_Unlock` BP_PC))

(event `Toggle`
  (params (BP_PC :type "/Game/MyContent/Blueprints/Core/BP_PC_Default Object Reference"))
  ;[1 1 1 1 30] Interaction
  ;;[0 0 0] Toggle
  (if (`self.IsToggle`)
    (if (`self.On`)
      (set `self.On` false)
      (`self.ToggleOff` BP_PC)
      (else
        (set `self.On` true :!label _label_2)
        (`self.ToggleOn` BP_PC)))
    (else
      (goto _label_2))))

(event `ToggleOff`
  (params (BP_PC :type "/Game/MyContent/Blueprints/Core/BP_PC_Default Object Reference"))
  ;[1 1 1 1 30] Interaction
  ;;[0 0 0] Toggle
)

(event `ToggleOn`
  (params (BP_PC :type "/Game/MyContent/Blueprints/Core/BP_PC_Default Object Reference"))
  ;[1 1 1 1 30] Interaction
  ;;[0 0 0] Toggle
)

(fn `GetInteractionsAmount`
  (returns (Amount :type Integer))
  (return (`KismetArrayLibrary.Array_Length` (`self.InteractionTypes`))))

(fn `Lockpicking_HideUI`
  (bind _ref_pc (`self.Ref_PC`))
  (if (and (`|EnumEquality` (`self.UnlockItem`) "NewEnumerator4") (`|EnumEquality` (`|GetArrayItem` (`/Game/MyContent/Blueprints/Core/BP_PC_Default.Items` _ref_pc) (`/Game/MyContent/Blueprints/Core/BP_PC_Default.SelectedItemIndex` _ref_pc)) "NewEnumerator4") (`self.ItemUnlock`) (not (`self.Unlocked`)))
    (set `Widget.Visibility` "Hidden" (`WidgetComponent.GetWidget` (`self.Widget`)))))

(fn `LookAt`
  (params (Examiner :type "/Game/MyContent/Blueprints/Core/BP_PC_Default Object Reference") (HitLocation :type "Vector Structure"))
  (returns (InteractionType :type "/Game/MyContent/Blueprints/Enums/E_InteractionTypes Enum") (Name :type String) (CanAccess :type Boolean))
  (bind _output_get (set `self.Ref_PC` Examiner))
  (set `/Game/MyContent/UI/W_WorldSpaceInteraction.Ref_PC` _output_get (`self.Ref_TextWidget`))
  (bind _widget (`self.Widget`)
    (:`then`
      (`SceneComponent.K2_SetWorldLocation` _widget HitLocation false false)
      (`self.LookedAt`)
      (return "NewEnumerator0" "" false))
    (:`else`)))

(fn `UserConstructionScript`)