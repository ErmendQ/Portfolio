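; Base tray item that can be picked up and carries glasses in slots marked by "Position"-tagged scene components.
; Interact falls back to parent pickup for empty hands, otherwise snaps the held glass, or OtherActor when the held item type contains "Tray", into the first free slot.
; A quick fix disables collision after loading a carried tray.
; Use has the user drop the first attached actor.
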(event `/Game/Blueprints/Interfaces/BPI_Interactable.Interact`
  (params (Interactor :type "/Game/Blueprints/Core/BP_FirstPersonCharacter Object Reference") (HitData :type "HitResult Structure") (OtherActor :type "Actor Object Reference"))
  ;[0 1 0 1 30] Interact
  (bind _returnvalue (`/Game/Blueprints/Core/BP_FirstPersonCharacter.GetHeldItem` Interactor))
  (`/Engine/EditorBlueprintResources/StandardMacros.IsValid` _returnvalue ; Is player holding item?
    (:`Is Valid`
      (bind _returnvalue_2 (message `/Game/Blueprints/Interfaces/BPI_Interactable.GetItemType` _returnvalue))
      (bind _returnvalue_3 (select `bool` (and (`KismetSystemLibrary.IsValid` OtherActor) (`KismetStringLibrary.Contains` (`|GetEnumeratorNameAsString` _returnvalue_2) "Tray" false true)) :`false` _returnvalue :`true` OtherActor))
      ;;[0 0 0] Place glass on tray
      (`/Engine/EditorBlueprintResources/StandardMacros.IsValid` (`self.GetComponentByClass` _returnvalue_3 "/Game/Blueprints/Components/BPC_Glass.BPC_Glass_C") ; Is player holding glass
        (:`Is Valid`
          (for _array_element (`self.GetComponentsByTag` "/Script/Engine.SceneComponent" "Position")
            (`/Engine/EditorBlueprintResources/StandardMacros.IsValid` (`SceneComponent.GetChildComponent` _array_element 0) ; Spot isnt taken
              (:`Is Not Valid`
                (message `/Game/Blueprints/Interfaces/BPI_Interactable.Drop` _returnvalue_3 (`SceneComponent.K2_GetComponentLocation` _array_element) false false (struct) false true)
                (`self.K2_AttachToComponent` _returnvalue_3 _array_element "None" "SnapToTarget" "KeepRelative" "KeepWorld" true)
                (break))))
          ;[1 1 1] (quick fix) update collision when picking up glasses while holding tray
          (if (`KismetSystemLibrary.IsValid` (`SceneComponent.GetAttachParent` (`self.Mesh`)))
            (`/Game/Blueprints/Interfaces/BPI_Interactable.SetCollision` false)))))
    (:`Is Not Valid`
      ;;[0 0 0] Pick up tray
      (`parent.Interact` Interactor (struct) null) ; Regular interaction: pick up
    )))

(event `/Game/Blueprints/Interfaces/BPI_Interactable.Drop`
  (params (Location :type "Vector Structure") (WithoutCollision :type Boolean) (SetRotation :type Boolean) (NewRotation :type "Rotator Structure") (`Thrown?` :type Boolean) (`DisablePhysics?` :type Boolean))
  ;[0 1 0 1 30] Drop
  (`parent.Drop` Location WithoutCollision SetRotation NewRotation `Thrown?` `DisablePhysics?`))

(event `/Game/Blueprints/Interfaces/BPI_Interactable.Use`
  (params (User :type "/Game/Blueprints/Core/BP_FirstPersonCharacter Object Reference"))
  (bind _outactors (`self.GetAttachedActors` true true))
  (if (`KismetArrayLibrary.Array_IsNotEmpty` _outactors)
    (`/Game/Blueprints/Core/BP_FirstPersonCharacter.DropOtherActor` User (`|GetArrayItem` _outactors))))

(fn `UserConstructionScript`
  (`parent.UserConstructionScript`))