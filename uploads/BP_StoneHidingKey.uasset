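; BP_StoneHidingKey is an interactable stone that yields a key item when used.
; InteractionA plays the actor's sequence and removes its interaction widget and component, making it single-use.
; It then looks up the "Key" row in DT_Items and spawns an inspectable BP_ItemNew at its location, using the DisplayName as row name.
; It manually calls the new item's IndicationSphereOverlap with the player character.
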(event `self.InteractionA`
  (bind _bpc_interactable (`self.BPC_Interactable`))
  (`ActorSequenceComponent.PlaySequence` (`self.ActorSequence`))
  (`Widget.RemoveFromParent` (`/Game/MyContent/Blueprints/Components/BPC_Interactable.InteractionWidget` _bpc_interactable))
  (`ActorComponent.K2_DestroyComponent` (`/Game/MyContent/Blueprints/Components/BPC_Interactable.InteractionWidgetComp` _bpc_interactable))
  (`ActorComponent.K2_DestroyComponent` _bpc_interactable)
  (bind _returnvalue (`|GetDataTableRow` "/Game/MyContent/SurviivalHorrorInventory/Data/DT_Items.DT_Items" "Key")
    (:`then`
      (bind _returnvalue_2 (`|SpawnActorFromClass` "/Game/MyContent/Blueprints/BP_ItemNew.BP_ItemNew_C" (`KismetMathLibrary.MakeTransform` (`self.K2_GetActorLocation`)) "Undefined" "MultiplyWithRoot" null (make `DataTableRowHandle` "/Game/MyContent/SurviivalHorrorInventory/Data/DT_Items.DT_Items" (`KismetStringLibrary.Conv_StringToName` (`KismetTextLibrary.Conv_TextToString` (`.DisplayName_12_45CB9414481FDDB0F64A9D879DC96C15` (break `/Game/MyContent/SurviivalHorrorInventory/Data/S_Item` _returnvalue))))) 1 true null))
      (`/Game/MyContent/Blueprints/Components/BPC_Interactable.IndicationSphereOverlap` :`self` (`self.GetComponentByClass` _returnvalue_2 "/Game/MyContent/Blueprints/Components/BPC_Interactable.BPC_Interactable_C") :`OtherActor` (`GameplayStatics.GetPlayerCharacter` 0)))))

(fn `UserConstructionScript`
  (`parent.UserConstructionScript`))