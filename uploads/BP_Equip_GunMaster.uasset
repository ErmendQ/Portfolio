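; Base gun actor for the player that handles shoot and aim input, with fire modes including three-round burst and full auto.
; A per-tick camera trace aims the barrel at the view target, and shots spawn projectiles through the player character.
; DT_ItemPickups, keyed by ItemType, supplies fire rate, damage, noise, recoil and sound.
; Each shot adds muzzle flash, recoil, rumble and an extra-effect call, with a DoOnce and delay gating fire rate.
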(event `self.ReceiveTick`
  (params (DeltaSeconds :type "Float (single-precision)"))
  ;[0.08305 1 0] Tick
  (`self.SetAimTarget`))

(event `self.ReceiveBeginPlay`
  ;[0 0.1434 1] Begin play
  (`|ExecutionSequence`
    (:`then_0`
      ;[1 1 1] SetInput
      (`self.EnableInput` (`GameplayStatics.GetPlayerController` 0))
      ;[1 1 1] Ref PC
      (bind _asbp_pc_default (cast `/Game/MyContent/Blueprints/Core/BP_PC_Default` (`GameplayStatics.GetPlayerController` 0)))
      (bind _output_get (set `self.Ref_PC` _asbp_pc_default))
      (set `self.Ref_Character` (`/Game/MyContent/Blueprints/Core/BP_PC_Default.Ref_PlayerCharacter` _output_get)))
    (:`then_1`
      ;[1 1 1] Set fire rate
      (bind _returnvalue (`|GetDataTableRow` "/Game/MyContent/Databases/Items/DT_ItemPickups.DT_ItemPickups" (`KismetStringLibrary.Conv_StringToName` (`|GetEnumeratorNameAsString` (`self.ItemType`))))
        (:`then`
          (set `self.FireRate` (`.ShotDelay_48_546CE2D74666B810337CA0B966E0935A` (break `/Game/MyContent/Databases/Items/F_ItemPickup` _returnvalue))))))))

(event `EnhancedInput|/Game/FirstPerson/Input/Actions_Default/IA_Shoot`
  (params (ActionValue :type Boolean) (ElapsedSeconds :type "Float (double-precision)") (TriggeredSeconds :type "Float (double-precision)") (InputAction :type "InputAction Object Reference" :default "/Game/FirstPerson/Input/Actions_Default/IA_Shoot.IA_Shoot"))
  (bind _ref_pc (`self.Ref_PC`))
  (bind _returnvalue (and (not (`/Game/MyContent/Blueprints/Core/BP_PC_Default.ControllingOther` _ref_pc)) (`KismetSystemLibrary.IsValid` _ref_pc)))
  ;[1 0.4063 0.3165] FireWeapon
  (:`Triggered`
    (if _returnvalue
      (`/Engine/EditorBlueprintResources/StandardMacros.DoOnce` false :!label _label
        (:`Completed`
          (`self.ShootUnholster`)
          (if (`|EnumInequality` (`self.Firemode`) "NewEnumerator1")
            ;;[1 1 1] SpawnProjectile
            (`self.FireGun`)
            (`self.PlaySound`)
            ;;[1 1 1] ShotDelay - single/auto
            (`KismetSystemLibrary.Delay` (`self.FireRate`))
            (`self.ResetShot`)
            (else
              (`|ExecutionSequence`
                (:`then_0`
                  ;;[1 1 1] SpawnProjectile1
                  (`self.FireGun`)
                  (`self.PlaySound`)
                  (`KismetSystemLibrary.Delay` 0.1)
                  ;;[1 1 1] SpawnProjectile2
                  (`self.FireGun`)
                  (`KismetSystemLibrary.Delay` 0.1)
                  ;;[1 1 1] SpawnProjectile3
                  (`self.FireGun`))
                (:`then_1`
                  ;;[1 1 1] ShotDelay - burst
                  (`KismetSystemLibrary.Delay` (`self.FireRate`))
                  (`self.ResetShot`)))))))))
  (:`Ongoing`
    (if _returnvalue
      ;;[1 1 1] Is full auto
      (if (`|EnumEquality` (`self.Firemode`) "NewEnumerator2")
        (goto _label)))))

(event `ResetShot`
  ;[1 0.4063 0.3165] FireWeapon
  (goto _label :!via `Reset`))

(event `SetAimTarget`
  (bind _ref_character (`self.Ref_Character`))
  (bind _firstpersoncamera (`/Game/FirstPerson/Blueprints/BP_FirstPersonCharacter.FirstPersonCamera` _ref_character))
  (bind _returnvalue (`SceneComponent.K2_GetComponentLocation` _firstpersoncamera))
  ;[1 1 1] Bullet target trace
  (bind (_outhit _returnvalue_2) (`KismetSystemLibrary.LineTraceSingle` _returnvalue (+ _returnvalue (* (`SceneComponent.GetForwardVector` _firstpersoncamera) 10000.0)) "TraceTypeQuery1" false (`|MakeArray` _ref_character :!type "Actor Object Reference")))
  (if _returnvalue_2
    (bind (_bblockinghit _binitialoverlap _time _distance _location _impactpoint _normal _impactnormal _physmat _hitactor _hitcomponent _hitbonename _bonename _hititem _elementindex _faceindex _tracestart _traceend) (`GameplayStatics.BreakHitResult` _outhit))
    ;;[0 0 0] Hit
    (set `self.LookAtRotation` (`KismetMathLibrary.FindLookAtRotation` (`SceneComponent.K2_GetComponentLocation` (`self.BarrelEnd`)) _location))
    (else
      ;;[0 0 0] No hit
      (set `self.LookAtRotation` (`KismetMathLibrary.FindLookAtRotation` (`SceneComponent.K2_GetComponentLocation` (`self.BarrelEnd`)) _traceend)))))

(event `EnhancedInput|/Game/FirstPerson/Input/Actions_Default/IA_Aim`
  (params (ActionValue :type Boolean) (ElapsedSeconds :type "Float (double-precision)") (TriggeredSeconds :type "Float (double-precision)") (InputAction :type "InputAction Object Reference" :default "/Game/FirstPerson/Input/Actions_Default/IA_Aim.IA_Aim"))
  (bind _ref_character (`self.Ref_Character`))
  ;[1 1 1] Aiming
  (:`Started`
    (`/Game/FirstPerson/Blueprints/BP_FirstPersonCharacter.AimIn` _ref_character))
  (:`Completed`
    (`/Game/FirstPerson/Blueprints/BP_FirstPersonCharacter.AimOut` _ref_character)))

(fn `FireGun`
  (bind _ref_character (`self.Ref_Character`))
  (bind _returnvalue_location (`KismetMathLibrary.BreakTransform` (`SceneComponent.K2_GetComponentToWorld` (`self.BarrelEnd`))))
  (bind _returnvalue (`|GetDataTableRow` "/Game/MyContent/Databases/Items/DT_ItemPickups.DT_ItemPickups" (`KismetStringLibrary.Conv_StringToName` (`|GetEnumeratorNameAsString` (`self.ItemType`))))
    (:`then`
      (bind (_typeid _name _description _icon _staticmesh _pickupsound _equipactor _dropspawnactor _isgun _damage _shotdelay _recoil _meleeattackspeed _throwforce _throwactor _noise) (break `/Game/MyContent/Databases/Items/F_ItemPickup` _returnvalue))
      (`/Game/FirstPerson/Blueprints/BP_FirstPersonCharacter.ShootProjectile` _ref_character _returnvalue_location (`self.LookAtRotation`) _damage (`/Game/FirstPerson/Blueprints/BP_FirstPersonCharacter.Ref_PC` _ref_character) _noise)
      (`NiagaraFunctionLibrary.SpawnSystemAttached` "/Game/Ana/VFX/MuzzleFlash/NS_MuzzleFlash.NS_MuzzleFlash" (`self.BarrelEnd`) "None" (0.0 0.0 0.0) (struct :`Yaw` -90.0) "KeepRelativeOffset" true)
      (`self.Recoil`)
      (`PlayerController.K2_ClientPlayForceFeedback` (`self.Ref_PC`) "/Game/MyContent/ControllerVibration/FF_ShootGun.FF_ShootGun" "None" false false false)
      (`self.ExtraShotEffect`))))

(fn `PlaySound`
  (bind _returnvalue (`|GetDataTableRow` "/Game/MyContent/Databases/Items/DT_ItemPickups.DT_ItemPickups" (`KismetStringLibrary.Conv_StringToName` (`|GetEnumeratorNameAsString` (`self.ItemType`))))
    (:`then`
      (`GameplayStatics.PlaySound2D` (`.ShootSound_61_3178D72F41C10063E8F3DE8D0D3DB9C4` (break `/Game/MyContent/Databases/Items/F_ItemPickup` _returnvalue)) 1.0 1.0 0.0 null null))))

(fn `Recoil`
  (bind _ref_character (`self.Ref_Character`))
  (bind _returnvalue (`|GetDataTableRow` "/Game/MyContent/Databases/Items/DT_ItemPickups.DT_ItemPickups" (`KismetStringLibrary.Conv_StringToName` (`|GetEnumeratorNameAsString` (`self.ItemType`))))
    (:`then`
      (bind (_typeid _name _description _icon _staticmesh _pickupsound _equipactor _dropspawnactor _isgun _damage _shotdelay _recoil) (break `/Game/MyContent/Databases/Items/F_ItemPickup` _returnvalue))
      (`Pawn.AddControllerPitchInput` _ref_character (`KismetMathLibrary.RandomFloatInRange` (* _recoil -0.5)))
      (`Pawn.AddControllerYawInput` _ref_character (`KismetMathLibrary.RandomFloatInRange` (* -0.25 _recoil) (* 0.25 _recoil)))
      (`GameplayStatics.PlayWorldCameraShake` "/Game/MyContent/Blueprints/CameraShakes/BP_CameraShakeRecoil.BP_CameraShakeRecoil_C" (`self.K2_GetActorLocation`) 100.0 100.0))))

(fn `ShootUnholster`
  (if (`/Game/FirstPerson/Blueprints/BP_FirstPersonCharacter.ItemHolstered` (`self.Ref_Character`))
    (`/Game/MyContent/Blueprints/Core/BP_PC_Default.ItemHolster` (`self.Ref_PC`))))

(fn `UserConstructionScript`)