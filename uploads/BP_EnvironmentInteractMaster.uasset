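; Base Blueprint for environment interactables that can be locked behind a required inventory item.
; Interacting while locked opens the inventory in required-item mode; unlocking optionally consumes the item, closes the inventory and triggers the interaction.
; Empty InteractionA and InteractionB events act as hooks, alternating when toggle interaction is enabled.
; Construction applies camera offset, item table and prompt text, while BeginPlay pins the widget to a tagged component or actor origin.
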(event `self.ReceiveBeginPlay`
  (bind _output (`|GetArrayItem` (`self.GetComponentsByTag` "/Script/Engine.SceneComponent" "WidgetPos")))
  (bind _interactionwidgetcomp (`/Game/MyContent/Blueprints/Components/BPC_Interactable.InteractionWidgetComp` (`self.BPC_Interactable`)))
  ;[1 1 1] Prevent widget comp to move with camera
  (`KismetSystemLibrary.Delay` 0.2)
  (`/Engine/EditorBlueprintResources/StandardMacros.IsValid` _output
    (:`Is Valid`
      (`SceneComponent.K2_SetWorldLocation` _interactionwidgetcomp (`SceneComponent.K2_GetComponentLocation` _output) false false))
    (:`Is Not Valid`
      (`SceneComponent.K2_SetWorldLocation` _interactionwidgetcomp (`self.K2_GetActorLocation`) false false))))

(event `self.BPC_Interactable.InteractedWith`
  (params (BPC :type "/Game/MyContent/SurviivalHorrorInventory/BPC_SurvivalHorrorInventory Object Reference"))
  (bind _w_inventory (`/Game/MyContent/SurviivalHorrorInventory/BPC_SurvivalHorrorInventory.W_Inventory` BPC))
  (bind (_datatable _rowname) (break `DataTableRowHandle` (`self.RequiredItem`)))
  (if (`self.Locked`)
    ;[1 1 1] Switch camera, open inventory and search for correct item
    (set `self.BPC` BPC)
    (`/Game/MyContent/SurviivalHorrorInventory/BPC_SurvivalHorrorInventory.ToggleInventory` BPC)
    (`/Game/MyContent/SurviivalHorrorInventory/Widgets/W_Inventory.SwitchToItems` _w_inventory true)
    (set `/Game/MyContent/SurviivalHorrorInventory/Widgets/W_Inventory.UseRequiredItemMode` true _w_inventory)
    (bind _returnvalue (`|GetDataTableRow` _datatable _rowname)
      (:`then`
        (set `/Game/MyContent/SurviivalHorrorInventory/Widgets/W_Inventory.RequiredItem` _returnvalue _w_inventory)
        (set `/Game/MyContent/SurviivalHorrorInventory/Widgets/W_Inventory.ActorRequiringItem` self _w_inventory)))
    (else
      (if (`self.ToggleInteraction`) :!label _label
        (`/Engine/EditorBlueprintResources/StandardMacros.FlipFlop`
          (:`A`
            (`self.InteractionA`))
          (:`B`
            (`self.InteractionB`)))
        (else
          (`self.InteractionA`))))))

(event `self.BPC_Interactable.Unlocked`
  (bind _bpc (`self.BPC`))
  (bind (_datatable _rowname) (break `DataTableRowHandle` (`self.RequiredItem`)))
  ;[1 1 1] Unlock and trigger interaction (remove required item if set to consume)
  (set `self.Locked` false)
  (`|ExecutionSequence`
    (:`then_0`
      (if (`self.ConsumeRequiredItem`)
        (bind _returnvalue (`|GetDataTableRow` _datatable _rowname)
          (:`then`
            (`/Game/MyContent/SurviivalHorrorInventory/Widgets/W_Inventory.Remove1OfItemTypeFromInventory` (`/Game/MyContent/SurviivalHorrorInventory/BPC_SurvivalHorrorInventory.W_Inventory` _bpc) _returnvalue)))))
    (:`then_1`
      (`/Game/MyContent/SurviivalHorrorInventory/BPC_SurvivalHorrorInventory.ToggleInventory` _bpc)
      (goto _label))))

(event `InteractionA`)

(event `InteractionB`)

(fn `HUDInfo`
  (returns (DisplayInfo :type Boolean) (Name :type Text) (Texture :type "Texture2D Object Reference") (`Item?` :type Boolean) (Item :type "/Game/MyContent/SurviivalHorrorInventory/Data/S_Item Structure"))
  (return false "" null false))

(fn `UserConstructionScript`
  (bind _bpc_interactable (`self.BPC_Interactable`))
  (`|ExecutionSequence`
    (:`then_0`
      (`SceneComponent.K2_SetRelativeLocationAndRotation` (`self.Camera`) (`self.CameraOffset`) (`self.CameraRotation`) false false)
      (bind _structout (setmembers `DataTableRowHandle` :`StructRef` (`self.RequiredItem`) :`DataTable` "/Game/MyContent/SurviivalHorrorInventory/Data/DT_Items.DT_Items"))
      (set `self.RequiredItem` _structout)
      ;[1 1 1] Prevent user from selecting second slot
      (if (== (`.RowName` (break `DataTableRowHandle` (`self.RequiredItem`))) "SecondSlot")
        (setmembers `DataTableRowHandle` :`StructRef` (`self.RequiredItem`) :`RowName` "None")))
    (:`then_1`
      (set `/Game/MyContent/Blueprints/Components/BPC_Interactable.InteractionTypeText` (`self.Action`) _bpc_interactable)
      (set `/Game/MyContent/Blueprints/Components/BPC_Interactable.InteractionNameText` (`self.Name`) _bpc_interactable))))