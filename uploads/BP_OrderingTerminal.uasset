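; BP_OrderingTerminal is an interactable terminal where players order items for timed delivery.
; Interact calls UseOrderingTerminal on the interactor, and focus toggles an outline overlay; the item and ammo functions are stubs.
; PlaceOrder deducts the cost and starts a timer, then DeliverOrder spawns the items in a row at the BP_DeliverySpot location.
; Money changes and spawns go through SRV calls on the cached first player controller.
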(event `/Game/Blueprints/Interfaces/BPI_Interactable.Interact`
  (params (Interactor :type "/Game/Blueprints/Core/BP_FirstPersonCharacter Object Reference") (HitData :type "HitResult Structure") (OtherActor :type "Actor Object Reference"))
  (`/Game/Blueprints/Core/BP_FirstPersonCharacter.UseOrderingTerminal` Interactor))

(event `self.ReceiveBeginPlay`
  ;[0 1 0 1 50] Begin play
  ;;[1 1 1] Get delivery spot location
  (bind _returnvalue (`GameplayStatics.GetActorOfClass` "/Game/Blueprints/GlobalLogic/BP_DeliverySpot.BP_DeliverySpot_C"))
  (set `self.DeliverySpot` (`self.K2_GetActorLocation` _returnvalue))
  ;;[1 1 1] Controller
  (bind _asbp_player_controller (cast `/Game/Blueprints/Core/BP_PlayerController` (`GameplayStatics.GetPlayerController` 0)))
  (set `self.Ref_PlayerController` _asbp_player_controller))

(event `PlaceOrder`
  (params (Items :type "Array of Actor Class Reference") (Cost :type Integer))
  ;[0 1 1 1 30] Place/deliver order
  (set `self.DeliveryItems` Items)
  (`/Game/Blueprints/Core/BP_PlayerController.SRV_AdjustMoney` (`self.Ref_PlayerController`) (* Cost -1))
  (bind _returnvalue (`KismetSystemLibrary.K2_SetTimerDelegate` (delegate `DeliverOrder`) (`self.DeliveryTime`)))
  (set `self.DeliveryTimerHandle` _returnvalue))

(event `DeliverOrder`
  ;[0 1 1 1 30] Place/deliver order
  (for (_array_element _array_index) (`self.DeliveryItems`)
    (`/Game/Blueprints/Core/BP_PlayerController.SRV_SpawnActor` (`self.Ref_PlayerController`) _array_element (`KismetMathLibrary.MakeTransform` (+ (`self.DeliverySpot`) (`KismetMathLibrary.MakeVector` (* _array_index 10)))))
    (`KismetSystemLibrary.K2_ClearAndInvalidateTimerHandle` (`self.DeliveryTimerHandle`))))

(event `/Game/Blueprints/Interfaces/BPI_Interactable.UnFocus`
  (`MeshComponent.SetOverlayMaterial` (`self.Cube`) null))

(fn `Focus`
  (params (HitLocation :type "Vector Structure"))
  (returns (Location :type "Vector Structure") (Zoom :type Boolean) (ZoomAmountInFOV :type "Float (double-precision)"))
  (`MeshComponent.SetOverlayMaterial` (`self.Cube`) "/Game/OurContent/Jagoda/Materials/Outlines/MI_Outline.MI_Outline")
  (return (0.0 0.0 0.0) false 0.0))

(fn `GetAmmo`
  (returns (Return :type Integer))
  (return 0))

(fn `GetAmmoText`
  (returns (Return :type "TextRenderComponent Object Reference"))
  (return null))

(fn `GetItemProperties`
  (returns (Return :type "/Game/Blueprints/DataTables/Structs/S_Item2 Structure"))
  (return))

(fn `GetItemType`
  (returns (ReturnValue :type "/Game/Blueprints/Enums/E_Items Enum"))
  (return "NewEnumerator1"))

(fn `GetMaxAmmo`
  (returns (Return :type Integer))
  (return 0))

(fn `SetAmmo`
  (params (Amount :type Integer))
  (returns (Return :type Integer))
  (return 0))

(fn `UserConstructionScript`)