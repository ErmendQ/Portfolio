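; Card table minigame of blackjack-style 21 between the player and an AI opponent, played to a set number of wins.
; It spawns, shuffles and stacks 52 mesh cards, splitting off a five-card public pile, identified by position, that either side can draw from.
; Player input hits, public-hits or stands; EndTurn alternates turns and scores rounds.
; The opponent hits by count-based odds or takes useful public cards; exiting restores player control and camera.
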(event `PublicCardUsed`
  ;[1 1 1] Use public card
  (for _array_element (`self.Cards`) :!label _label
    (if (`self.IsPublicCard` _array_element)
      (`SceneComponent.K2_AddLocalOffset` _array_element (0.0 -2.0 0.0) false false)
      (`self.BreakSearchForTopPublicUsed`))))

(event `BreakSearchForTopPublicUsed`
  ;[1 1 1] Use public card
  (goto _label :!via `Break`))

(event `MoveTopPublicCard`
  ;[1 1 1] Reveal top 2 cards in public deck
  (for _array_element (`self.Cards`) :!label _label_2
    (if (`self.IsPublicCard` _array_element)
      (`SceneComponent.K2_AddLocalOffset` _array_element (0.0 -2.0 0.0) false false)
      (`self.BreakSearchForTopPublic`)))
  (`self.PlayerHit`)
  (`self.OppHit`)
  (set `self.PlayerStands` false)
  (set `self.OppStands` false))

(event `PlayerPublicHit`
  (bind (_relativelocation_x _relativelocation_y _relativelocation_z) (`KismetMathLibrary.BreakVector` (`SceneComponent.RelativeLocation` (`self.PlayerCardPos`))))
  ;[1 1 1] Public hit Player / Opp
  (for _array_element (`self.Cards`) :!label _label_3
    (if (`self.IsPublicCard` _array_element)
      (`self.BreakSearchForTopPublicPlayer`)
      (`SceneComponent.K2_SetRelativeLocation` _array_element (`KismetMathLibrary.MakeVector` _relativelocation_x (+ _relativelocation_y (* (`KismetArrayLibrary.Array_Length` (`self.PlayerCards`)) 7)) _relativelocation_z) false false)
      (`SceneComponent.K2_SetRelativeRotation` :`self` _array_element)
      (`KismetArrayLibrary.Array_Add` (`self.PlayerCards`) _array_element)
      (`self.RefreshCounters`)
      (`self.PublicCardUsed`)
      (bind _result (`/Engine/EditorBlueprintResources/StandardMacros.IncrementInt` (`self.PublicCardsUsed`))
        (:`  `
          (set `self.PublicCardsUsed` _result))))))

(event `BreakSearchForTopPublic`
  ;[1 1 1] Reveal top 2 cards in public deck
  (goto _label_2 :!via `Break`))

(event `BreakSearchForTopPublicPlayer`
  ;[1 1 1] Public hit Player / Opp
  (goto _label_3 :!via `Break`))

(event `CreatePublicDeck`
  (bind _cards (`self.Cards`))
  (bind _returnvalue (`KismetArrayLibrary.Array_Length` (`self.Cards`)))
  (bind (_relativelocation_x _relativelocation_y _relativelocation_z) (`KismetMathLibrary.BreakVector` (`SceneComponent.RelativeLocation` (`self.PublicDeckPos`))))
  ;[1 1 1] Public deck
  (bind _output_get (set `self.PublicCards` (`|MakeArray` (`|GetArrayItem` _cards (- _returnvalue 1)) (`|GetArrayItem` _cards (- _returnvalue 2)) (`|GetArrayItem` _cards (- _returnvalue 3)) (`|GetArrayItem` _cards (- _returnvalue 4)) (`|GetArrayItem` _cards (- _returnvalue 5)))))
  (for (_array_element _array_index) _output_get
    (`SceneComponent.K2_SetRelativeLocationAndRotation` :`self` _array_element :`NewLocation` (`KismetMathLibrary.MakeVector` _relativelocation_x _relativelocation_y (+ _relativelocation_z (* _array_index 0.1)))))
  (`self.MoveTopPublicCard`))

(event `PlayerHit`
  (bind _output (`self.GetTopCardOnDeck`))
  (bind (_relativelocation_x _relativelocation_y _relativelocation_z) (`KismetMathLibrary.BreakVector` (`SceneComponent.RelativeLocation` (`self.PlayerCardPos`))))
  ;[1 1 1] Hit Player/Opp
  (`SceneComponent.K2_SetRelativeLocation` _output (`KismetMathLibrary.MakeVector` _relativelocation_x (+ _relativelocation_y (* (`KismetArrayLibrary.Array_Length` (`self.PlayerCards`)) 7)) _relativelocation_z) false false)
  (`SceneComponent.K2_SetRelativeRotation` :`self` _output)
  (`KismetArrayLibrary.Array_Add` (`self.PlayerCards`) _output)
  (`self.RefreshCounters`))

(event `OppPublicHit`
  (bind (_relativelocation_x _relativelocation_y _relativelocation_z) (`KismetMathLibrary.BreakVector` (`SceneComponent.RelativeLocation` (`self.OppCardPos`))))
  ;[1 1 1] Public hit Player / Opp
  (for _array_element (`self.Cards`) :!label _label_4
    (if (`self.IsPublicCard` _array_element)
      (`self.BreakSearchForTopPublicOpp`)
      (`SceneComponent.K2_SetRelativeLocation` _array_element (`KismetMathLibrary.MakeVector` _relativelocation_x (+ _relativelocation_y (* (`KismetArrayLibrary.Array_Length` (`self.OppCards`)) 7)) _relativelocation_z) false false)
      (`SceneComponent.K2_SetRelativeRotation` :`self` _array_element)
      (`KismetArrayLibrary.Array_Add` (`self.OppCards`) _array_element)
      (`self.RefreshCounters`)
      (`self.PublicCardUsed`)
      (bind _result (`/Engine/EditorBlueprintResources/StandardMacros.IncrementInt` (`self.PublicCardsUsed`))
        (:`  `
          (set `self.PublicCardsUsed` _result))))))

(event `OppHit`
  (bind _output (`self.GetTopCardOnDeck`))
  (bind (_relativelocation_x _relativelocation_y _relativelocation_z) (`KismetMathLibrary.BreakVector` (`SceneComponent.RelativeLocation` (`self.OppCardPos`))))
  ;[1 1 1] Hit Player/Opp
  (`SceneComponent.K2_SetRelativeLocation` _output (`KismetMathLibrary.MakeVector` _relativelocation_x (+ _relativelocation_y (* (`KismetArrayLibrary.Array_Length` (`self.OppCards`)) 7)) _relativelocation_z) false false)
  (`SceneComponent.K2_SetRelativeRotation` :`self` _output)
  (`KismetArrayLibrary.Array_Add` (`self.OppCards`) _output)
  (`self.RefreshCounters`))

(event `Reset`
  ;[0 0.1429 1] Start / Reset
  (`SceneComponent.SetVisibility` (`self.Controls`) true false)
  (`SceneComponent.SetVisibility` (`self.Score`) true false)
  (`SceneComponent.SetVisibility` (`self.OppCount`) true false)
  (`SceneComponent.SetVisibility` (`self.PlayerCount`) true false)
  (`|ExecutionSequence`
    (:`then_0`
      ;[1 1 1] New cards
      (if (`KismetArrayLibrary.Array_IsNotEmpty` (`self.Cards`))
        (for _array_element (`self.Cards`)
          (`ActorComponent.K2_DestroyComponent` _array_element))
        (`KismetArrayLibrary.Array_Clear` (`self.Cards`))))
    (:`then_1`
      (`self.CreateCard`))
    (:`then_2`
      (`/Engine/EditorBlueprintResources/StandardMacros.DoOnce` false
        (:`Completed`
          (`KismetSystemLibrary.K2_SetTimerDelegate` (`|CreateDelegate` :!event `CheckForEndCondition`) 5.0 true true))))))

(event `BreakSearchForTopPublicOpp`
  ;[1 1 1] Public hit Player / Opp
  (goto _label_4 :!via `Break`))

(event `ShuffleCards`
  (bind (_relativelocation_x _relativelocation_y _relativelocation_z) (`KismetMathLibrary.BreakVector` (`SceneComponent.RelativeLocation` (`self.DeckPos`))))
  ;[1 1 1] ShuffleCards
  (bind _output (`/Game/Erik/SMs/Cards/NewMacroLibrary.ShuffleArray` (`self.Cards`) (`KismetMathLibrary.MakeRandomStream` (`KismetMathLibrary.RandomInteger` 2147483647)))
    (:`Out`
      (set `self.Cards` _output)
      (for (_array_element _array_index) _output
        (`SceneComponent.K2_SetRelativeLocation` _array_element (`KismetMathLibrary.MakeVector` _relativelocation_x _relativelocation_y (+ _relativelocation_z (* _array_index 0.1))) false false))
      (`self.CreatePublicDeck`))))

(event `RefreshCounters`
  ;[1 1 1] Refresh / Show card value count
  (set `self.PlayerCountValue` 0)
  (set `self.OppCountValue` 0)
  (for _array_element (`self.PlayerCards`)
    (bind _output_get (set `self.PlayerCountValue` (+ (`self.GetCardValue` _array_element) (`self.PlayerCountValue`))))
    (if (and (== _output_get 21) (not (`self.PlayerStands`)))
      (set `self.PlayerStands` true)
      (elif (> _output_get 21)
        (set `self.PlayerStands` true)
        (set `self.OppStands` true))))
  (for _array_element_2 (`self.OppCards`)
    (bind _output_get_2 (set `self.OppCountValue` (+ (`self.GetCardValue` _array_element_2) (`self.OppCountValue`))))
    (if (and (== _output_get_2 21) (not (`self.OppStands`)))
      (set `self.OppStands` true)
      (elif (> _output_get_2 21)
        (set `self.PlayerStands` true)
        (set `self.OppStands` true))))
  (`TextRenderComponent.K2_SetText` (`self.PlayerCount`) (`KismetTextLibrary.Conv_IntToText` (`self.PlayerCountValue`)))
  (`TextRenderComponent.K2_SetText` (`self.OppCount`) (`KismetTextLibrary.Conv_IntToText` (`self.OppCountValue`))))

(event `CreateCard`
  (bind (_relativelocation_x _relativelocation_y _relativelocation_z) (`KismetMathLibrary.BreakVector` (`SceneComponent.RelativeLocation` (`self.DeckPos`))))
  ;[1 1 1] Create deck of cards
  (if (!= (`self.CardCount`) 52)
    (bind _returnvalue (`AddComponent|NODE_AddStaticMeshComponent-1` :`RelativeTransform` (`KismetMathLibrary.MakeTransform` (`KismetMathLibrary.MakeVector` _relativelocation_x _relativelocation_y (+ _relativelocation_z (* (`self.CardCount`) 0.1))) (struct :`Roll` 180.0))))
    (`KismetArrayLibrary.Array_Add` (`self.Cards`) _returnvalue)
    (bind _result (`/Engine/EditorBlueprintResources/StandardMacros.IncrementInt` (`self.CardCount`))
      (:`  `
        (set `self.CardCount` _result)
        (`KismetSystemLibrary.Delay` 0.01)
        (`self.CreateCard`)))
    (else
      (for (_array_element _array_index) (`self.Cards`)
        (`StaticMeshComponent.SetStaticMesh` _array_element (select `int` _array_index :`0` "/Game/Erik/SMs/Cards/SM_S2.SM_S2" :`1` "/Game/Erik/SMs/Cards/SM_S2.SM_S2" :`2` "/Game/Erik/SMs/Cards/SM_S2.SM_S2" :`3` "/Game/Erik/SMs/Cards/SM_S2.SM_S2" :`4` "/Game/Erik/SMs/Cards/SM_S3.SM_S3" :`5` "/Game/Erik/SMs/Cards/SM_S3.SM_S3" :`6` "/Game/Erik/SMs/Cards/SM_S3.SM_S3" :`7` "/Game/Erik/SMs/Cards/SM_S3.SM_S3" :`8` "/Game/Erik/SMs/Cards/SM_S4.SM_S4" :`9` "/Game/Erik/SMs/Cards/SM_S4.SM_S4" :`10` "/Game/Erik/SMs/Cards/SM_S4.SM_S4" :`11` "/Game/Erik/SMs/Cards/SM_S4.SM_S4" :`12` "/Game/Erik/SMs/Cards/SM_S5.SM_S5" :`13` "/Game/Erik/SMs/Cards/SM_S5.SM_S5" :`14` "/Game/Erik/SMs/Cards/SM_S5.SM_S5" :`15` "/Game/Erik/SMs/Cards/SM_S5.SM_S5" :`16` "/Game/Erik/SMs/Cards/SM_S6.SM_S6" :`17` "/Game/Erik/SMs/Cards/SM_S6.SM_S6" :`18` "/Game/Erik/SMs/Cards/SM_S6.SM_S6" :`19` "/Game/Erik/SMs/Cards/SM_S6.SM_S6" :`20` "/Game/Erik/SMs/Cards/SM_S7.SM_S7" :`21` "/Game/Erik/SMs/Cards/SM_S7.SM_S7" :`22` "/Game/Erik/SMs/Cards/SM_S7.SM_S7" :`23` "/Game/Erik/SMs/Cards/SM_S7.SM_S7" :`24` "/Game/Erik/SMs/Cards/SM_S8.SM_S8" :`25` "/Game/Erik/SMs/Cards/SM_S8.SM_S8" :`26` "/Game/Erik/SMs/Cards/SM_S8.SM_S8" :`27` "/Game/Erik/SMs/Cards/SM_S8.SM_S8" :`28` "/Game/Erik/SMs/Cards/SM_S9.SM_S9" :`29` "/Game/Erik/SMs/Cards/SM_S9.SM_S9" :`30` "/Game/Erik/SMs/Cards/SM_S9.SM_S9" :`31` "/Game/Erik/SMs/Cards/SM_S9.SM_S9" :`32` "/Game/Erik/SMs/Cards/SM_S10.SM_S10" :`33` "/Game/Erik/SMs/Cards/SM_S10.SM_S10" :`34` "/Game/Erik/SMs/Cards/SM_S10.SM_S10" :`35` "/Game/Erik/SMs/Cards/SM_S10.SM_S10" :`36` "/Game/Erik/SMs/Cards/SM_SD.SM_SD" :`37` "/Game/Erik/SMs/Cards/SM_SD.SM_SD" :`38` "/Game/Erik/SMs/Cards/SM_SD.SM_SD" :`39` "/Game/Erik/SMs/Cards/SM_SD.SM_SD" :`40` "/Game/Erik/SMs/Cards/SM_SC.SM_SC" :`41` "/Game/Erik/SMs/Cards/SM_SC.SM_SC" :`42` "/Game/Erik/SMs/Cards/SM_SC.SM_SC" :`43` "/Game/Erik/SMs/Cards/SM_SC.SM_SC" :`44` "/Game/Erik/SMs/Cards/SM_SB.SM_SB" :`45` "/Game/Erik/SMs/Cards/SM_SB.SM_SB" :`46` "/Game/Erik/SMs/Cards/SM_SB.SM_SB" :`47` "/Game/Erik/SMs/Cards/SM_SB.SM_SB" :`48` "/Game/Erik/SMs/Cards/SM_SA.SM_SA" :`49` "/Game/Erik/SMs/Cards/SM_SA.SM_SA" :`50` "/Game/Erik/SMs/Cards/SM_SA.SM_SA" :`51` "/Game/Erik/SMs/Cards/SM_SA.SM_SA" :`52` null :!type "StaticMesh Object Reference")))
      (for (_array_element_2 _array_index_2) (`self.Cards`)
        (switch `int` (mod (+ _array_index_2 1) 4)
          (:`0`
            (`PrimitiveComponent.SetMaterial` _array_element_2 0 "/Game/Erik/SMs/Cards/M_CardGlow_Blue.M_CardGlow_Blue"))
          (:`1`
            (`PrimitiveComponent.SetMaterial` _array_element_2 0 "/Game/Erik/SMs/Cards/M_CardGlow_Green.M_CardGlow_Green"))
          (:`2`
            (`PrimitiveComponent.SetMaterial` _array_element_2 0 "/Game/Erik/SMs/Cards/M_CardGlow_Red.M_CardGlow_Red"))
          (:`3`
            (`PrimitiveComponent.SetMaterial` _array_element_2 0 "/Game/Erik/SMs/Cards/M_CardGlow_Yellow.M_CardGlow_Yellow"))))
      (`self.ShuffleCards`))))

(event `EndTurn`
  (bind _winsneeded (`self.WinsNeeded`))
  ;[1 1 1] End turn
  (`|ExecutionSequence`
    (:`then_0`
      (if (`self.PlayerTurn`)
        (set `self.PlayerTurn` false)
        (`self.OppTakeTurn`)
        (else
          (set `self.PlayerTurn` true)
          (if (and (`self.PlayerStands`) (not (`self.OppStands`)))
            (`self.EndTurn`)))))
    (:`then_1`
      ;[1 1 1] End condition and reset
      (if (and (`self.PlayerStands`) (`self.OppStands`)) :!label _label_5
        (`/Engine/EditorBlueprintResources/StandardMacros.DoOnce` false :!label _label_6
          (:`Completed`
            (`|ExecutionSequence`
              (:`then_0`
                ;;[0 0 0] Wins
                (if (and (> (`self.PlayerCountValue`) 21) (< (`self.OppCountValue`) 22))
                  (bind _result (`/Engine/EditorBlueprintResources/StandardMacros.IncrementInt` (`self.OppWins`))
                    (:`  `
                      (set `self.OppWins` _result)))
                  (elif (and (> (`self.OppCountValue`) 21) (< (`self.PlayerCountValue`) 22))
                    (bind _result_2 (`/Engine/EditorBlueprintResources/StandardMacros.IncrementInt` (`self.PlayerWins`))
                      (:`  `
                        (set `self.PlayerWins` _result_2)))
                    (elif (and (< (`self.OppCountValue`) 22) (< (`self.PlayerCountValue`) 22))
                      (`|ExecutionSequence`
                        (:`then_0`
                          (if (> (`self.OppCountValue`) (`self.PlayerCountValue`))
                            (bind _result_3 (`/Engine/EditorBlueprintResources/StandardMacros.IncrementInt` (`self.OppWins`))
                              (:`  `
                                (set `self.OppWins` _result_3)))))
                        (:`then_1`
                          (if (< (`self.OppCountValue`) (`self.PlayerCountValue`))
                            (bind _result_4 (`/Engine/EditorBlueprintResources/StandardMacros.IncrementInt` (`self.PlayerWins`))
                              (:`  `
                                (set `self.PlayerWins` _result_4))))))))))
              (:`then_1`
                ;;[0 0 0] Set score
                (`KismetSystemLibrary.Delay` 1.0)
                (`TextRenderComponent.K2_SetText` (`self.Score`) (`|FormatText` "{opp} : {player}" (`self.OppWins`) (`self.PlayerWins`)))
                ;;[0 0 0] Check for winner
                (if (== (`self.PlayerWins`) _winsneeded)
                  (`self.PlayerWon`)
                  (`self.EndGame` :!label _label_7)
                  (elif (== (`self.OppWins`) _winsneeded)
                    (`self.OppWon`)
                    (goto _label_7))))
              (:`then_2`
                ;;[0 0 0] Reset
                (`KismetSystemLibrary.Delay` 2.0)
                (set `self.PlayerCountValue` 0)
                (set `self.OppCountValue` 0)
                (`KismetArrayLibrary.Array_Clear` (`self.PlayerCards`))
                (`KismetArrayLibrary.Array_Clear` (`self.OppCards`))
                (set `self.PlayerTurn` true)
                (set `self.PublicCardsUsed` 0)
                (set `self.CardCount` 0)
                (`self.Reset`)
                (`self.ResetEndCheck`)))))))))

(event `CheckForEndCondition`
  ;[1 1 1] End condition and reset
  (goto _label_5))

(event `ResetEndCheck`
  ;[1 1 1] End condition and reset
  (goto _label_6 :!via `Reset`))

(event `EnhancedInput|/Game/FirstPerson/Input/Actions_Default/IA_PeekRight`
  (params (ActionValue :type Boolean) (ElapsedSeconds :type "Float (double-precision)") (TriggeredSeconds :type "Float (double-precision)") (InputAction :type "InputAction Object Reference" :default "/Game/FirstPerson/Input/Actions_Default/IA_PeekRight.IA_PeekRight"))
  ;[1 1 1] Stand
  (:`Triggered`
    (if (`self.PlayerTurn`)
      (set `self.PlayerStands` true)
      (`self.EndTurn`))))

(event `EnhancedInput|/Game/FirstPerson/Input/Actions_Default/IA_PeekLeft`
  (params (ActionValue :type Boolean) (ElapsedSeconds :type "Float (double-precision)") (TriggeredSeconds :type "Float (double-precision)") (InputAction :type "InputAction Object Reference" :default "/Game/FirstPerson/Input/Actions_Default/IA_PeekLeft.IA_PeekLeft"))
  ;[1 1 1] Public hit
  (:`Triggered`
    (if (and (`self.PlayerTurn`) (< (`self.PublicCardsUsed`) 5) (not (`self.PlayerStands`)))
      (`self.PlayerPublicHit`)
      (`self.EndTurn`))))

(event `EnhancedInput|/Game/FirstPerson/Input/Actions_Default/IA_Interact`
  (params (ActionValue :type Boolean) (ElapsedSeconds :type "Float (double-precision)") (TriggeredSeconds :type "Float (double-precision)") (InputAction :type "InputAction Object Reference" :default "/Game/FirstPerson/Input/Actions_Default/IA_Interact.IA_Interact"))
  ;[1 1 1] Hit
  (:`Triggered`
    (if (and (`self.PlayerTurn`) (not (`self.PlayerStands`)))
      (`self.PlayerHit`)
      (`self.EndTurn`))))

(event `EndGame`
  (bind _playercontroller (`self.PlayerController`))
  ;[1 1 1] Exit card game
  (`self.EnableInput` _playercontroller _playercontroller :!label _label)
  (`self.EnableInput` _playercontroller _playercontroller)
  (`self.EnableInput` (`/Game/MyContent/Blueprints/Core/BP_PC_Default.Ref_PlayerCharacter` _playercontroller) _playercontroller)
  (set `/Game/MyContent/Blueprints/Core/BP_PC_Default.ControllingOther` false _playercontroller)
  (`PlayerController.SetViewTargetWithBlend` _playercontroller (`/Game/MyContent/Blueprints/Core/BP_PC_Default.Ref_PlayerCharacter` _playercontroller) 0.0 "VTBlend_Linear" 0.0 false)
  (`SceneComponent.SetVisibility` (`self.Controls`) false false)
  (`SceneComponent.SetVisibility` (`self.Score`) false false)
  (`SceneComponent.SetVisibility` (`self.OppCount`) false false)
  (`SceneComponent.SetVisibility` (`self.PlayerCount`) false false)
  (for _array_element (`self.Cards`)
    (`ActorComponent.K2_DestroyComponent` _array_element)))

(event `EnhancedInput|/Game/FirstPerson/Input/Actions_Default/IA_Pause`
  (params (ActionValue :type Boolean) (ElapsedSeconds :type "Float (double-precision)") (TriggeredSeconds :type "Float (double-precision)") (InputAction :type "InputAction Object Reference" :default "/Game/FirstPerson/Input/Actions_Default/IA_Pause.IA_Pause"))
  ;[1 1 1] Exit card game
  (:`Triggered`
    (goto _label)))

(event `EnhancedInput|/Game/FirstPerson/Input/Actions_Default/IA_ControllerBack`
  (params (ActionValue :type Boolean) (ElapsedSeconds :type "Float (double-precision)") (TriggeredSeconds :type "Float (double-precision)") (InputAction :type "InputAction Object Reference" :default "/Game/FirstPerson/Input/Actions_Default/IA_ControllerBack.IA_ControllerBack"))
  ;[1 1 1] Exit card game
  (:`Triggered`
    (goto _label)))

(event `OppTryHit`
  (params (Public :type Boolean))
  ;[1 1 1] Try hit
  (if (not (`self.OppStands`))
    (if (or (> (`self.OppCountValue`) 21) (> (`self.PlayerCountValue`) 21))
      (`self.OppStand`)
      (else
        (`KismetSystemLibrary.Delay` (`KismetMathLibrary.RandomFloatInRange` 1.0 3.0))
        (if Public
          (`self.OppPublicHit`)
          (else
            (`self.OppHit`)))
        (`self.EndTurn`)))))

(event `OppStand`
  ;[1 1 1] Stand
  (set `self.OppStands` true)
  (`self.EndTurn`))

(event `OppTakeTurn`
  ;[1 1 1] Hit chances
  (if (not (`self.PlayerStands`))
    (switch `int` (`self.OppCountValue`) :!label _label
      (:`Default`
        (`self.OppTryHit` false))
      (:`12`
        (`self.ChanceToHit` 61.54))
      (:`13`
        (`self.ChanceToHit` 53.85))
      (:`14`
        (`self.ChanceToHit` 46.15))
      (:`15`
        (`self.ChanceToHit` 38.46))
      (:`16`
        (`self.ChanceToHit` 30.77))
      (:`17`
        (`self.ChanceToHit` 23.08))
      (:`18`
        (`self.ChanceToHit` 15.38))
      (:`19`
        (`self.ChanceToHit` 7.69))
      (:`20`
        (`self.OppStand`)))
    (else
      ;;[0 0 0] Try to outsmart player
      (for _array_element (`self.Cards`) :!label _label_2
        (if (`self.IsPublicCard` _array_element)
          (`self.xd`)
          (bind _returnvalue (+ (`self.GetCardValue` _array_element) (`self.OppCountValue`)))
          (if (and (<= _returnvalue 21) (> _returnvalue (`self.PlayerCountValue`)))
            (`self.OppTryHit` true)
            (else
              (goto _label))))))))

(event `xd`
  ;[1 1 1] Hit chances
  ;;[0 0 0] Try to outsmart player
  (goto _label_2 :!via `Break`))

(event `ChanceToHit`
  (params (`%` :type "Float (double-precision)"))
  ;[1 1 1] Hit chances
  ;;[0 0 0] Template
  (if (< (`KismetMathLibrary.RandomFloatInRange` 0.0 100.0) `%`)
    (`self.OppTryHit` false)
    (elif (< (`self.PublicCardsUsed`) 5)
      (for _array_element (`self.Cards`) :!label _label_3
        (if (`self.IsPublicCard` _array_element)
          (`self.StopOppSearchForTopPublic`)
          (if (<= (+ (`self.GetCardValue` _array_element) (`self.OppCountValue`)) 21)
            (`self.OppTryHit` true)
            (else
              (`self.OppStand` :!label _label_4)))))
      (else
        (goto _label_4)))))

(event `StopOppSearchForTopPublic`
  ;[1 1 1] Hit chances
  ;;[0 0 0] Template
  (goto _label_3 :!via `Break`))

(fn `UserConstructionScript`)