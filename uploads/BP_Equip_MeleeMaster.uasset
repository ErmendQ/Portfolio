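; Master Blueprint for equippable melee weapons, which loads its stats from DT_ItemPickups by item type.
; IA_Shoot plays the swing locally and through the character's SRVMeleeSwing, unholsters the item if needed and plays the table's swing sound.
; A DoOnce gates attacks until a reset delay scaled by attack speed.
; The character's MeleeAttack applies the hit after a fixed temporary delay, independent of attack speed.
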(event `self.ReceiveBeginPlay`
  ;[1 1 1] Input
  (`self.EnableInput` (`GameplayStatics.GetPlayerController` 0))
  ;[1 1 1] Character ref
  (bind _asbp_first_person_character (cast `/Game/FirstPerson/Blueprints/BP_FirstPersonCharacter` (`GameplayStatics.GetPlayerCharacter` 0)))
  (set `self.Ref_Character` _asbp_first_person_character)
  ;[1 1 1] Get item properties
  (bind _returnvalue (`|GetDataTableRow` "/Game/MyContent/Databases/Items/DT_ItemPickups.DT_ItemPickups" (`KismetStringLibrary.Conv_StringToName` (`|GetEnumeratorNameAsString` (`self.ItemType`))))
    (:`then`
      (set `self.Properties` _returnvalue))))

(event `EnhancedInput|/Game/FirstPerson/Input/Actions_Default/IA_Shoot`
  (params (ActionValue :type Boolean) (ElapsedSeconds :type "Float (double-precision)") (TriggeredSeconds :type "Float (double-precision)") (InputAction :type "InputAction Object Reference" :default "/Game/FirstPerson/Input/Actions_Default/IA_Shoot.IA_Shoot"))
  (bind _skeletalmesh (`self.SkeletalMesh`))
  (bind (_typeid _name _description _icon _staticmesh _pickupsound _equipactor _dropspawnactor _isgun _damage _shotdelay _recoil _meleeattackspeed) (break `/Game/MyContent/Databases/Items/F_ItemPickup` (`self.Properties`)))
  ;[1 1 1] Attack
  (:`Triggered`
    (`/Engine/EditorBlueprintResources/StandardMacros.DoOnce` false :!label _label
      (:`Completed`
        (`|ExecutionSequence`
          (:`then_0`
            ;;[0 0 0] Anim
            (`SkeletalMeshComponent.PlayAnimation` _skeletalmesh "/Game/FPSwordAndShield/Animations/AttackDown.AttackDown" false)
            (`SkeletalMeshComponent.SetPlayRate` _skeletalmesh _meleeattackspeed)
            ;;[0 0 0] Anim
            (`/Game/FirstPerson/Blueprints/BP_FirstPersonCharacter.SRV_MeleeSwing` (`self.Ref_Character`))
            ;;[0 0 0] Attack reset
            (`KismetSystemLibrary.Delay` (/ 1.43 _meleeattackspeed))
            (`self.AttackReset`))
          (:`then_1`
            ;;[0 0 0] Attack function
            (`KismetSystemLibrary.Delay` 0.35) ; Temporary delay to make hit realistic
            (`/Game/FirstPerson/Blueprints/BP_FirstPersonCharacter.MeleeAttack` (`self.Ref_Character`) (`.Damage_38_89E4817C4BCBEC94E3DEFB890B1A38DB` (break `/Game/MyContent/Databases/Items/F_ItemPickup` (`self.Properties`))) (`self.HitParticle`)))
          (:`then_2`
            ;;[0 0 0] Extras
            (`self.HitUnholster`)
            (`self.PlaySwingSound`)))))))

(event `AttackReset`
  ;[1 1 1] Attack
  (goto _label :!via `Reset`))

(fn `HitUnholster`
  (bind _ref_character (`self.Ref_Character`))
  (if (`/Game/FirstPerson/Blueprints/BP_FirstPersonCharacter.ItemHolstered` _ref_character)
    (`/Game/MyContent/Blueprints/Core/BP_PC_Default.ItemHolster` (`/Game/FirstPerson/Blueprints/BP_FirstPersonCharacter.Ref_PC` _ref_character))))

(fn `PlaySwingSound`
  (bind _returnvalue (`|GetDataTableRow` "/Game/MyContent/Databases/Items/DT_ItemPickups.DT_ItemPickups" (`KismetStringLibrary.Conv_StringToName` (`|GetEnumeratorNameAsString` (`self.ItemType`))))
    (:`then`
      (`GameplayStatics.PlaySound2D` (`.SwingSound_63_E3EFD7BE4C8B5CD83D80CF9BA04F1581` (break `/Game/MyContent/Databases/Items/F_ItemPickup` _returnvalue)) 1.0 1.0 0.0 null null))))

(fn `UserConstructionScript`)