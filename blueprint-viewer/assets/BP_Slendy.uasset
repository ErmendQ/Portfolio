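; Slenderman-style enemy for a horror game that grows more aggressive and kills the player on touch through BPC_SanityCameraGlith.
; Aggression rises every second, with each destroyed BP_Page, and faster while in player sight, judged by camera yaw and distance without a trace.
; Helper functions map aggression to randomized action cooldown, halved while the player sprints, and spawn distance, plus yaw-facing toward the player; none are called here.
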(event `self.ReceiveBeginPlay`
  (bind _returnvalue (`GameplayStatics.GetActorOfClass` "/Game/MyContent/Blueprints/Core/BP_HorrorCharacter.BP_HorrorCharacter_C"))
  (bind _output_get (set `self.Player` _returnvalue))
  (set `self.PlayerCamera` (`/Game/MyContent/Blueprints/FirstPerson/Blueprints/BP_FirstPersonCharacter.FirstPersonCamera` _output_get))
  ; Set agr per second
  (`KismetSystemLibrary.K2_SetTimerDelegate` (delegate `AggressionPerSecondTimer`) 1.0 true)
  ; Set agr per collectible
  (bind _outactors (`GameplayStatics.GetAllActorsOfClass` "/Game/MyContent/Blueprints/Logic/BP_Page.BP_Page_C"))
  (for _array_element _outactors
    (add `self.OnDestroyed` _array_element (delegate `PageCollected`)))
  ; Check for in player sight
  (`KismetSystemLibrary.K2_SetTimerDelegate` (delegate `UpdateInPlayerSight`) 0.1 true))

(event `PageCollected` :!signature `self.OnDestroyed`
  (params (DestroyedActor :type "Actor Object Reference"))
  ; Set agr per collectible
  (`self.AddAggression` (`self.AggressionPerCollectible`)))

(event `UpdateInPlayerSight`
  (bind _playercamera (`self.PlayerCamera`))
  (bind (_returnvalue_roll _returnvalue_pitch _returnvalue_yaw) (`KismetMathLibrary.BreakRotator` (`KismetMathLibrary.NormalizedDeltaRotator` (`SceneComponent.K2_GetComponentRotation` _playercamera) (`KismetMathLibrary.FindLookAtRotation` (`SceneComponent.K2_GetComponentLocation` _playercamera) (`self.K2_GetActorLocation`)))))
  ; Check for in player sight
  (bind _output_get (set `self.InPlayerSight` (and (< (`KismetMathLibrary.Abs` _returnvalue_yaw) 70.0) (> (`self.VisibilityDistance`) (`KismetMathLibrary.Vector_Distance` (`self.K2_GetActorLocation` (`self.Player`)) (`self.K2_GetActorLocation`))))))
  (if _output_get
    (`self.AddAggression` (/ (`self.AggressionPerSecond`) 10.0))))

(event `AggressionPerSecondTimer`
  ; Set agr per second
  (`self.AddAggression` (`self.AggressionPerSecond`)))

(event `AddAggression`
  (params (Amount :type "Float (double-precision)"))
  ;[0.15 0.15 0.15 0.5 30] Increase agr
  (set `self.Aggression` (+ Amount (`self.Aggression`))))

(event `self.InstaKillCol.OnComponentBeginOverlap`
  (params (OverlappedComponent :type "PrimitiveComponent Object Reference") (OtherActor :type "Actor Object Reference") (OtherComp :type "PrimitiveComponent Object Reference") (OtherBodyIndex :type Integer) (bFromSweep :type Boolean) (SweepResult :type "HitResult Structure (by ref)"))
  (bind _returnvalue (`self.GetComponentByClass` OtherActor "/Game/MyContent/Blueprints/Components/BPC_SanityCameraGlith.BPC_SanityCameraGlith_C"))
  (`/Engine/EditorBlueprintResources/StandardMacros.IsValid` _returnvalue
    (:`Is Valid`
      (`/Game/MyContent/Blueprints/Components/BPC_SanityCameraGlith.Death` _returnvalue))))

(fn `CalculateCooldown`
  (returns (Out :type "Float (double-precision)"))
  (bind _player (`self.Player`))
  (bind _returnvalue (`KismetMathLibrary.MapRangeClamped` (`self.Aggression`) 0.0 (`self.MaxAggression`) (`self.MinAgrActionCooldown`) (`self.MaxAgrActionCooldown`)))
  (bind _returnvalue_2 (* _returnvalue (/ (`self.CooldownPlusMinusPercent`) 100)))
  (bind _returnvalue_3 (`KismetMathLibrary.RandomFloatInRange` (- _returnvalue _returnvalue_2) (+ _returnvalue _returnvalue_2)))
  (return (select `bool` (== (`CharacterMovementComponent.MaxWalkSpeed` (`Character.CharacterMovement` _player)) (`/Game/MyContent/Blueprints/Core/BP_HorrorCharacter.SprintSpeed` _player)) :`false` _returnvalue_3 :`true` (/ _returnvalue_3 2.0))))

(fn `CalculateSpawnDistance`
  (returns (Out :type "Float (double-precision)"))
  (bind _returnvalue (`KismetMathLibrary.MapRangeUnclamped` (`self.Aggression`) 0.0 (`self.MaxAggression`) (`self.MinAgrSpawnDistance`) (`self.MaxAgressionSpawnDistance`)))
  (bind _returnvalue_2 (* _returnvalue (/ (`self.SpawnDistancePlusMinusPercent`) 100)))
  (return (`KismetMathLibrary.RandomFloatInRange` (- _returnvalue _returnvalue_2) (+ _returnvalue _returnvalue_2))))

(fn `RotateTowardsPlayer`
  (bind (_returnvalue_roll _returnvalue_pitch _returnvalue_yaw) (`KismetMathLibrary.BreakRotator` (`KismetMathLibrary.FindLookAtRotation` (`self.K2_GetActorLocation`) (`self.K2_GetActorLocation` (`GameplayStatics.GetPlayerCharacter` 0)))))
  (`self.K2_SetActorRotation` (`KismetMathLibrary.MakeRotator` 0.0 0.0 _returnvalue_yaw)))

(fn `UserConstructionScript`)