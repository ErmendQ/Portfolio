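; Master interactable test door with keycard, lockpick, numpad and two-player variants, configured in the Construction Script through panel visibility, glow colors and interaction types.
; Toggle events update interaction prompts and play or reverse a yaw timeline, with position-checked open/close sounds.
; First keycard use plays a swipe animation before opening, lockpicking triggers Niagara sparks, and a server-to-multicast event forces opening.
; Two-player mode only starts a looping countdown timer; highlighting uses custom-depth stencils.
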(event `/Game/MyContent/Blueprints/Interfaces/BI_Interaction.OverrideInteract`
  ;[1 1 1] Force open/close
  (`self.SRV_ForceOpen`))

(event `SRV_ForceOpen`
  ;[1 1 1] Force open/close
  (`self.MC_ForceOpen`))

(event `Two player counter`
  ;[1 1 1] TwoPlayer system (meh)
  (set `self.OpenCount` (`KismetMathLibrary.Clamp` (- (`self.OpenCount`) 1) 0 3)))

(event `MC_ForceOpen`
  (bind _array (`|MakeArray` "NewEnumerator8" :!type "/Game/MyContent/Blueprints/Enums/E_InteractionTypes Enum"))
  (bind _ref_textwidget (`self.Ref_TextWidget`))
  (bind _niagara (`self.Niagara`))
  ;[1 1 1] Force open/close
  ;[1 1 1] On/Off
  (set `self.InteractionTypes` _array :!label _label)
  (set `/Game/MyContent/UI/W_WorldSpaceInteraction.Interactions` _array _ref_textwidget)
  (`/Game/MyContent/UI/W_WorldSpaceInteraction.Update` _ref_textwidget)
  (`self.Widget`
    (:`then`
      (`PrimitiveComponent.SetMaterial` (`self.Panel1Glow`) 0 "/Game/Erik/Mats/M_GreyboxGlowBlue.M_GreyboxGlowBlue")
      (`PrimitiveComponent.SetMaterial` (`self.Panel2Glow`) 0 "/Game/Erik/Mats/M_GreyboxGlowBlue.M_GreyboxGlowBlue")
      ;[1 1 1] Door movement
      (bind (_direction _newtrack_0) (`Timeline|DoorOpen` :!label _label_2)
        (:`Update`
          (`self.PlaySound`)
          (`SceneComponent.K2_SetRelativeRotation` (`self.Scene`) (`KismetMathLibrary.MakeRotator` 0.0 0.0 _newtrack_0) false false)
          (`|ExecutionSequence`
            (:`then_0`
              ;[1 1 1] Destroy spark after unlock
              (`/Engine/EditorBlueprintResources/StandardMacros.DoOnce` false
                (:`Completed`
                  (`KismetSystemLibrary.Delay` 1.0)
                  (`/Engine/EditorBlueprintResources/StandardMacros.IsValid` _niagara
                    (:`Is Valid`
                      (`ActorComponent.K2_DestroyComponent` _niagara))))))))))
    (:`else`)))

(event `self.ToggleOn`
  (params (BP_PC :type "/Game/MyContent/Blueprints/Core/BP_PC_Default Object Reference"))
  (bind _niagara (`self.Niagara`))
  ;[1 1 1] Check two player
  (if (`self.TwoPlayer`)
    ;[1 1 1] TwoPlayer system (meh)
    (`|ExecutionSequence`
      (:`then_0`
        (`/Engine/EditorBlueprintResources/StandardMacros.DoOnce` false
          (:`Completed`
            (`KismetSystemLibrary.K2_SetTimerDelegate` (delegate `Two player counter`) 1.0 true)))))
    (elif (not (`|EnumEquality` (`self.UsedItem`) "NewEnumerator2"))
      (if (not (`|EnumEquality` (`self.UsedItem`) "NewEnumerator4"))
        (goto _label)
        (else
          ;[1 1 1] Spark
          (`/Engine/EditorBlueprintResources/StandardMacros.IsValid` _niagara
            (:`Is Valid`
              (`ActorComponent.Activate` _niagara false)
              (goto _label))
            (:`Is Not Valid`
              (goto _label)))))
      (else
        ;[1 1 1] Keycard anim
        (if (`self.UnlockAnimationDone`)
          (goto _label)
          (else
            (`/Engine/EditorBlueprintResources/StandardMacros.DoOnce` false
              (:`Completed`
                (`SceneComponent.SetVisibility` (`self.SM_Keycard`) true false)
                (bind (_direction _position) (`Timeline|Keycard swipe`)
                  (:`Update`
                    (`SceneComponent.K2_SetRelativeLocation` (`self.SM_Keycard`) (`KismetMathLibrary.MakeVector` 25.0 -73.101112 _position) false false))
                  (:`Finished`
                    (set `self.UnlockAnimationDone` true) ; Finish
                    (`ActorComponent.K2_DestroyComponent` (`self.SM_Keycard`))
                    (goto _label)))))))))))

(event `self.ToggleOff`
  (params (BP_PC :type "/Game/MyContent/Blueprints/Core/BP_PC_Default Object Reference"))
  (bind _array (`|MakeArray` "NewEnumerator6" :!type "/Game/MyContent/Blueprints/Enums/E_InteractionTypes Enum"))
  (bind _ref_textwidget (`self.Ref_TextWidget`))
  ;[1 1 1] On/Off
  (set `self.InteractionTypes` _array)
  (set `/Game/MyContent/UI/W_WorldSpaceInteraction.Interactions` _array _ref_textwidget)
  (`/Game/MyContent/UI/W_WorldSpaceInteraction.Update` _ref_textwidget)
  (`self.Widget`
    (:`then`
      (`PrimitiveComponent.SetMaterial` (`self.Panel1Glow`) 0 "/Game/Erik/Mats/M_GreyboxGlowGreen.M_GreyboxGlowGreen")
      (`PrimitiveComponent.SetMaterial` (`self.Panel2Glow`) 0 "/Game/Erik/Mats/M_GreyboxGlowGreen.M_GreyboxGlowGreen")
      (goto _label_2 :!via `Reverse`))
    (:`else`)))

(event `/Game/MyContent/Blueprints/Interfaces/BI_Interaction.Highlight`
  (bind _panel2base (`self.Panel2Base`))
  ;[1 1 1] Highlight
  (`PrimitiveComponent.SetRenderCustomDepth` _panel2base true)
  (`PrimitiveComponent.SetRenderCustomDepth` (`self.Panel1Base`) true)
  (`PrimitiveComponent.SetCustomDepthStencilValue` _panel2base 2)
  (`PrimitiveComponent.SetCustomDepthStencilValue` (`self.Panel1Base`) 2))

(event `/Game/MyContent/Blueprints/Interfaces/BI_Interaction.DeHighlight`
  (bind _panel2base (`self.Panel2Base`))
  ;[1 1 1] Highlight
  (`PrimitiveComponent.SetRenderCustomDepth` _panel2base false)
  (`PrimitiveComponent.SetRenderCustomDepth` (`self.Panel1Base`) false)
  (`PrimitiveComponent.SetCustomDepthStencilValue` _panel2base 0)
  (`PrimitiveComponent.SetCustomDepthStencilValue` (`self.Panel1Base`) 0))

(fn `PlaySound`
  (bind _returnvalue (`self.K2_GetActorLocation`))
  (bind _scene (`self.Scene`))
  (if (and (`self.On`) (== (`SceneComponent.RelativeRotation` _scene) (struct :`Yaw` -10.0) :`ErrorTolerance` 2.0))
    (`GameplayStatics.PlaySoundAtLocation` "/Game/MyContent/Audio/CUEs/Door/SC_Door_Open.SC_Door_Open" _returnvalue (struct) 1.0 1.0 0.0 null null null null)
    (elif (and (not (`self.On`)) (== (`SceneComponent.RelativeRotation` _scene) (struct :`Yaw` -10.0) :`ErrorTolerance` 2.0))
      (`GameplayStatics.PlaySoundAtLocation` "/Game/MyContent/Audio/CUEs/Door/SC_Door_Close.SC_Door_Close" _returnvalue (struct) 1.0 1.0 0.0 null null null null))))

(fn `UserConstructionScript`
  (`parent.UserConstructionScript`)
  (`|ExecutionSequence`
    (:`then_0`
      ;[1 1 1] Door panel color
      (if (`self.Unlocked`)
        (`PrimitiveComponent.SetMaterial` (`self.Panel1Glow`) 0 "/Game/Erik/Mats/M_GreyboxGlowGreen.M_GreyboxGlowGreen")
        (`PrimitiveComponent.SetMaterial` (`self.Panel2Glow`) 0 "/Game/Erik/Mats/M_GreyboxGlowGreen.M_GreyboxGlowGreen")
        (else
          (`PrimitiveComponent.SetMaterial` (`self.Panel1Glow`) 0 "/Game/Erik/Mats/M_GreyboxGlowRed.M_GreyboxGlowRed")
          (`PrimitiveComponent.SetMaterial` (`self.Panel2Glow`) 0 "/Game/Erik/Mats/M_GreyboxGlowRed.M_GreyboxGlowRed"))))
    (:`then_1`
      ;[1 1 1] Two player door setup
      (if (`self.TwoPlayer`)
        (set `self.ItemUnlock` false)
        (set `self.IsToggle` false)
        (set `self.Hackable` false)
        (set `self.Numpad` false)
        (`SceneComponent.SetVisibility` (`self.Panel2Base`) true false)
        (`SceneComponent.SetVisibility` (`self.Panel2Glow`) true false)
        (else
          (`SceneComponent.SetVisibility` (`self.Panel2Glow`) false false)
          (`SceneComponent.SetVisibility` (`self.Panel2Base`) false false))))
    (:`then_2`
      ;[1 1 1] Lockpick panel visibility
      (if (`KismetArrayLibrary.Array_Contains` (`self.InteractionTypes`) "NewEnumerator4")
        (`SceneComponent.SetVisibility` (`self.Lock_PanelJoin`) true false)))
    (:`then_3`
      ;[1 1 1] Numpad visuals
      (if (`self.Numpad`)
        (set `self.TwoPlayer` false)
        (set `self.ItemUnlock` false)
        (set `self.InteractionTypes` (`|MakeArray` "NewEnumerator6" "NewEnumerator13" :!type "/Game/MyContent/Blueprints/Enums/E_InteractionTypes Enum"))
        (if (`self.Unlocked`)
          (`PrimitiveComponent.SetMaterial` (`self.Panel1Glow`) 0 "/Game/Erik/Mats/M_GreyboxGlowGreen.M_GreyboxGlowGreen")
          (`PrimitiveComponent.SetMaterial` (`self.Panel2Glow`) 0 "/Game/Erik/Mats/M_GreyboxGlowGreen.M_GreyboxGlowGreen")
          (else
            (`PrimitiveComponent.SetMaterial` (`self.Panel1Glow`) 0 "/Game/Erik/Mats/M_GreyboxGlowRed.M_GreyboxGlowRed")
            (`PrimitiveComponent.SetMaterial` (`self.Panel2Glow`) 0 "/Game/Erik/Mats/M_GreyboxGlowRed.M_GreyboxGlowRed")))))))