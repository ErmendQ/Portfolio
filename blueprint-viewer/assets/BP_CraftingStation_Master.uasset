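; Master crafting station actor with two ingredient slots and a result slot, all built on child actor components.
; Each slot swaps a placement actor for the placed pickup and reverts when that pickup is taken.
; Every slot change rechecks hard-coded recipes, some gated by the interactor's chemistry skill, to spawn the result pickup.
; Taking the result resets both slots, and custom depth stencil highlights the bench.
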(event `self.ReceiveBeginPlay`
  (`self.Reset item 1`)
  (`self.Reset item 2`))

(event `Reset item 1`
  (bind _item1 (`self.Item1`))
  ;[1 1 1] Item 1 placement
  (`ChildActorComponent.SetChildActorClass` _item1 "/Game/MyContent/Blueprints/EnvironmentInteractables/CraftingStation/BP_CraftingStation_ItemPlacement.BP_CraftingStation_ItemPlacement_C")
  (bind _asbp_crafting_station_item_placement (cast `/Game/MyContent/Blueprints/EnvironmentInteractables/CraftingStation/BP_CraftingStation_ItemPlacement` (`ChildActorComponent.ChildActor` _item1)))
  (bind _output_get (set `self.Ref_Item1` _asbp_crafting_station_item_placement))
  (add `/Game/MyContent/Blueprints/EnvironmentInteractables/CraftingStation/BP_CraftingStation_ItemPlacement.PlacedItem` _output_get (delegate `PlacedItem_Event`))
  (`self.UpdateCraftResult`))

(event `PlacedItem_Event`
  (params (Item :type "Actor Class Reference") (Interactor :type "/Game/MyContent/Blueprints/Core/BP_PC_Default Object Reference"))
  (bind _item1 (`self.Item1`))
  ;[1 1 1] Item 1 placement
  (set `self.Skill Chemistry Expert` (`/Game/MyContent/Blueprints/Core/BP_PC_Default.Skill_ChemistryExpert` Interactor))
  (`ChildActorComponent.SetChildActorClass` _item1 Item)
  (bind _asbp_pickup_test_parent (cast `/Game/MyContent/Blueprints/ItemPickups/BP_PickupTestParent` (`ChildActorComponent.ChildActor` _item1)))
  (add `/Game/MyContent/Blueprints/ItemPickups/BP_PickupTestParent.PickedUp` _asbp_pickup_test_parent (delegate `PickedUp_Item1`))
  (`self.UpdateCraftResult`))

(event `PickedUp_Item1`
  ;[1 1 1] Item 1 placement
  (`self.Reset item 1`))

(event `Reset item 2`
  (bind _item2 (`self.Item2`))
  ;[1 1 1] Item 2 placement
  (`ChildActorComponent.SetChildActorClass` _item2 "/Game/MyContent/Blueprints/EnvironmentInteractables/CraftingStation/BP_CraftingStation_ItemPlacement.BP_CraftingStation_ItemPlacement_C")
  (bind _asbp_crafting_station_item_placement (cast `/Game/MyContent/Blueprints/EnvironmentInteractables/CraftingStation/BP_CraftingStation_ItemPlacement` (`ChildActorComponent.ChildActor` _item2)))
  (bind _output_get (set `self.Ref_Item2` _asbp_crafting_station_item_placement))
  (add `/Game/MyContent/Blueprints/EnvironmentInteractables/CraftingStation/BP_CraftingStation_ItemPlacement.PlacedItem` _output_get (delegate `PlacedItem_Event_0`))
  (`self.UpdateCraftResult`))

(event `PlacedItem_Event_0`
  (params (Item :type "Actor Class Reference") (Interactor :type "/Game/MyContent/Blueprints/Core/BP_PC_Default Object Reference"))
  (bind _item2 (`self.Item2`))
  ;[1 1 1] Item 2 placement
  (set `self.Skill Chemistry Expert` (`/Game/MyContent/Blueprints/Core/BP_PC_Default.Skill_ChemistryExpert` Interactor))
  (`ChildActorComponent.SetChildActorClass` _item2 Item)
  (bind _asbp_pickup_test_parent (cast `/Game/MyContent/Blueprints/ItemPickups/BP_PickupTestParent` (`ChildActorComponent.ChildActor` _item2)))
  (add `/Game/MyContent/Blueprints/ItemPickups/BP_PickupTestParent.PickedUp` _asbp_pickup_test_parent (delegate `PickedUp_Item2`))
  (`self.UpdateCraftResult`))

(event `PickedUp_Item2`
  ;[1 1 1] Item 2 placement
  (`self.Reset item 2`))

(event `UpdateCraftResult`
  (bind _resultitem (`self.ResultItem`))
  (bind _resultitem_2 (`self.ResultItem`))
  (bind _resultitem_3 (`self.ResultItem`))
  (bind _resultitem_4 (`self.ResultItem`))
  (bind _resultitem_5 (`self.ResultItem`))
  ;[1 1 1] Update craft result
  (`ChildActorComponent.SetChildActorClass` (`self.ResultItem`) null)
  (set `self.PlacedItems` (`|MakeArray` (`ChildActorComponent.ChildActorClass` (`self.Item1`)) (`ChildActorComponent.ChildActorClass` (`self.Item2`))))
  (`|ExecutionSequence`
    (:`then_0`
      ;[1 1 1] Craft: smoke bomb
      (if (and (`KismetArrayLibrary.Array_Contains` (`self.PlacedItems`) "/Game/MyContent/Blueprints/ItemPickups/BP_Pickup_Chemicals.BP_Pickup_Chemicals_C") (`KismetArrayLibrary.Array_Contains` (`self.PlacedItems`) "/Game/MyContent/Blueprints/ItemPickups/BP_Pickup_Can.BP_Pickup_Can_C"))
        (`ChildActorComponent.SetChildActorClass` _resultitem_2 "/Game/MyContent/Blueprints/ItemPickups/BP_Pickup_SmokeBomb.BP_Pickup_SmokeBomb_C")
        (bind _asbp_pickup_test_parent (cast `/Game/MyContent/Blueprints/ItemPickups/BP_PickupTestParent` (`ChildActorComponent.ChildActor` _resultitem_2)))
        (add `/Game/MyContent/Blueprints/ItemPickups/BP_PickupTestParent.PickedUp` _asbp_pickup_test_parent (delegate `PickedUp_SmokeBomb`))))
    (:`then_1`
      ;[1 1 1] Craft: smoke bomb
      (if (and (`KismetArrayLibrary.Array_Contains` (`self.PlacedItems`) "/Game/MyContent/Blueprints/ItemPickups/BP_Pickup_Battery.BP_Pickup_Battery_C") (`KismetArrayLibrary.Array_Contains` (`self.PlacedItems`) "/Game/MyContent/Blueprints/ItemPickups/BP_Pickup_Pipe.BP_Pickup_Pipe_C"))
        (`ChildActorComponent.SetChildActorClass` _resultitem_3 "/Game/MyContent/Blueprints/ItemPickups/BP_Pickup_ElectricPipe.BP_Pickup_ElectricPipe_C")
        (bind _asbp_pickup_test_parent_2 (cast `/Game/MyContent/Blueprints/ItemPickups/BP_PickupTestParent` (`ChildActorComponent.ChildActor` _resultitem_3)))
        (add `/Game/MyContent/Blueprints/ItemPickups/BP_PickupTestParent.PickedUp` _asbp_pickup_test_parent_2 (delegate `PickedUp_ElectricPipe`))))
    (:`then_2`
      ;[1 1 1] Craft: premium drugs
      (if (and (`KismetArrayLibrary.Array_Contains` (`self.PlacedItems`) "/Game/MyContent/Blueprints/ItemPickups/BP_Pickup_Chemicals.BP_Pickup_Chemicals_C") (`KismetArrayLibrary.Array_Contains` (`self.PlacedItems`) "/Game/MyContent/Blueprints/ItemPickups/BP_Pickup_Drugs.BP_Pickup_Drugs_C") (`self.Skill Chemistry Expert`))
        (`ChildActorComponent.SetChildActorClass` _resultitem_4 "/Game/MyContent/Blueprints/ItemPickups/BP_Pickup_PremiumDrugs.BP_Pickup_PremiumDrugs_C")
        (bind _asbp_pickup_test_parent_3 (cast `/Game/MyContent/Blueprints/ItemPickups/BP_PickupTestParent` (`ChildActorComponent.ChildActor` _resultitem_4)))
        (add `/Game/MyContent/Blueprints/ItemPickups/BP_PickupTestParent.PickedUp` _asbp_pickup_test_parent_3 (delegate `PickedUp_PremiumDrugs`))))
    (:`then_3`
      ;[1 1 1] Craft: med injector
      (if (and (`KismetArrayLibrary.Array_Contains` (`self.PlacedItems`) "/Game/MyContent/Blueprints/ItemPickups/BP_Pickup_Chemicals.BP_Pickup_Chemicals_C") (`KismetArrayLibrary.Array_Contains` (`self.PlacedItems`) "/Game/MyContent/Blueprints/ItemPickups/BP_Pickup_Herb.BP_Pickup_Herb_C") (`self.Skill Chemistry Expert`))
        (`ChildActorComponent.SetChildActorClass` _resultitem_5 "/Game/MyContent/Blueprints/ItemPickups/BP_Pickup_MedInjector.BP_Pickup_MedInjector_C")
        (bind _asbp_pickup_test_parent_4 (cast `/Game/MyContent/Blueprints/ItemPickups/BP_PickupTestParent` (`ChildActorComponent.ChildActor` _resultitem_5)))
        (add `/Game/MyContent/Blueprints/ItemPickups/BP_PickupTestParent.PickedUp` _asbp_pickup_test_parent_4 (delegate `PickedUp_MedInjector`))))
    (:`then_4`
      ;[1 1 1] Craft: eletric dart
      (if (and (`KismetArrayLibrary.Array_Contains` (`self.PlacedItems`) "/Game/MyContent/Blueprints/ItemPickups/BP_Pickup_Battery.BP_Pickup_Battery_C") (`KismetArrayLibrary.Array_Contains` (`self.PlacedItems`) "/Game/MyContent/Blueprints/ItemPickups/BP_Pickup_Stick.BP_Pickup_Stick_C"))
        (`ChildActorComponent.SetChildActorClass` _resultitem "/Game/MyContent/Blueprints/ItemPickups/BP_Pickup_ElectricDart.BP_Pickup_ElectricDart_C")
        (bind _asbp_pickup_test_parent_5 (cast `/Game/MyContent/Blueprints/ItemPickups/BP_PickupTestParent` (`ChildActorComponent.ChildActor` _resultitem)))
        (add `/Game/MyContent/Blueprints/ItemPickups/BP_PickupTestParent.PickedUp` _asbp_pickup_test_parent_5 (delegate `CustomEvent`))))))

(event `PickedUp_SmokeBomb`
  ;[1 1 1] Craft: smoke bomb
  (`self.Reset item 1`)
  (`self.Reset item 2`))

(event `PickedUp_ElectricPipe`
  ;[1 1 1] Craft: smoke bomb
  (`self.Reset item 1`)
  (`self.Reset item 2`))

(event `/Game/MyContent/Blueprints/Interfaces/BI_Interaction.Highlight`
  (bind _crafting_bench_cube_001 (`self.Crafting_bench_Cube_001`))
  ;[1 1 1] Highlighting
  (`PrimitiveComponent.SetRenderCustomDepth` _crafting_bench_cube_001 true)
  (`PrimitiveComponent.SetCustomDepthStencilValue` _crafting_bench_cube_001 2))

(event `PickedUp_PremiumDrugs`
  ;[1 1 1] Craft: premium drugs
  (`self.Reset item 1`)
  (`self.Reset item 2`))

(event `/Game/MyContent/Blueprints/Interfaces/BI_Interaction.DeHighlight`
  (bind _crafting_bench_cube_001 (`self.Crafting_bench_Cube_001`))
  ;[1 1 1] Highlighting
  (`PrimitiveComponent.SetRenderCustomDepth` _crafting_bench_cube_001 false)
  (`PrimitiveComponent.SetCustomDepthStencilValue` _crafting_bench_cube_001 0))

(event `PickedUp_MedInjector`
  ;[1 1 1] Craft: med injector
  (`self.Reset item 1`)
  (`self.Reset item 2`))

(event `CustomEvent`
  ;[1 1 1] Craft: eletric dart
  (`self.Reset item 1`)
  (`self.Reset item 2`))

(fn `LookAt`
  (params (Examiner :type "/Game/MyContent/Blueprints/Core/BP_PC_Default Object Reference") (HitLocation :type "Vector Structure"))
  (returns (InteractionType :type "/Game/MyContent/Blueprints/Enums/E_InteractionTypes Enum") (Name :type String) (CanAccess :type Boolean))
  (return "NewEnumerator0" "" false))

(fn `UserConstructionScript`)