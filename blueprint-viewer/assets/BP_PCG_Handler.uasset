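; BP_PCG_Handler is a procedural placement actor that fills an adjustable rectangle with a randomized grid of buildings.
; Its construction script positions four bound components from distance settings, then spawns row-by-column static mesh components between them, without using PCG graphs.
; Each building gets a random mesh, with helper functions supplying offset, rotation (fixed list or range) and scale.
; Optional custom colors set glass and emissive material parameters through CalculateColor.
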(event EventBeginPlay)

(fn ConstructionScript
  (bind _returnvalue (Utilities|CalculateColor))
  (Utilities|FlowControl|Sequence
    (:then_0
      ;[0.15 0.15 0.15 0.5] Set bounds
      (Transformation|SetRelativeLocation (Variables|Default|GetRightBound) (Math|Vector|MakeVector 0.0 (Variables|Bounds|GetRightDistance) 0.0) false false)
      (Transformation|SetRelativeLocation (Variables|Default|GetLeftBound) (Math|Vector|MakeVector 0.0 (* (Variables|Bounds|GetLeftDistance) -1.0) 0.0) false false)
      (Transformation|SetRelativeLocation (Variables|Default|GetTopBound) (Math|Vector|MakeVector (Variables|Bounds|GetTopDistance) 0.0 0.0) false false)
      (Transformation|SetRelativeLocation (Variables|Default|GetBottomBound) (Math|Vector|MakeVector (* (Variables|Bounds|GetBottomDistance) -1.0) 0.0 0.0) false false))
    (:then_1
      ;[0.15 0.15 0.15 0.5] Generate buildings
      (Variables|Default|SetBuildingsInColumnTemp (- (Variables|BuildingCount|GetBuildingsInColumn) 1))
      (bind _output_get (Variables|Default|SetBuildingsInRowTemp (- (Variables|BuildingCount|GetBuildingsInRow) 1)))
      (for _index (range 0 _output_get)
        (for _index_2 (range 0 (Variables|Default|GetBuildingsInColumnTemp))
          (bind _returnvalue_2 (AddComponent|AddStaticMeshComponent false (Math|Transform|MakeTransform (+ (Math|Vector|MakeVector (+ (* _index_2 (/ (+ (Variables|Bounds|GetTopDistance) (Variables|Bounds|GetBottomDistance)) (Variables|Default|GetBuildingsInColumnTemp))) (.x (Variables|/Script/Engine.SceneComponent|GetRelativeLocation (Variables|Default|GetBottomBound)))) (+ (* _index (/ (+ (Variables|Bounds|GetRightDistance) (Variables|Bounds|GetLeftDistance)) (Variables|Default|GetBuildingsInRowTemp))) (.y (Variables|/Script/Engine.SceneComponent|GetRelativeLocation (Variables|Default|GetLeftBound)))) 0.0) (Utilities|CalculateRandomOffset)) (Utilities|CalculateRandomRotation) (Utilities|CalculateRandomScale))))
          ;[0.15 0.15 0.15 0.5] Set meshes and materials
          (Components|StaticMesh|SetStaticMesh _returnvalue_2 (.OutItem (Utilities|Array|Random (Variables|Default|GetBuildingMeshes))))
          (if (Variables|Colors|GetCustomColors)
            (Rendering|Material|SetColorParameterValueonMaterials _returnvalue_2 "Glass Color" _returnvalue)
            (Rendering|Material|SetColorParameterValueonMaterials _returnvalue_2 "EmissiveColor" _returnvalue)))))))