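; Base bottle item that a player holds and pours from, moved by mouse within a limited radius.
; Use shifts the mesh pivot to the opening, starts BPCPouring and loops a timer that eases the bottle above the traced surface.
; BPCPouring's consume event lowers the stored volume, updates the Fill material parameter and stops pouring when empty.
; CancelUse resets transforms and pivot; interact and drop toggle the user's pour target.
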(event `self.ReceiveBeginPlay`
  (bind _returnvalue (`SceneComponent.K2_GetComponentLocation` (`self.Pour`)))
  (bind _returnvalue_2 (`SceneComponent.K2_GetComponentLocation` (`self.Mesh`)))
  ;[0 1 0] Begin play
  (`parent.ReceiveBeginPlay`)
  (set `self.MaxVolume` (`self.GetVolume`))
  (add `/Game/Blueprints/Components/BPC_Pouring.ConsumeVolume` (`self.BPC_Pouring`) (delegate `ConsumeVolume_Event`))
  ;;[1 1 1] Set so that changing pivots always works despite mesh shape or size
  (set `self.BottleOffset` (- _returnvalue _returnvalue_2))
  (set `self.DistanceFromPourPosToPivot` (`KismetMathLibrary.Vector_Distance` _returnvalue _returnvalue_2)))

(event `ConsumeVolume_Event`
  (params (Amount :type "Float (double-precision)"))
  (bind _returnvalue (- (`self.GetVolume`) Amount))
  (bind _returnvalue_2 (select `bool` (< _returnvalue 0.0) :`false` _returnvalue))
  ;[0 1 0] Begin play
  ;;[0 1 1] Consume volume
  (setmembers `/Game/Blueprints/DataTables/Structs/S_Item2` :`StructRef` (`self.Properties`) :`Liquid_Volume` _returnvalue_2) ; Set volume on actor
  (`MeshComponent.SetScalarParameterValueOnMaterials` (`self.Liquid`) "Fill" (/ _returnvalue_2 (`self.MaxVolume`))) ; Update fill material
  (if (<= (`self.GetVolume`) 0.0)
    (`/Engine/EditorBlueprintResources/StandardMacros.DoOnce` false
      (:`Completed`
        (`/Game/Blueprints/Components/BPC_Pouring.StopPour` (`self.BPC_Pouring`))))))

(event `/Game/Blueprints/Interfaces/BPI_Interactable.Use`
  (params (User :type "/Game/Blueprints/Core/BP_FirstPersonCharacter Object Reference"))
  (bind _cancelusetimerhandle (`self.CancelUseTimerHandle`))
  (bind (_item _spawnclass _name _description _held_offset _held_slowamount _placed_offset _placed_rotation _weapon_damage _liquid_volume _liquid_pressuremuliplier _liquid_drinktype) (break `/Game/Blueprints/DataTables/Structs/S_Item2` (`self.Properties`)))
  (bind (_returnvalue_x _returnvalue_y _returnvalue_z) (`KismetMathLibrary.BreakVector` (`SceneComponent.K2_GetComponentLocation` (`/Game/Blueprints/Core/BP_FirstPersonCharacter.PouringPos` (`self.User`)))))
  ;[0 1 0] Use
  (set `self.InitialPouringPositionUponUse` (`SceneComponent.K2_GetComponentLocation` (`/Game/Blueprints/Core/BP_FirstPersonCharacter.PouringPos` User)))
  (bind _returnvalue (`KismetSystemLibrary.K2_SetTimerDelegate` (delegate `MoveToTarget`) 0.01 true))
  (add `/Game/Blueprints/Core/BP_FirstPersonCharacter.MouseMoved` User (delegate `ChangeTargetLoc`))
  (set `/Game/Blueprints/Core/BP_FirstPersonCharacter.Tapping` true User)
  (`|ExecutionSequence`
    (:`then_0`
      ;[0 1 1] Start pouring
      ;;[1 1 1] Place privot to bottle opening to calculate pour destination
      (`SceneComponent.K2_SetRelativeLocation` (`self.Mesh`) (`KismetMathLibrary.MakeVector` 0.0 0.0 (* (`self.DistanceFromPourPosToPivot`) -1.0)) false false)
      ;;[1 1 1] Set locked height (Z) for actor
      (set `self.LockedActorZ` _returnvalue_z)
      ;;[1 1 1] Only pour if item has volume
      (if (> (`self.GetVolume`) 0.0)
        (`/Game/Blueprints/Components/BPC_Pouring.StartPour` (`self.BPC_Pouring`) _liquid_pressuremuliplier _liquid_drinktype)))
    (:`then_1`
      (set `self.UseTimerHandle` _returnvalue)
      (if (`KismetSystemLibrary.K2_IsValidTimerHandle` _cancelusetimerhandle)
        (`KismetSystemLibrary.K2_ClearAndInvalidateTimerHandle` _cancelusetimerhandle)))))

(event `/Game/Blueprints/Interfaces/BPI_Interactable.Interact`
  (params (Interactor :type "/Game/Blueprints/Core/BP_FirstPersonCharacter Object Reference") (HitData :type "HitResult Structure") (OtherActor :type "Actor Object Reference"))
  ;[0 1 0] (De-)Activate pour target
  (`parent.Interact` Interactor HitData null)
  (bind _returnvalue (`/Game/Blueprints/Core/BP_FirstPersonCharacter.GetHeldItem` Interactor))
  (if (== _returnvalue self)
    (`/Game/Blueprints/Core/BP_FirstPersonCharacter.SetPourTargetActive` Interactor true)
    (set `self.User` Interactor)))

(event `ChangeTargetLoc`
  (params (X :type "Float (double-precision)") (Y :type "Float (double-precision)"))
  (bind _pouringpos (`/Game/Blueprints/Core/BP_FirstPersonCharacter.PouringPos` (`self.User`)))
  (bind (_returnvalue_x _returnvalue_y) (`KismetMathLibrary.BreakVector` (`SceneComponent.K2_GetComponentLocation` _pouringpos)))
  ;[0 1 1] Change target location and rotation
  (`SceneComponent.K2_AddLocalOffset` _pouringpos (`KismetMathLibrary.MakeVector` (* Y -1.0) (* X 1.0)) false false)
  ;;[1 1 1] Prevent moving in the Z axis
  (`SceneComponent.K2_SetWorldLocation` _pouringpos (`KismetMathLibrary.MakeVector` _returnvalue_x _returnvalue_y (`self.LockedActorZ`)) false false)
  (if (not (< (`KismetMathLibrary.Vector_Distance` (`self.InitialPouringPositionUponUse`) (`SceneComponent.K2_GetComponentLocation` _pouringpos)) (`self.AllowedRadiusOfPouring`)))
    (`SceneComponent.K2_AddLocalOffset` _pouringpos (`KismetMathLibrary.MakeVector` Y (* X -1.0)) false false)))

(event `MoveToTarget`
  ;[0 1 1] Smootly move to target location and rotation
  (`self.SmoothMoveToTargetTransform` 10.0))

(event `/Game/Blueprints/Interfaces/BPI_Interactable.Drop`
  (params (Location :type "Vector Structure") (WithoutCollision :type Boolean) (SetRotation :type Boolean) (NewRotation :type "Rotator Structure") (`Thrown?` :type Boolean) (`DisablePhysics?` :type Boolean))
  ;[0 1 0] (De-)Activate pour target
  (`parent.Drop` Location WithoutCollision SetRotation NewRotation false false)
  (`/Game/Blueprints/Core/BP_FirstPersonCharacter.SetPourTargetActive` (`self.User`) false))

(event `/Game/Blueprints/Interfaces/BPI_Interactable.CancelUse`
  (params (User :type "/Game/Blueprints/Core/BP_FirstPersonCharacter Object Reference"))
  (bind _usetimerhandle (`self.UseTimerHandle`))
  (bind _user (`self.User`))
  ;[0 1 0] Cancel use
  (`/Game/Blueprints/Interfaces/BPI_Interactable.Interact` User)
  (`self.K2_SetActorRelativeRotation` (struct))
  (`self.K2_SetActorRelativeLocation` (0.0 0.0 0.0))
  (clear `/Game/Blueprints/Core/BP_FirstPersonCharacter.MouseMoved` User)
  (set `/Game/Blueprints/Core/BP_FirstPersonCharacter.Tapping` false User)
  ;;[1 1 1] Place back to original (held) position
  (`SceneComponent.K2_SetRelativeLocation` (`/Game/Blueprints/Core/BP_FirstPersonCharacter.PouringPos` _user) (`/Game/Blueprints/Core/BP_FirstPersonCharacter.DefaultPourPosition_Relative` _user) false false)
  (`/Game/Blueprints/Components/BPC_Pouring.StopPour` (`self.BPC_Pouring`))
  ;;[1 1 1] Reset pivot to bottle bottom
  (`SceneComponent.K2_SetRelativeLocation` (`self.Mesh`) (0.0 0.0 0.0) false false)
  (if (`KismetSystemLibrary.K2_IsValidTimerHandle` _usetimerhandle)
    (`KismetSystemLibrary.K2_ClearAndInvalidateTimerHandle` _usetimerhandle)))

(fn `SmoothMoveToTargetTransform`
  (params (Speed :type "Float (double-precision)"))
  (bind _returnvalue (`SceneComponent.K2_GetComponentLocation` (`/Game/Blueprints/Core/BP_FirstPersonCharacter.PouringPos` (`self.User`))))
  (bind _returnvalue_2 (`SceneComponent.K2_GetComponentRotation` (`/Game/Blueprints/Core/BP_FirstPersonCharacter.PouringRot` (`self.User`))))
  ; Gets the location on the Surface upon which to place the bottle
  (bind _outhit (`KismetSystemLibrary.LineTraceSingle` _returnvalue (- _returnvalue (0.0 0.0 200.0)) "TraceTypeQuery4"))
  ; Set the location and rotation (also interpolate based on world time)
  (bind (_returnloc _returnrot) (`/Game/Blueprints/BarGameFunctions.FInternpLocationAndRotation` (.location (`self.GetTransform`)) (.rotation (`self.GetTransform`)) (- (+ (`.Location` (`GameplayStatics.BreakHitResult` _outhit)) (`KismetMathLibrary.MakeVector` 0.0 0.0 (`self.DistanceFromTableWhenPouring`))) (`KismetMathLibrary.GreaterGreater_VectorRotator` (`self.BottleOffset`) _returnvalue_2)) _returnvalue_2 (`GameplayStatics.GetWorldDeltaSeconds`) (`local.Speed`)))
  (`self.K2_SetActorLocationAndRotation` _returnloc _returnrot)
  (`SceneComponent.K2_SetWorldRotation` (`self.Pour`) (struct :`Pitch` -90.0) false false))

(fn `UserConstructionScript`
  (`parent.UserConstructionScript`))