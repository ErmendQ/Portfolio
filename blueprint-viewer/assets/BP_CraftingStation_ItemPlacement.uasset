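; Interactable item placement point for a crafting station that takes the player's selected inventory item.
; LookAt fills a world-space widget with that item's name from DT_ItemPickups, or "Select item", and a retriggerable delay hides it when no longer looked at.
; Interaction relays through server to multicast, which broadcasts PlacedItem with the item's DropSpawnActor, plays a placement sound and calls the player's drop-item multicast.
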(event `self.ReceiveBeginPlay`
  (`self.UpdateWidgetText`)
  ;[1 1 1] WidgetRef
  (bind _asw_world_space_interaction (cast `/Game/MyContent/UI/W_WorldSpaceInteraction` (`WidgetComponent.GetWidget` (`self.Widget`))))
  (set `self.Ref_TextWidget` _asw_world_space_interaction))

(event `LookedAt`
  ;[1 1 1] Looking at actor
  (`|ExecutionSequence`
    (:`then_0`
      (bind _widget (`self.Widget`)
        (:`then`
          (`SceneComponent.SetVisibility` _widget true false))
        (:`else`)))
    (:`then_1`
      (`KismetSystemLibrary.RetriggerableDelay` 0.1)
      (bind _widget_2 (`self.Widget`)
        (:`then`
          (`SceneComponent.SetVisibility` _widget_2 false false))
        (:`else`)))))

(event `UpdateWidgetText`
  (bind _ref_textwidget (`self.Ref_TextWidget`))
  (bind _ref_pc (`self.Ref_PC`))
  (bind _ref_textwidget_2 (`self.Ref_TextWidget`))
  ;[1 1 1] Update text
  (`/Engine/EditorBlueprintResources/StandardMacros.IsValid` (`self.Ref_TextWidget`)
    (:`Is Valid`
      ;;[0 0 0] Get selected item properties
      (bind _returnvalue (`|GetDataTableRow` "/Game/MyContent/Databases/Items/DT_ItemPickups.DT_ItemPickups" (`KismetStringLibrary.Conv_StringToName` (`|GetEnumeratorNameAsString` (`|GetArrayItem` (`/Game/MyContent/Blueprints/Core/BP_PC_Default.Items` _ref_pc) (`/Game/MyContent/Blueprints/Core/BP_PC_Default.SelectedItemIndex` _ref_pc)))))
        (:`then`
          (bind (_typeid _name) (break `/Game/MyContent/Databases/Items/F_ItemPickup` _returnvalue))
          (if (== _name "None")
            ;;[0 0 0] Set Widget Text (no item)
            (set `/Game/MyContent/UI/W_WorldSpaceInteraction.Name` "Select item" _ref_textwidget_2)
            (set `/Game/MyContent/UI/W_WorldSpaceInteraction.Interactions` (`|MakeArray` "NewEnumerator10" :!type "/Game/MyContent/Blueprints/Enums/E_InteractionTypes Enum") _ref_textwidget_2)
            (else
              ;;[0 0 0] Set Widget Text (item)
              (set `/Game/MyContent/UI/W_WorldSpaceInteraction.Interactions` (`|MakeArray` "NewEnumerator10" :!type "/Game/MyContent/Blueprints/Enums/E_InteractionTypes Enum") _ref_textwidget)
              (set `/Game/MyContent/UI/W_WorldSpaceInteraction.Name` (`KismetTextLibrary.Conv_NameToText` _name) _ref_textwidget))))))))

(event `/Game/MyContent/Blueprints/Interfaces/BI_Interaction.Interaction`
  (params (Interactor :type "/Game/MyContent/Blueprints/Core/BP_PC_Default Object Reference") (Inventory :type "Array of /Game/MyContent/Blueprints/Enums/E_Items Enum (by ref)" :default _) (Proceed :type Boolean) (InteractionOptionIndex :type Integer))
  ;[1 1 1] Interact
  (`self.SRV_Interact` Interactor))

(event `SRV_Interact`
  (params (Interactor :type "/Game/MyContent/Blueprints/Core/BP_PC_Default Object Reference"))
  ;[1 1 1] Interact
  (`self.MC_Interact` Interactor))

(event `MC_Interact`
  (params (Interactor :type "/Game/MyContent/Blueprints/Core/BP_PC_Default Object Reference"))
  (bind _output (`|GetArrayItem` (`/Game/MyContent/Blueprints/Core/BP_PC_Default.Items` Interactor) (`/Game/MyContent/Blueprints/Core/BP_PC_Default.SelectedItemIndex` Interactor)))
  ;[1 1 1] Interact
  (`/Engine/EditorBlueprintResources/StandardMacros.IsValid` Interactor
    (:`Is Valid`
      (`|ExecutionSequence`
        (:`then_0`
          (bind _returnvalue (`|GetDataTableRow` "/Game/MyContent/Databases/Items/DT_ItemPickups.DT_ItemPickups" (`KismetStringLibrary.Conv_StringToName` (`|GetEnumeratorNameAsString` _output)))
            (:`then`
              (bind (_typeid _name _description _icon _staticmesh _pickupsound _equipactor _dropspawnactor) (break `/Game/MyContent/Databases/Items/F_ItemPickup` _returnvalue))
              (bind _returnvalue_2 (!= _dropspawnactor null))
              (if _returnvalue_2
                (`self.PlacedItem` _dropspawnactor Interactor)
                (`GameplayStatics.PlaySoundAtLocation` "/Game/MyContent/Audio/CUEs/SC_ItemPlace.SC_ItemPlace" (`self.K2_GetActorLocation`) (struct) 1.0 1.0 0.0 null null null null)))))
        (:`then_1`
          (if _returnvalue_2
            (`/Game/MyContent/Blueprints/Core/BP_PC_Default.Multicast_DropItem` Interactor _output (0.0 0.0 0.0))))))))

(fn `GetInteractionsAmount`
  (returns (Amount :type Integer))
  (return 0))

(fn `LookAt`
  (params (Examiner :type "/Game/MyContent/Blueprints/Core/BP_PC_Default Object Reference") (HitLocation :type "Vector Structure"))
  (returns (InteractionType :type "/Game/MyContent/Blueprints/Enums/E_InteractionTypes Enum") (Name :type String) (CanAccess :type Boolean))
  (bind _output_get (set `self.Ref_PC` Examiner))
  (set `/Game/MyContent/UI/W_WorldSpaceInteraction.Ref_PC` _output_get (`self.Ref_TextWidget`))
  (`self.UpdateWidgetText`)
  (`self.LookedAt`)
  (return "NewEnumerator0" "" false))

(fn `UserConstructionScript`)