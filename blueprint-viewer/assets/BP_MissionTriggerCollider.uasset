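; BP_MissionTriggerCollider is a one-shot trigger volume that delivers a mission message or clue to the first-person player.
; When its Box component is overlapped by an actor whose class is exactly BP_FirstPersonCharacter, it passes its Info and Type variables to that character's FeedbackMessage with a fixed feedback type.
; It then sets an InfoGiven guard and destroys itself.
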(event `self.Box.OnComponentBeginOverlap`
  (params (OverlappedComponent :type "PrimitiveComponent Object Reference") (OtherActor :type "Actor Object Reference") (OtherComp :type "PrimitiveComponent Object Reference") (OtherBodyIndex :type Integer) (bFromSweep :type Boolean) (SweepResult :type "HitResult Structure (by ref)"))
  (if (== (`GameplayStatics.GetObjectClass` OtherActor) "/Game/FirstPerson/Blueprints/BP_FirstPersonCharacter.BP_FirstPersonCharacter_C")
    (if (not (`self.InfoGiven`))
      (bind _asbp_first_person_character (cast `/Game/FirstPerson/Blueprints/BP_FirstPersonCharacter` OtherActor))
      (`/Game/FirstPerson/Blueprints/BP_FirstPersonCharacter.FeedbackMessage` _asbp_first_person_character (`self.Info`) (`self.Type`) "NewEnumerator1" "NewEnumerator0")
      (set `self.InfoGiven` true)
      (`self.K2_DestroyActor`))))

(fn `UserConstructionScript`)