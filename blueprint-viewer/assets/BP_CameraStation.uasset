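; Interactable security camera station that lets a player view and cycle through the level's BP_SecurityCamera actors.
; On BeginPlay it gathers the cameras and creates a W_SecurityCam widget showing the current area.
; Toggleon moves input from player to station, blends the view to the first camera and marks the station busy through the controller.
; Peek inputs step the index; Interact, Back or Pause restores the player; custom depth handles highlighting.
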(event `self.ReceiveBeginPlay`
  (`parent.ReceiveBeginPlay`)
  ;[1 1 1] Widget
  (bind _returnvalue (`|CreateWidget` "/Game/MyContent/UI/Interactables/W_SecurityCam.W_SecurityCam_C" (`self.MC_Ref_PC`)))
  (set `self.Ref_CamWidget` _returnvalue)
  ;[1 1 1] Add all cameras to array
  (bind _outactors (`GameplayStatics.GetAllActorsOfClass` "/Game/MyContent/Blueprints/EnvironmentInteractables/SecurityCameras/BP_SecurityCamera.BP_SecurityCamera_C"))
  (for _array_element _outactors
    (`KismetArrayLibrary.Array_Add` (`self.Cameras`) _array_element)))

(event `self.ToggleOn`
  (params (BP_PC :type "/Game/MyContent/Blueprints/Core/BP_PC_Default Object Reference"))
  (bind _ref_camwidget (`self.Ref_CamWidget`))
  ;[1 1 1] Input switch - enter
  (`/Engine/EditorBlueprintResources/StandardMacros.IsValid` BP_PC
    (:`Is Valid`
      (`|ExecutionSequence`
        (:`then_0`
          (set `/Game/MyContent/UI/Interactables/W_SecurityCam.Ref_PC` BP_PC (`self.Ref_CamWidget`))
          (`self.DisableInput` BP_PC BP_PC)
          (bind _ref_playercharacter (`/Game/MyContent/Blueprints/Core/BP_PC_Default.Ref_PlayerCharacter` BP_PC)
            (:`then`
              (`self.DisableInput` _ref_playercharacter BP_PC)
              (`/Game/MyContent/Blueprints/Core/BP_PC_Default.HUD_Visibility` BP_PC false)
              ;[1 1 1] OpenFirstCamera
              (`PlayerController.SetViewTargetWithBlend` (`self.MC_Ref_PC`) (`|GetArrayItem` (`self.Cameras`)) 0.0 "VTBlend_Linear" 0.0 false)
              (`UserWidget.AddToViewport` _ref_camwidget 0)
              (`TextBlock.SetText` (`/Game/MyContent/UI/Interactables/W_SecurityCam.TextBlock_1` _ref_camwidget) (`KismetTextLibrary.Conv_StringToText` (`|GetEnumeratorNameAsString` (`/Game/MyContent/Blueprints/EnvironmentInteractables/SecurityCameras/BP_SecurityCamera.Area` (`|GetArrayItem` (`self.Cameras`)))))))
            (:`else`)))
        (:`then_1`
          (`self.EnableInput` BP_PC)
          (`/Game/MyContent/Blueprints/Core/BP_PC_Default.SRV_SetBusy` BP_PC self true) ; Set station busy
        )))))

(event `EnhancedInput|/Game/FirstPerson/Input/Actions_Default/IA_PeekRight`
  (params (ActionValue :type Boolean) (ElapsedSeconds :type "Float (double-precision)") (TriggeredSeconds :type "Float (double-precision)") (InputAction :type "InputAction Object Reference" :default "/Game/FirstPerson/Input/Actions_Default/IA_PeekRight.IA_PeekRight"))
  ;[1 1 1] +/- index
  (:`Triggered`
    (`/Engine/EditorBlueprintResources/StandardMacros.DoOnce` false :!label _label
      (:`Completed`
        (if (< (+ (`self.Index`) 1) (`KismetArrayLibrary.Array_Length` (`self.Cameras`)))
          (bind _result (`/Engine/EditorBlueprintResources/StandardMacros.IncrementInt` (`self.Index`))
            (:`  `
              (set `self.Index` _result)
              (`self.ChangeCamera` :!label _label_2)))))))
  (:`Completed`
    (goto _label :!via `Reset`)))

(event `EnhancedInput|/Game/FirstPerson/Input/Actions_Default/IA_Interact`
  (params (ActionValue :type Boolean) (ElapsedSeconds :type "Float (double-precision)") (TriggeredSeconds :type "Float (double-precision)") (InputAction :type "InputAction Object Reference" :default "/Game/FirstPerson/Input/Actions_Default/IA_Interact.IA_Interact"))
  ;[1 1 1] Input switch - exit
  (:`Triggered`
    (`|ExecutionSequence` :!label _label_3
      (:`then_0`
        (bind _mc_ref_pc (`self.MC_Ref_PC`)
          (:`then`
            (`self.EnableInput` _mc_ref_pc _mc_ref_pc)
            (bind _ref_playercharacter (`/Game/MyContent/Blueprints/Core/BP_PC_Default.Ref_PlayerCharacter` _mc_ref_pc)
              (:`then`
                (`self.EnableInput` _ref_playercharacter _mc_ref_pc)
                (`/Game/MyContent/Blueprints/Core/BP_PC_Default.HUD_Visibility` _mc_ref_pc true))
              (:`else`)))
          (:`else`)))
      (:`then_1`
        (`self.DisableInput` _mc_ref_pc)
        (`Widget.RemoveFromParent` (`self.Ref_CamWidget`))
        (set `self.Index` 0) ; Camera index
      )
      (:`then_2`
        (`PlayerController.SetViewTargetWithBlend` _mc_ref_pc (`/Game/MyContent/Blueprints/Core/BP_PC_Default.Ref_PlayerCharacter` _mc_ref_pc) 0.0 "VTBlend_Linear" 0.0 false) ; View back to player
        (`/Game/MyContent/Blueprints/Core/BP_PC_Default.SRV_SetBusy` _mc_ref_pc self false) ; Set not busy for camera
      ))))

(event `EnhancedInput|/Game/FirstPerson/Input/Actions_Default/IA_ControllerBack`
  (params (ActionValue :type Boolean) (ElapsedSeconds :type "Float (double-precision)") (TriggeredSeconds :type "Float (double-precision)") (InputAction :type "InputAction Object Reference" :default "/Game/FirstPerson/Input/Actions_Default/IA_ControllerBack.IA_ControllerBack"))
  ;[1 1 1] Input switch - exit
  (:`Triggered`
    (goto _label_3)))

(event `EnhancedInput|/Game/FirstPerson/Input/Actions_Default/IA_Pause`
  (params (ActionValue :type Boolean) (ElapsedSeconds :type "Float (double-precision)") (TriggeredSeconds :type "Float (double-precision)") (InputAction :type "InputAction Object Reference" :default "/Game/FirstPerson/Input/Actions_Default/IA_Pause.IA_Pause"))
  ;[1 1 1] Input switch - exit
  (:`Triggered`
    (goto _label_3)))

(event `EnhancedInput|/Game/FirstPerson/Input/Actions_Default/IA_PeekLeft`
  (params (ActionValue :type Boolean) (ElapsedSeconds :type "Float (double-precision)") (TriggeredSeconds :type "Float (double-precision)") (InputAction :type "InputAction Object Reference" :default "/Game/FirstPerson/Input/Actions_Default/IA_PeekLeft.IA_PeekLeft"))
  ;[1 1 1] +/- index
  (:`Triggered`
    (`/Engine/EditorBlueprintResources/StandardMacros.DoOnce` false :!label _label_4
      (:`Completed`
        (if (> (`self.Index`) 0)
          (bind _result (`/Engine/EditorBlueprintResources/StandardMacros.DecrementInt` (`self.Index`))
            (:`  `
              (set `self.Index` _result)
              (goto _label_2)))))))
  (:`Completed`
    (goto _label_4 :!via `Reset`)))

(event `ChangeCamera`
  (bind _output (`|GetArrayItem` (`self.Cameras`) (`self.Index`)))
  ;[1 1 1] ChangeCamera
  (`PlayerController.SetViewTargetWithBlend` (`self.MC_Ref_PC`) _output 0.0 "VTBlend_Linear" 0.0 false)
  (`TextBlock.SetText` (`/Game/MyContent/UI/Interactables/W_SecurityCam.TextBlock_1` (`self.Ref_CamWidget`)) (`KismetTextLibrary.Conv_StringToText` (`|GetEnumeratorNameAsString` (`/Game/MyContent/Blueprints/EnvironmentInteractables/SecurityCameras/BP_SecurityCamera.Area` _output))))
  (`GameplayStatics.PlaySound2D` "/Game/MyContent/Audio/CUEs/SC_CameraSwitch.SC_CameraSwitch" 1.0 2.0 0.0 null null))

(event `/Game/MyContent/Blueprints/Interfaces/BI_Interaction.Highlight`
  (bind _sm_pc (`self.SM_PC`))
  ;[1 1 1] Highlighting
  (`PrimitiveComponent.SetRenderCustomDepth` _sm_pc true)
  (`PrimitiveComponent.SetCustomDepthStencilValue` _sm_pc 2))

(event `/Game/MyContent/Blueprints/Interfaces/BI_Interaction.DeHighlight`
  (bind _sm_pc (`self.SM_PC`))
  ;[1 1 1] Highlighting
  (`PrimitiveComponent.SetRenderCustomDepth` _sm_pc false)
  (`PrimitiveComponent.SetCustomDepthStencilValue` _sm_pc 0))

(fn `UserConstructionScript`
  (`parent.UserConstructionScript`)
  (set `self.IsToggle` false)
  (set `self.TwoPlayer` false))