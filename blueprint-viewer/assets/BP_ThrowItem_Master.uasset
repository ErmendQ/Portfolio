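; Base actor for thrown items, with damage, throw force and noise looked up in DT_ItemPickups by its ItemType.
; On BeginPlay it launches the static mesh along its forward vector with an impulse and stores the damage.
; The first mesh hit calls HitEvent, empty here as a hook for children, then makes noise and destroys the actor after a delay.
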(event `self.ReceiveBeginPlay`
  (bind _staticmesh (`self.StaticMesh`))
  ;[1 1 1] AddForceOnThrow
  (bind _returnvalue (`|GetDataTableRow` "/Game/MyContent/Databases/Items/DT_ItemPickups.DT_ItemPickups" (`KismetStringLibrary.Conv_StringToName` (`|GetEnumeratorNameAsString` (`self.ItemType`))))
    (:`then`
      (bind (_typeid _name _description _icon _staticmesh_2 _pickupsound _equipactor _dropspawnactor _isgun _damage _shotdelay _recoil _meleeattackspeed _throwforce _throwactor _noise) (break `/Game/MyContent/Databases/Items/F_ItemPickup` _returnvalue))
      (`PrimitiveComponent.AddImpulse` _staticmesh (* (`SceneComponent.GetForwardVector` _staticmesh) _throwforce) "None" false)
      (set `self.Damage` _damage))))

(event `self.StaticMesh.OnComponentHit`
  (params (HitComponent :type "PrimitiveComponent Object Reference") (OtherActor :type "Actor Object Reference") (OtherComp :type "PrimitiveComponent Object Reference") (NormalImpulse :type "Vector Structure") (Hit :type "HitResult Structure (by ref)"))
  (bind _staticmesh (`self.StaticMesh`))
  ;[1 1 1] On hit
  (`/Engine/EditorBlueprintResources/StandardMacros.DoOnce` false
    (:`Completed`
      (`self.Hit event` (`.Location` (`GameplayStatics.BreakHitResult` Hit)) OtherActor)
      (`/Engine/EditorBlueprintResources/StandardMacros.IsValid` _staticmesh
        (:`Is Valid`
          ;[1 1 1] Noise
          (`self.MakeNoise` (`.Noise_69_66C3EFDC4B10677C737C3D92921EDF26` (break `/Game/MyContent/Databases/Items/F_ItemPickup` (stale `self.ReceiveBeginPlay` _returnvalue))) null (`SceneComponent.K2_GetComponentLocation` _staticmesh))
          ;[1 1 1] Destroy shortly after event triggered
          (`KismetSystemLibrary.Delay` (`self.Duration`))
          (`self.K2_DestroyActor`))))))

(event `Hit event`
  (params (Location :type "Vector Structure") (Hit :type "Actor Object Reference")))

(fn `UserConstructionScript`)