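; World item pickup, configured by a row in DT_Items, that goes into the player's inventory when interacted with.
; The construction script locks the handle to that table, applies the row's mesh and transform (or an override), clamps stackable quantity and guards against the SecondSlot row.
; On interaction it destroys itself, passes the quantity-clamped item to the interacting component, and either opens inspection or just plays a pickup sound.
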(event `self.BPC_Interactable.InteractedWith`
  (params (BPC :type "/Game/MyContent/SurviivalHorrorInventory/BPC_SurvivalHorrorInventory Object Reference"))
  (bind _returnvalue (`|GetDataTableRow` "/Game/MyContent/SurviivalHorrorInventory/Data/DT_Items.DT_Items" (`.RowName` (break `DataTableRowHandle` (`self.Item`))))
    (:`then`
      (bind _structout (setmembers `/Game/MyContent/SurviivalHorrorInventory/Data/S_Item` :`StructRef` _returnvalue :`Quantity` (`KismetMathLibrary.Clamp` (`self.Quantity`) 0 (`.MaxStack_4_72FD03864A6FE346D101B6BE6914549B` (break `/Game/MyContent/SurviivalHorrorInventory/Data/S_Item` _returnvalue)))))
      (`self.K2_DestroyActor`)
      (`/Game/MyContent/SurviivalHorrorInventory/BPC_SurvivalHorrorInventory.AddItemToInv` BPC _structout (`self.Item`))
      (if (`self.Inspect`)
        (`/Game/MyContent/SurviivalHorrorInventory/BPC_SurvivalHorrorInventory.InspectItem` BPC _structout true false)
        (`GameplayStatics.PlaySound2D` "/Game/MyContent/Audio/SW_ItemFound.SW_ItemFound" 1.0 1.0 0.0 null null)
        (else
          (`GameplayStatics.PlaySound2D` "/Game/MyContent/Sound/SC_ItemPickup.SC_ItemPickup" 1.0 1.0 0.0 null null))))))

(fn `UserConstructionScript`
  (locals (SItem_Local :type "/Game/MyContent/SurviivalHorrorInventory/Data/S_Item Structure"))
  (bind _staticmesh (`self.StaticMesh`))
  (bind _staticmesh_2 (`self.StaticMesh`))
  ;[1 1 1] Lock data table for handle
  (`|ExecutionSequence`
    (:`then_0`
      (bind _structout (setmembers `DataTableRowHandle` :`StructRef` (`self.Item`) :`DataTable` "/Game/MyContent/SurviivalHorrorInventory/Data/DT_Items.DT_Items"))
      (bind _output_get (set `self.Item` _structout))
      ;[1 1 1] Set static mesh
      (bind _returnvalue (`|GetDataTableRow` "/Game/MyContent/SurviivalHorrorInventory/Data/DT_Items.DT_Items" (`.RowName` (break `DataTableRowHandle` _output_get)))
        (:`then`
          (set `local.SItem_Local` _returnvalue)
          (bind (_displayname _description _icon _staticmesh_3 _meshtransform _stackable _quantity _maxstack) (break `/Game/MyContent/SurviivalHorrorInventory/Data/S_Item` _returnvalue))
          (`StaticMeshComponent.SetStaticMesh` (`self.StaticMesh`) _staticmesh_3)
          (if _stackable
            (`|ExecutionSequence`
              (:`then_0`
                ;[1 1 1] Prevent user from creating a stack larger than max stack allows
                (if (> (`self.Quantity`) _maxstack)
                  (set `self.Quantity` _maxstack)))
              (:`then_1`
                ;[1 1 1] Prevent user from setting quantity to 0
                (if (> 1 (`self.Quantity`))
                  (set `self.Quantity` 1))))))))
    (:`then_1`
      ;[1 1 1] Set offset and rotation
      (if (`self.OverrideMeshTransform`)
        (`SceneComponent.K2_SetRelativeLocationAndRotation` _staticmesh_2 (`self.ItemOffset`) (`self.ItemRotation`) false false)
        (`SceneComponent.SetRelativeScale3D` _staticmesh_2 (`self.ItemScale`))
        (else
          (`SceneComponent.K2_SetRelativeLocationAndRotation` _staticmesh (.location (`.MeshTransform_39_6E60F8C94CDE0BF623F733AC57FFE01B` (break `/Game/MyContent/SurviivalHorrorInventory/Data/S_Item` (`local.SItem_Local`)))) (.rotation (`.MeshTransform_39_6E60F8C94CDE0BF623F733AC57FFE01B` (break `/Game/MyContent/SurviivalHorrorInventory/Data/S_Item` (`local.SItem_Local`)))) false false)
          (`SceneComponent.SetRelativeScale3D` _staticmesh (.scale (`.MeshTransform_39_6E60F8C94CDE0BF623F733AC57FFE01B` (break `/Game/MyContent/SurviivalHorrorInventory/Data/S_Item` (`local.SItem_Local`))))))))
    (:`then_2`
      ;[1 1 1] Prevent user from selecting second slot
      (if (== (`.RowName` (break `DataTableRowHandle` (`self.Item`))) "SecondSlot")
        (setmembers `DataTableRowHandle` :`StructRef` (`self.Item`) :`RowName` "None")))))