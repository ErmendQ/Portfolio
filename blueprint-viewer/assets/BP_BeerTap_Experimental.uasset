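; Interactable beer tap that takes a placed beer glass or keg and pours beer through a mouse-dragged handle.
; Grabbing the handle binds mouse movement to its clamped roll; paired DoOnce gates start pouring near full pull with a non-empty keg and stop it otherwise.
; BPCPouring reports consumed volume, which drains the keg until empty.
; Focus drives handle outline, glow and a camera focus point, while keg placement and pouring broadcast tutorial messages.
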(event `/Game/Blueprints/Interfaces/BPI_Interactable.CancelInteract`
  (params (Interactor :type "/Game/Blueprints/Core/BP_FirstPersonCharacter Object Reference"))
  ;[0 1 0] "Release" handle
  (if (`/Game/Blueprints/Core/BP_FirstPersonCharacter.Tapping` Interactor)
    (remove `/Game/Blueprints/Core/BP_FirstPersonCharacter.MouseMoved` Interactor (delegate `MoveTapHandle`))
    (`KismetSystemLibrary.RetriggerableDelay` 0.1) ; Prevent quick camera movement after releasing handle
    (set `/Game/Blueprints/Core/BP_FirstPersonCharacter.Tapping` false Interactor)
    (`MeshComponent.SetScalarParameterValueOnMaterials` (`self.HandleTip`) "Emissive" 1.0) ; Change light to dim yellow
  ))

(event `MoveTapHandle`
  (params (X :type "Float (double-precision)") (Y :type "Float (double-precision)"))
  (bind _handlepourpitch (`self.HandlePourPitch`))
  (bind _handleorigin (`self.HandleOrigin`))
  (bind _placedkeg (`self.PlacedKeg`))
  (bind _relativerotation_roll (`KismetMathLibrary.BreakRotator` (`SceneComponent.RelativeRotation` _handleorigin)))
  ;[0 1 1] Move tap handle & start/stop pour
  (`SceneComponent.K2_SetRelativeRotation` _handleorigin (`KismetMathLibrary.MakeRotator` (`KismetMathLibrary.FClamp` (+ _relativerotation_roll Y) 0.0 _handlepourpitch)) false false)
  (if (> _relativerotation_roll (- _handlepourpitch 5.0))
    (`/Engine/EditorBlueprintResources/StandardMacros.IsValid` _placedkeg ; Is keg placed?
      (:`Is Valid`
        (if (> (`/Game/Blueprints/PickupItems/BP_BeerKeg.Volume` _placedkeg) 0.0)
          (`/Engine/EditorBlueprintResources/StandardMacros.DoOnce` false :!label _label
            (:`Completed`
              (`self.StartPour`)
              (goto _label_2 :!via `Reset`))))))
    (else
      (`/Engine/EditorBlueprintResources/StandardMacros.DoOnce` false :!label _label_2
        (:`Completed`
          (`self.StopPour`)
          (goto _label :!via `Reset`))))))

(event `/Game/Blueprints/Interfaces/BPI_Interactable.Interact`
  (params (Interactor :type "/Game/Blueprints/Core/BP_FirstPersonCharacter Object Reference") (HitData :type "HitResult Structure") (OtherActor :type "Actor Object Reference"))
  (bind _kegpos (`self.KegPos`))
  ;[0 1 0] Interaction
  (bind _returnvalue (`/Game/Blueprints/Core/BP_FirstPersonCharacter.GetHeldItem` Interactor))
  (`/Engine/EditorBlueprintResources/StandardMacros.IsValid` _returnvalue ; If player is holding any item
    (:`Is Valid`
      (`|ExecutionSequence`
        (:`then_0`
          (bind _returnvalue_2 (message `/Game/Blueprints/Interfaces/BPI_Interactable.GetItemType` _returnvalue))
          (if (`|EnumEquality` _returnvalue_2 "NewEnumerator6")
            (message `/Game/Blueprints/Interfaces/BPI_Interactable.Drop` _returnvalue (`SceneComponent.K2_GetComponentLocation` (`self.BeerPos`)) false false (struct) false false) ; Place beer in right position
          ))
        (:`then_1`
          (bind _returnvalue_3 (message `/Game/Blueprints/Interfaces/BPI_Interactable.GetItemType` _returnvalue))
          (if (`|EnumEquality` _returnvalue_3 "NewEnumerator20")
            (bind _asbp_beer_keg (cast `/Game/Blueprints/PickupItems/BP_BeerKeg` _returnvalue))
            (bind _output_get (set `self.PlacedKeg` _asbp_beer_keg)) ; Save keg reference
            (message `/Game/Blueprints/Interfaces/BPI_Interactable.Drop` _output_get (`SceneComponent.K2_GetComponentLocation` _kegpos) false true (`SceneComponent.K2_GetComponentRotation` _kegpos) false true) ; Place keg in right position
            (add `/Game/Blueprints/PickupItems/BP_ItemMaster.PickedUp` _output_get (delegate `KegPickedUp_Event`))
            (`SceneComponent.K2_SetRelativeRotation` :`self` (`self.HandleOrigin`)) ; Reset handle position when instering new keg
            ;;[0 0 0] TUTORIAL
            (`/Engine/EditorBlueprintResources/StandardMacros.DoOnce` false :!label _label_3
              (:`Completed`
                (`AsyncMessageSystemBlueprintLibrary.QueueAsyncMessageForBroadcast` (make `AsyncMessageId` (struct :`TagName` "Tutorial.KegPlaced")))
                (`KismetSystemLibrary.RetriggerableDelay` 0.1)
                (goto _label_3 :!via `Reset`)))))))
    (:`Is Not Valid`
      ;;[1 1 1] "Grab" handle
      (add `/Game/Blueprints/Core/BP_FirstPersonCharacter.MouseMoved` Interactor (delegate `MoveTapHandle`))
      (set `/Game/Blueprints/Core/BP_FirstPersonCharacter.Tapping` true Interactor)
      (`MeshComponent.SetScalarParameterValueOnMaterials` (`self.HandleTip`) "Emissive" 20.0) ; Set light to bright yellow
    )))

(event `KegPickedUp_Event`
  ;[0 1 0] Interaction
  (set `self.PlacedKeg` null))

(event `FocusLightIndication`
  ;[0 1 1] Change light on handle
  (`|ExecutionSequence`
    (:`then_0`
      (`MeshComponent.SetVectorParameterValueOnMaterials` (`self.HandleTip`) "Color" (`KismetMathLibrary.Conv_LinearColorToVector` (struct :`R` 0.019221 :`G` 0.109375 :`A` 1.0))) ; Turn on light
    )
    (:`then_1`
      (`KismetSystemLibrary.RetriggerableDelay` 0.1)
      (`MeshComponent.SetVectorParameterValueOnMaterials` (`self.HandleTip`) "Color" (`KismetMathLibrary.Conv_LinearColorToVector` (struct :`A` 1.0))) ; Turn off light
    )))

(event `StartPour`
  (bind _bpc_pouring (`self.BPC_Pouring`))
  ;[1 0 0] This needs to be moved to the BPC so it can be reused
  (`/Game/Blueprints/Components/BPC_Pouring.StartPour` _bpc_pouring (`self.Pressure Multiplier`) "NewEnumerator1")
  (add `/Game/Blueprints/Components/BPC_Pouring.ConsumeVolume` _bpc_pouring (delegate `ConsumeVolume_Event`)) ; After every projectile, subtract volume based on pressure multiplier
  (`AudioComponent.Play` (`self.Sound_WaterPouring`) 0.0))

(event `ConsumeVolume_Event`
  (params (Amount :type "Float (double-precision)"))
  (bind _placedkeg (`self.PlacedKeg`))
  ;[1 0 0] This needs to be moved to the BPC so it can be reused
  (`/Engine/EditorBlueprintResources/StandardMacros.IsValid` _placedkeg
    (:`Is Valid`
      (`/Game/Blueprints/PickupItems/BP_BeerKeg.SubtractVolume` _placedkeg Amount)
      (`|ExecutionSequence`
        (:`then_0`
          (`|ExecutionSequence`
            (:`then_0`
              ;[0 0 0] TUTORIAL
              (`/Engine/EditorBlueprintResources/StandardMacros.DoOnce` false :!label _label_4
                (:`Completed`
                  (`AsyncMessageSystemBlueprintLibrary.QueueAsyncMessageForBroadcast` (make `AsyncMessageId` (struct :`TagName` "Tutorial.BeerTapUsed"))))))
            (:`then_1`
              (`KismetSystemLibrary.RetriggerableDelay` 0.1)
              (goto _label_4 :!via `Reset`))))
        (:`then_1`
          (if (< (`/Game/Blueprints/PickupItems/BP_BeerKeg.Volume` _placedkeg) 1.0)
            (`/Game/Blueprints/Components/BPC_Pouring.StopPour` (`self.BPC_Pouring`) :!label _label_5)
            (`AudioComponent.Stop` (`self.Sound_WaterPouring`))))))
    (:`Is Not Valid`
      (goto _label_5))))

(event `StopPour`
  ;[1 0 0] This needs to be moved to the BPC so it can be reused
  (goto _label_5))

(event `/Game/Blueprints/Interfaces/BPI_Interactable.UnFocus`
  (`MeshComponent.SetOverlayMaterial` (`self.HandleMesh`) null))

(fn `Focus`
  (params (HitLocation :type "Vector Structure"))
  (returns (Location :type "Vector Structure") (Zoom :type Boolean) (ZoomAmountInFOV :type "Float (double-precision)"))
  (`self.FocusLightIndication`)
  (`MeshComponent.SetOverlayMaterial` (`self.HandleMesh`) "/Game/OurContent/Jagoda/Materials/Outlines/MI_Outline.MI_Outline")
  (return (select `bool` (and (< (`KismetMathLibrary.Vector_Distance` HitLocation (`SceneComponent.K2_GetComponentLocation` (`self.FocusPos`))) (`KismetMathLibrary.Vector_Distance` HitLocation (`SceneComponent.K2_GetComponentLocation` (`self.KegPos`)))) (> (`KismetArrayLibrary.Array_Length` (`PrimitiveComponent.GetOverlappingActors` (`self.BeerGlassDetector`) "/Game/Blueprints/PickupItems/Glasses/BP_BeerGlass.BP_BeerGlass_C")) 0)) :`true` (`SceneComponent.K2_GetComponentLocation` (`self.FocusPos`))) false 0.0))

(fn `GetAmmo`
  (returns (Return :type Integer))
  (return 0))

(fn `GetAmmoText`
  (returns (Return :type "TextRenderComponent Object Reference"))
  (return null))

(fn `GetIsPickUp`
  (returns (IsPickup :type Boolean))
  (return false))

(fn `GetItemProperties`
  (returns (Return :type "/Game/Blueprints/DataTables/Structs/S_Item2 Structure"))
  (return))

(fn `GetItemType`
  (returns (ReturnValue :type "/Game/Blueprints/Enums/E_Items Enum"))
  (return "NewEnumerator1"))

(fn `GetMaxAmmo`
  (returns (Return :type Integer))
  (return 0))

(fn `SetAmmo`
  (params (Amount :type Integer))
  (returns (Return :type Integer))
  (return 0))

(fn `SetItemProperties`
  (params (NewProperties :type "/Game/Blueprints/DataTables/Structs/S_Item2 Structure"))
  (return))

(fn `UserConstructionScript`)