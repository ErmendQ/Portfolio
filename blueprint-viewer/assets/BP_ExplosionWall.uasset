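; Breakable wall that the player can highlight and trigger to blow up after a short delay.
; Toggleon removes the highlighted cube and widget, turns the mesh red and starts the timer for Explosion.
; Explosion triggers the player's alarm, plays particles, sounds and camera shake, then fires a child-actor field system (FS_BombField) on the geometry collection.
; A later cleanup timer disables physics and collision on GCCube5.
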(event `self.ReceiveBeginPlay`
  (`parent.ReceiveBeginPlay`))

(event `/Game/MyContent/Blueprints/Interfaces/BI_Interaction.Highlight`
  ;[1 1 1] Highlighting
  (bind _cube1 (`self.Cube1`)
    (:`then`
      (`PrimitiveComponent.SetRenderCustomDepth` _cube1 true)
      (`PrimitiveComponent.SetCustomDepthStencilValue` _cube1 2))
    (:`else`)))

(event `/Game/MyContent/Blueprints/Interfaces/BI_Interaction.DeHighlight`
  ;[1 1 1] Highlighting
  (bind _cube1 (`self.Cube1`)
    (:`then`
      (`PrimitiveComponent.SetRenderCustomDepth` _cube1 false)
      (`PrimitiveComponent.SetCustomDepthStencilValue` _cube1 0))
    (:`else`)))

(event `PlaySounds`
  (bind _returnvalue (`SceneComponent.K2_GetComponentLocation` (`self.StaticMesh`)))
  (`GameplayStatics.PlaySoundAtLocation` "/Game/MyContent/Audio/CUEs/Explosion/SC_Explosion.SC_Explosion" _returnvalue (struct) 1.0 1.0 0.0 null null null null)
  (`GameplayStatics.PlaySoundAtLocation` "/Game/MyContent/Audio/CUEs/Explosion/SC_ExplosionRubble.SC_ExplosionRubble" _returnvalue (struct) 1.0 1.0 0.0 null null null null))

(event `self.ToggleOn`
  (params (BP_PC :type "/Game/MyContent/Blueprints/Core/BP_PC_Default Object Reference"))
  (bind _cube1 (`self.Cube1`)
    (:`then`
      (bind _widget (`self.Widget`)
        (:`then`
          (`ActorComponent.K2_DestroyComponent` _cube1)
          (`ActorComponent.K2_DestroyComponent` _widget)
          (`PrimitiveComponent.SetMaterial` (`self.StaticMesh`) 0 "/Game/Erik/Mats/Red.Red")
          (`KismetSystemLibrary.K2_SetTimerDelegate` (delegate `Explosion`) 1.0))
        (:`else`)))
    (:`else`)))

(event `Explosion`
  (bind _asbp_first_person_character (cast `/Game/FirstPerson/Blueprints/BP_FirstPersonCharacter` (`GameplayStatics.GetPlayerCharacter` 0)))
  (`/Game/FirstPerson/Blueprints/BP_FirstPersonCharacter.TriggerAlarm` _asbp_first_person_character _asbp_first_person_character)
  (`ActorComponent.Activate` (`self.ParticleSystem`) false)
  (`self.PlaySounds`)
  (`LegacyCameraShake.StartLegacyCameraShake` (`GameplayStatics.GetPlayerCameraManager` 0) "/Game/MyContent/Blueprints/CameraShakes/BP_CameraShake_DamageReceived.BP_CameraShake_DamageReceived_C" 5.0)
  (`ActorComponent.K2_DestroyComponent` (`self.StaticMesh`))
  (bind _asfs_bomb_field_prototype_edited (cast `/Game/MyContent/Blueprints/EnvironmentInteractables/FS_BombField_Prototype_Edited` (`ChildActorComponent.ChildActor` (`self.FS_BombField_Prototype`))))
  (set `/Game/MyContent/Blueprints/EnvironmentInteractables/FS_BombField_Prototype_Edited.Field Active` true _asfs_bomb_field_prototype_edited)
  (`/Game/MyContent/Blueprints/EnvironmentInteractables/FS_BombField_Prototype_Edited.ReExplode` _asfs_bomb_field_prototype_edited)
  (`KismetSystemLibrary.Delay` 0.2)
  (`ActorComponent.K2_DestroyComponent` (`self.FS_BombField_Prototype`))
  (`KismetSystemLibrary.K2_SetTimerDelegate` (delegate `EventCleanup`) 3.0))

(event `EventCleanup`
  (bind _gc_cube5 (`self.GC_Cube5`))
  (`PrimitiveComponent.SetSimulatePhysics` _gc_cube5 false)
  (`PrimitiveComponent.SetEnableGravity` _gc_cube5 false)
  (`PrimitiveComponent.SetCollisionEnabled` _gc_cube5 "NoCollision"))

(fn `UserConstructionScript`
  (`parent.UserConstructionScript`))