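; BP_Crawler is a horror enemy that teleports through actors tagged CrawlerSpawn, killing the player when the points run out.
; Each timed jump plays a Timeline that drains sanity via BPC_SanityDropGhost, then heals it after a delay that grows per jump.
; Overlapping Sphere2 also kills the player through BPC_SurvivalHorrorInventory.
; Its own death, via BPC_NPC_Health, restores sanity, damages the player and destroys the actor.
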(event `self.ReceiveBeginPlay`
  (bind _outactors (`GameplayStatics.GetAllActorsWithTag` "CrawlerSpawn"))
  (set `self.Out Actors` _outactors)
  (`self.TimerToMove`)
  (`GameplayStatics.PlaySound2D` "/Game/MyContent/Characters/Ghost/SW_Buildup_Cue.SW_Buildup_Cue" 1.0 1.0 0.0 null null false))

(event `TimerToMove`
  (`KismetSystemLibrary.K2_SetTimerDelegate` (delegate `CustomEvent`) 1.0))

(event `CustomEvent`
  (bind _returnvalue (`self.GetComponentByClass` (`GameplayStatics.GetPlayerCharacter` 0) "/Game/MyContent/Blueprints/Components/BPC_SanityDropGhost.BPC_SanityDropGhost_C"))
  (if (< (`self.SpawnCount`) (`KismetArrayLibrary.Array_Length` (`self.Out Actors`)))
    (bind _result (`/Engine/EditorBlueprintResources/StandardMacros.IncrementInt` (`self.SpawnCount`))
      (:`  `
        (bind _output (`|GetArrayItem` (`self.Out Actors`) (- _result 1)))
        (`self.K2_SetActorLocationAndRotation` (`self.K2_GetActorLocation` _output) (`self.K2_GetActorRotation` _output))
        (`Timeline|Timeline` :!via `PlayFromStart`
          (:`Update`
            (`/Game/MyContent/Blueprints/Components/BPC_SanityDropGhost.Damage` _returnvalue))
          (:`Finished`
            (`KismetSystemLibrary.Delay` (* (`self.SpawnCount`) 0.1))
            (`/Game/MyContent/Blueprints/Components/BPC_SanityDropGhost.Heal` _returnvalue)
            (`self.TimerToMove`)))))
    (else
      (`/Game/MyContent/SurviivalHorrorInventory/BPC_SurvivalHorrorInventory.Death` (`self.GetComponentByClass` (`GameplayStatics.GetPlayerCharacter` 0) "/Game/MyContent/SurviivalHorrorInventory/BPC_SurvivalHorrorInventory.BPC_SurvivalHorrorInventory_C")))))

(event `self.Sphere2.OnComponentBeginOverlap`
  (params (OverlappedComponent :type "PrimitiveComponent Object Reference") (OtherActor :type "Actor Object Reference") (OtherComp :type "PrimitiveComponent Object Reference") (OtherBodyIndex :type Integer) (bFromSweep :type Boolean) (SweepResult :type "HitResult Structure (by ref)"))
  (bind _returnvalue (`self.GetComponentByClass` OtherActor "/Game/MyContent/SurviivalHorrorInventory/BPC_SurvivalHorrorInventory.BPC_SurvivalHorrorInventory_C"))
  (`/Engine/EditorBlueprintResources/StandardMacros.IsValid` _returnvalue
    (:`Is Valid`
      (`/Game/MyContent/SurviivalHorrorInventory/BPC_SurvivalHorrorInventory.Death` _returnvalue))))

(event `self.BPC_NPC_Health.Death`
  (bind _returnvalue (`GameplayStatics.GetPlayerCharacter` 0))
  (`/Game/MyContent/Blueprints/Components/BPC_SanityDropGhost.Heal` (`self.GetComponentByClass` _returnvalue "/Game/MyContent/Blueprints/Components/BPC_SanityDropGhost.BPC_SanityDropGhost_C"))
  (`/Game/MyContent/SurviivalHorrorInventory/BPC_SurvivalHorrorInventory.DamagePlayer` (`self.GetComponentByClass` _returnvalue "/Game/MyContent/SurviivalHorrorInventory/BPC_SurvivalHorrorInventory.BPC_SurvivalHorrorInventory_C") 40)
  (`self.K2_DestroyActor`))

(fn `UserConstructionScript`)