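; BP_Test_ItemCabinet is a locker that opens once to reveal a stored item.
; The construction script tints the Cube red or green from the ItemUnlock flag.
; Toggleon plays a sound, removes the Widget and, if it was valid, slides the Cube along Z via the DoorOpen timeline.
; It also looks up the StoredItem enum in DT_ItemPickups, sets the ChildActor class to that drop actor and turns the color blue.
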(event `SetLightColor`
  (params (index :type Integer))
  ;[1 1 1] Set light color
  (switch `int` index
    (:`1`
      (`MeshComponent.SetVectorParameterValueOnMaterials` (`self.Cube`) "Color" (1.0 0.0 0.0)))
    (:`2`
      (`MeshComponent.SetVectorParameterValueOnMaterials` (`self.Cube`) "Color" (0.0 1.0 0.0)))
    (:`3`
      (`MeshComponent.SetVectorParameterValueOnMaterials` (`self.Cube`) "Color" (0.0 0.0 1.0)))))

(event `self.ReceiveBeginPlay`
  (`parent.ReceiveBeginPlay`))

(event `self.ToggleOn`
  (params (BP_PC :type "/Game/MyContent/Blueprints/Core/BP_PC_Default Object Reference"))
  (`/Engine/EditorBlueprintResources/StandardMacros.DoOnce` false
    (:`Completed`
      (`GameplayStatics.PlaySoundAtLocation` "/Game/MyContent/Audio/CUEs/SC_LockerOpen.SC_LockerOpen" (`self.K2_GetActorLocation`) (struct) 1.0 1.0 0.0 null null null null)
      (`|ExecutionSequence`
        (:`then_0`
          ;[1 1 1] Door opening
          (bind _widget (`self.Widget`)
            (:`then`
              (`ActorComponent.K2_DestroyComponent` _widget)
              (bind (_direction _newtrack_0) (`Timeline|DoorOpen`)
                (:`Update`
                  (`SceneComponent.K2_SetRelativeLocation` (`self.Cube`) (`KismetMathLibrary.MakeVector` 19.774417 343.829823 _newtrack_0) false false))))
            (:`else`)))
        (:`then_1`
          ;[1 1 1] SpawnItem
          (bind _returnvalue (`|GetDataTableRow` "/Game/MyContent/Databases/Items/DT_ItemPickups.DT_ItemPickups" (`KismetStringLibrary.Conv_StringToName` (`|GetEnumeratorNameAsString` (`self.StoredItem`))))
            (:`then`
              (`ChildActorComponent.SetChildActorClass` (`self.ChildActor`) (`.DropSpawnActor_30_62431BA44E767B265C61EF89D07FD1FB` (break `/Game/MyContent/Databases/Items/F_ItemPickup` _returnvalue)))
              (`self.SetLightColor` 3))))))))

(fn `UserConstructionScript`
  (`parent.UserConstructionScript`)
  (if (`self.ItemUnlock`)
    (`self.SetLightColor` 1)
    (else
      (`self.SetLightColor` 2))))