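; BP_ItemMaster is a base pickup item that players can focus, carry, drop and throw, with properties loaded from DT_Items by its type enum.
; Interact attaches it to the player's hand, or forwards it to a held tray.
; Drop detaches it, restores collision and physics unless told otherwise, and adds an impulse when thrown.
; Collision changes propagate to attached actors' tagged meshes, and glass types play a breaking sound when destroyed.
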(event `self.ReceiveBeginPlay`
  ;[0.609 1 0.59 1 30] Begin play - set properties based on enum (type)
  (bind _returnvalue (`|GetDataTableRow` "/Game/Blueprints/DataTables/DT_Items.DT_Items" (`KismetStringLibrary.Conv_StringToName` (`|GetEnumeratorNameAsString` (`self.ItemType`))))
    (:`then`
      (set `self.Properties` _returnvalue))))

(event `/Game/Blueprints/Interfaces/BPI_Interactable.Interact`
  (params (Interactor :type "/Game/Blueprints/Core/BP_FirstPersonCharacter Object Reference") (HitData :type "HitResult Structure") (OtherActor :type "Actor Object Reference"))
  ;[0.609 1 0.59] Interact
  (set `self.LastInteractor` Interactor)
  (bind _returnvalue (`/Game/Blueprints/Core/BP_FirstPersonCharacter.GetHeldItem` Interactor))
  (`/Engine/EditorBlueprintResources/StandardMacros.IsValid` _returnvalue
    (:`Is Valid`
      ;;[1 1 1] Is player holding a tray?
      (bind _returnvalue_2 (message `/Game/Blueprints/Interfaces/BPI_Interactable.GetItemType` _returnvalue))
      (if (`KismetStringLibrary.Contains` (`|GetEnumeratorNameAsString` _returnvalue_2) "Tray" false true)
        (`PrimitiveComponent.SetSimulatePhysics` (`self.Mesh`) false)
        (message `/Game/Blueprints/Interfaces/BPI_Interactable.Interact` _returnvalue (`self.LastInteractor`) (struct) self) ; Put item on tray (in player's hand)
      ))
    (:`Is Not Valid`
      (`PrimitiveComponent.SetSimulatePhysics` (`self.Mesh`) false)
      (`self.K2_AttachToComponent` (`/Game/Blueprints/Core/BP_FirstPersonCharacter.HeldItemPos` Interactor) "None" "SnapToTarget" "SnapToTarget" "KeepWorld")
      (`self.K2_AddActorLocalOffset` (`.Held_Offset_31_F34959A24CA516816DD8AF88C46E556C` (break `/Game/Blueprints/DataTables/Structs/S_Item2` (`self.Properties`))))
      (`/Game/Blueprints/Interfaces/BPI_Interactable.SetCollision` false)
      (`self.PickedUp`)
      (`/Game/Blueprints/Core/BP_FirstPersonCharacter.UpdateCurrentSpeed` (`self.LastInteractor`)))))

(event `/Game/Blueprints/Interfaces/BPI_Interactable.Drop`
  (params (Location :type "Vector Structure") (WithoutCollision :type Boolean) (SetRotation :type Boolean) (NewRotation :type "Rotator Structure") (`Thrown?` :type Boolean) (`DisablePhysics?` :type Boolean))
  ;[0.609 1 0.59] Drop
  (`self.K2_DetachFromActor` "KeepWorld" "KeepWorld" "KeepWorld")
  (`self.K2_SetActorRotation` (select `bool` SetRotation :`true` NewRotation) true)
  (if (not `Thrown?`)
    (`self.K2_SetActorLocation` Location true)
    (`/Game/Blueprints/Interfaces/BPI_Interactable.SetCollision` (not WithoutCollision)))
  (if `DisablePhysics?`
    (`/Game/Blueprints/Interfaces/BPI_Interactable.SetSimulation` false)
    (else
      (`/Game/Blueprints/Interfaces/BPI_Interactable.SetCollision` true)
      (`/Game/Blueprints/Interfaces/BPI_Interactable.SetSimulation` true)
      ;[0.15 0 0 0.5] Perk (Throwing)
      (if `Thrown?`
        (`PrimitiveComponent.AddImpulse` (`self.Mesh`) Location "None" false)))))

(event `/Game/Blueprints/Interfaces/BPI_Interactable.SetCollision`
  (params (Collision :type Boolean))
  (bind _returnvalue (`KismetMathLibrary.SelectName` "ItemPhysics" "NoCollision" Collision))
  (bind _outactors (`self.GetAttachedActors` true true))
  ;[0.609 1 0.59] Collision / Physics(?)
  (`PrimitiveComponent.SetCollisionProfileName` (`self.Mesh`) _returnvalue true)
  (if (`KismetArrayLibrary.Array_IsNotEmpty` _outactors)
    (for _array_element _outactors
      (bind _output (`|GetArrayItem` (`self.GetComponentsByTag` _array_element "/Script/Engine.StaticMeshComponent" "BaseMesh")))
      (`/Engine/EditorBlueprintResources/StandardMacros.IsValid` _output
        (:`Is Valid`
          (`PrimitiveComponent.SetCollisionProfileName` _output _returnvalue true))))))

(event `/Game/Blueprints/Interfaces/BPI_Interactable.UnFocus`
  ;[0 1 1] Unfocus
  (`MeshComponent.SetOverlayMaterial` (`self.Mesh`) null))

(event `/Game/Blueprints/Interfaces/BPI_Interactable.SetSimulation`
  (params (`Simulate?` :type Boolean))
  (`PrimitiveComponent.SetSimulatePhysics` (`self.Mesh`) `Simulate?`))

(event `self.ReceiveDestroyed`
  ;[0 1 1] Audio on destroyed
  (switch `/Game/Blueprints/Enums/E_Items` (`self.ItemType`)
    (:`NewEnumerator6`
      _)
    (:`NewEnumerator0`
      _)
    (:`NewEnumerator2`
      _)
    (:`NewEnumerator3`
      _))
  (`GameplayStatics.PlaySoundAtLocation` "/Game/Assets/Sounds/Sound_GlassBreaking.Sound_GlassBreaking" (`self.K2_GetActorLocation`) (struct) 1.0 1.0 0.0 "/Game/Assets/Sounds/AttenuationSettings/SA_ProjectileSounds.SA_ProjectileSounds" null null null))

(fn `Focus`
  (params (HitLocation :type "Vector Structure"))
  (returns (Location :type "Vector Structure") (Zoom :type Boolean) (ZoomAmountInFOV :type "Float (double-precision)"))
  (`MeshComponent.SetOverlayMaterial` (`self.Mesh`) "/Game/OurContent/Jagoda/Materials/Outlines/MI_OverlayPickUp_Inst.MI_OverlayPickUp_Inst") ; ShineEffect
  (return (0.0 0.0 0.0) false 0.0))

(fn `GetAmmo`
  (returns (Return :type Integer))
  (return 0))

(fn `GetAmmoText`
  (returns (Return :type "TextRenderComponent Object Reference"))
  (return null))

(fn `GetItemProperties`
  (returns (Return :type "/Game/Blueprints/DataTables/Structs/S_Item2 Structure"))
  (return (`self.Properties`)))

(fn `GetItemType`
  (returns (ReturnValue :type "/Game/Blueprints/Enums/E_Items Enum"))
  (return (`self.ItemType`)))

(fn `GetMaxAmmo`
  (returns (Return :type Integer))
  (return 0))

(fn `SetAmmo`
  (params (Amount :type Integer))
  (returns (Return :type Integer))
  (return 0))

(fn `SetItemProperties`
  (params (NewProperties :type "/Game/Blueprints/DataTables/Structs/S_Item2 Structure"))
  (set `self.Properties` NewProperties)
  (return))

(fn `UserConstructionScript`)