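; BP_Watcher is a ghost actor that turns to face the player and drives the player's BPC_SanityDropGhost component.
; It registers in that component's ActiveGhosts and calls Damage every Tick while TriggerProximity is false.
; Overlapping its radius-configurable sphere clears that flag, then after a brief delay destroys the ghost and calls Heal.
; An optional duration timer also heals and removes it.
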(event `self.ReceiveTick`
  (params (DeltaSeconds :type "Float (single-precision)"))
  (if (not (`self.TriggerProximity`))
    (`/Game/MyContent/Blueprints/Components/BPC_SanityDropGhost.Damage` (`self.StaticRef`))))

(event `self.ReceiveBeginPlay`
  (bind _returnvalue (`self.GetComponentByClass` (`GameplayStatics.GetPlayerCharacter` 0) "/Game/MyContent/Blueprints/Components/BPC_SanityDropGhost.BPC_SanityDropGhost_C"))
  (`|ExecutionSequence`
    (:`then_0`
      (if (`self.ForDuration`)
        (`KismetSystemLibrary.K2_SetTimerDelegate` (delegate `Destroy`) (`self.Duration`))))
    (:`then_1`
      (`KismetSystemLibrary.K2_SetTimerDelegate` (delegate `RotateTowardsPlayer`) 0.1 true))
    (:`then_2`
      (`KismetArrayLibrary.Array_Add` (`/Game/MyContent/Blueprints/Components/BPC_SanityDropGhost.ActiveGhosts` _returnvalue) self)
      (set `self.StaticRef` _returnvalue))))

(event `Destroy`
  (`/Game/MyContent/Blueprints/Components/BPC_SanityDropGhost.Heal` (`self.StaticRef`))
  (`self.K2_DestroyActor`))

(event `RotateTowardsPlayer`
  (bind (_returnvalue_roll _returnvalue_pitch _returnvalue_yaw) (`KismetMathLibrary.BreakRotator` (`KismetMathLibrary.FindLookAtRotation` (`self.K2_GetActorLocation`) (`self.K2_GetActorLocation` (`GameplayStatics.GetPlayerCharacter` 0)))))
  (`self.K2_SetActorRotation` (`KismetMathLibrary.MakeRotator` 0.0 0.0 _returnvalue_yaw)))

(event `self.Sphere2.OnComponentBeginOverlap`
  (params (OverlappedComponent :type "PrimitiveComponent Object Reference") (OtherActor :type "Actor Object Reference") (OtherComp :type "PrimitiveComponent Object Reference") (OtherBodyIndex :type Integer) (bFromSweep :type Boolean) (SweepResult :type "HitResult Structure (by ref)"))
  (bind _returnvalue (`self.GetComponentByClass` OtherActor "/Game/MyContent/Blueprints/Components/BPC_SanityDropGhost.BPC_SanityDropGhost_C"))
  ;[1 1 1] Disappear and trigger glitch on proximity
  (`/Engine/EditorBlueprintResources/StandardMacros.IsValid` _returnvalue
    (:`Is Valid`
      (set `self.TriggerProximity` false)
      (`KismetSystemLibrary.Delay` 0.1)
      (`self.K2_DestroyActor`)
      (`/Game/MyContent/Blueprints/Components/BPC_SanityDropGhost.Heal` _returnvalue))))

(fn `UserConstructionScript`
  (`SphereComponent.SetSphereRadius` (`self.Sphere2`) (`self.In Sphere Radius`) true))