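; BP_SolitaryControl is a control actor that unlocks the solitary cells in the level.
; Its Toggleon event checks that the passed BPPC is valid, then finds every BP_Cells actor and calls Unlock with BPPC on those flagged Solitary.
; The construction script sets Cube2 to a green or red glow material from the Unlocked flag, which Toggleon does not change.
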(event `self.ToggleOn`
  (params (BP_PC :type "/Game/MyContent/Blueprints/Core/BP_PC_Default Object Reference"))
  ;[1 1 1] Disable
  (`/Engine/EditorBlueprintResources/StandardMacros.IsValid` BP_PC
    (:`Is Valid`
      (bind _outactors (`GameplayStatics.GetAllActorsOfClass` "/Game/Mara/EnvironmentBlueprints/BP_Cells.BP_Cells_C"))
      (for _array_element _outactors
        (if (`/Game/Mara/EnvironmentBlueprints/BP_Cells.Solitary` _array_element)
          (`/Game/Mara/EnvironmentBlueprints/BP_Cells.Unlock` _array_element BP_PC))))))

(fn `UserConstructionScript`
  (bind _cube2 (`self.Cube2`))
  (`parent.UserConstructionScript`)
  (if (`self.Unlocked`)
    (`PrimitiveComponent.SetMaterial` _cube2 0 "/Game/Erik/Mats/M_GreyboxGlowGreen.M_GreyboxGlowGreen")
    (else
      (`PrimitiveComponent.SetMaterial` _cube2 0 "/Game/Erik/Mats/M_GreyboxGlowRed.M_GreyboxGlowRed"))))