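; Nightmare turret actor that tracks the first player's character and fires projectiles while it is Active.
; Tick calls RotateTowardsPlayer, which snaps the Scene component to a look-at rotation toward the player's location.
; A looping timer started on BeginPlay with the ShotDelay interval spawns BP_FirstPersonProjectile at the Scene component's world transform.
; The Active flag gates both rotation and shooting, while the timer keeps running regardless.
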(event `self.ReceiveBeginPlay`
  (`KismetSystemLibrary.K2_SetTimerDelegate` (delegate `Shoot`) (`self.ShotDelay`) true))

(event `Shoot`
  (bind _returnvalue (`SceneComponent.K2_GetComponentToWorld` (`self.Scene`)))
  (if (`self.Active`)
    (`|SpawnActorFromClass` "/Game/FirstPerson/Blueprints/BP_FirstPersonProjectile.BP_FirstPersonProjectile_C" (`KismetMathLibrary.MakeTransform` (.location _returnvalue) (`KismetMathLibrary.MakeRotator` (.roll (.rotation _returnvalue)) (.pitch (.rotation _returnvalue)) (.yaw (.rotation _returnvalue))) (.scale _returnvalue)) "Undefined" "MultiplyWithRoot" null null)))

(event `self.ReceiveTick`
  (params (DeltaSeconds :type "Float (single-precision)"))
  (bind _scene (`self.Scene`))
  ;[1 1 1] Tick
  (if (`self.Active`)
    (`SceneComponent.K2_SetWorldRotation` _scene (`KismetMathLibrary.FindLookAtRotation` (`SceneComponent.K2_GetComponentLocation` _scene) (`self.K2_GetActorLocation` (`GameplayStatics.GetPlayerCharacter` 0))) false false)))

(fn `UserConstructionScript`)